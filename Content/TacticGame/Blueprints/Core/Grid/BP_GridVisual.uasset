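; BP_GridVisual renders the tactics grid through two child BP_GridMeshInst instanced-mesh actors.
; The normal grid shows walkable tiles colored by state at a ground offset; the tactical grid colors by tile type, including obstacles.
; Tactical tiles stretch in Z down to the tracked lowest tile, regenerating lazily via a dirty flag when enabled.
; Toggling tactical mode hides "NotTactical"-tagged actors and switches tactical grid visibility and collision.
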(event `self.ReceiveBeginPlay`
  ;[1 1 1] Disables the Tick
  (`self.SetActorTickEnabled` false))

(fn `DestroyGridVisual`
  (bind _gridmeshinst (`self.GridMeshInst`))
  (bind _gridmeshinst_tactical (`self.GridMeshInst_Tactical`))
  (`|ExecutionSequence`
    (:`then_0`
      ;[1 1 1] Normal Grid
      (`/Engine/EditorBlueprintResources/StandardMacros.IsValid` _gridmeshinst
        (:`Is Valid`
          (`/Game/TacticGame/Blueprints/Core/Grid/Utilities/BP_GridMeshInst.ClearInstances` _gridmeshinst))))
    (:`then_1`
      ;[1 1 1] Tactical Grid
      (`/Engine/EditorBlueprintResources/StandardMacros.IsValid` _gridmeshinst_tactical
        (:`Is Valid`
          (`/Game/TacticGame/Blueprints/Core/Grid/Utilities/BP_GridMeshInst.ClearInstances` _gridmeshinst_tactical))))
    (:`then_2`
      (`self.SetGridLowestZ` 999999.0) ; If the Grid is destroyed, the lowest Z is reset
    )))

(fn `InitializeGridVisual`
  (params (Grid :type "/Game/TacticGame/Blueprints/Core/Grid/BP_Grid Object Reference"))
  (bind (_meshsize _mesh _meshmaterial _flatmesh _flatmaterial) (break `/Game/TacticGame/Blueprints/Core/Grid/GridShapes/S_GridShapeData` (`/Game/TacticGame/Blueprints/Core/Grid/BP_Grid.GetCurrentShapeData` (`self.Grid`))))
  (bind (_meshsize_2 _mesh_2 _meshmaterial_2) (break `/Game/TacticGame/Blueprints/Core/Grid/GridShapes/S_GridShapeData` (`/Game/TacticGame/Blueprints/Core/Grid/BP_Grid.GetCurrentShapeData` (`self.Grid`))))
  (set `self.Grid` Grid)
  (set `self.GridMeshInst` (cast `/Game/TacticGame/Blueprints/Core/Grid/Utilities/BP_GridMeshInst` (`ChildActorComponent.ChildActor` (`self.ChildActor_GridMeshInst`)) :!pure true))
  (set `self.GridMeshInst_Tactical` (cast `/Game/TacticGame/Blueprints/Core/Grid/Utilities/BP_GridMeshInst` (`ChildActorComponent.ChildActor` (`self.ChildActor_GridMeshInst_Tactical`)) :!pure true))
  ;[1 1 1] Setup the components for the Normal Grid
  (`/Game/TacticGame/Blueprints/Core/Grid/Utilities/BP_GridMeshInst.InitializeGridMeshInst` (`self.GridMeshInst`) _flatmesh _flatmaterial false "QueryOnly") ; Normal Grid - Colors based on State
  ;[1 1 1] Setup the components for the Tactical Grid
  (`/Game/TacticGame/Blueprints/Core/Grid/Utilities/BP_GridMeshInst.InitializeGridMeshInst` (`self.GridMeshInst_Tactical`) _mesh_2 _meshmaterial_2 true "QueryOnly") ; Tactical Grid - Colors based on Tile Type
  (`self.K2_SetActorLocation` (0.0 0.0 0.0)) ; Center Grid in World (0,0,0)
  (`self.SetOffsetFromGround` (`self.OffsetFromGround`))
  (`self.SetGridLowestZ` 999999.0) ; Reset lowest Z
  (`self.SetIsTactical` (`self.IsTactical`)) ; To make the level start without the tactical grid visible
)

(fn `SetGridLowestZ`
  (params (Z :type "Float (double-precision)" :default 999999.0))
  (set `self.GridLowestZ` Z)
  (set `self.NeedToRegenerateTacticalOnNextEnable` true))

(fn `SetIsTactical`
  (params (Tactical :type Boolean))
  (bind _grid (`self.Grid`))
  (bind _gridmeshinst_tactical (`self.GridMeshInst_Tactical`))
  (set `self.IsTactical` Tactical)
  ;[1 1 1] Added just for the Viewport flickering
  (`SceneComponent.SetVisibility` (`/Game/TacticGame/Blueprints/Core/Grid/Utilities/BP_GridMeshInst.InstancedStaticMesh` (`self.GridMeshInst_Tactical`)) (`self.IsTactical`) false) ; To avoid flickering in Viewport
  ;[1 1 1] If tactical is set, show the tactical grid
  (`SceneComponent.SetHiddenInGame` (`self.ChildActor_GridMeshInst_Tactical`) (not (`self.IsTactical`)) false)
  ;[1 1 1] Get all the Actors in the game with the Tag "NotTactical" and hide them
  (bind _outactors (`GameplayStatics.GetAllActorsWithTag` "NotTactical"))
  (for _array_element _outactors
    (`self.SetActorHiddenInGame` _array_element (`self.IsTactical`)))
  (`|ExecutionSequence`
    (:`then_0`
      ;[1 1 1] If tactical grid was just selected and we need to generate the grid,
      ; then we set the need to regenerate flag to FALSE, because we're doing right after this node
      (if (and (`self.IsTactical`) (`self.NeedToRegenerateTacticalOnNextEnable`))
        (set `self.NeedToRegenerateTacticalOnNextEnable` false)
        ;[1 1 1] Tactical Grid regeneration, go through all the tiles and call the UpdateTileVisualTactical on them
        ; (ONLY the tactical visual update, not the normal one)
        (`/Engine/EditorBlueprintResources/StandardMacros.IsValid` _grid
          (:`Is Valid`
            (bind _values (`BlueprintMapLibrary.Map_Values` (`/Game/TacticGame/Blueprints/Core/Grid/BP_Grid.GridTiles` _grid)))
            (for _array_element_2 _values
              (`self.UpdateTileVisual_Tactical` _array_element_2))))))
    (:`then_1`
      ;[1 1 1] We want to disable the collision if the Grid is in tactical mode
      (`/Engine/EditorBlueprintResources/StandardMacros.IsValid` _gridmeshinst_tactical ; Invalid if Grid never generated
        (:`Is Valid`
          (`PrimitiveComponent.SetCollisionEnabled` (`/Game/TacticGame/Blueprints/Core/Grid/Utilities/BP_GridMeshInst.InstancedStaticMesh` _gridmeshinst_tactical) (select `bool` (`self.IsTactical`) :`false` "NoCollision" :`true` "QueryOnly" :!type "ECollisionEnabled Enum")))))))

(fn `SetOffsetFromGround`
  (params (Offset :type "Float (double-precision)"))
  (set `self.OffsetFromGround` Offset)
  ;[1 1 1] Please note that the SetRelativeLocation is called only on the GridMeshInst
  ; that means that GridMeshInst_Tactical will not be adjusted by the Offset from ground
  ; It is intended because the tactical grid should replace the terrain entirely and
  ; should be placed at its level (and not above it like the normal grid)
  (`SceneComponent.K2_SetRelativeLocation` (`self.ChildActor_GridMeshInst`) (`KismetMathLibrary.MakeVector` 0.0 0.0 (`self.OffsetFromGround`)) false false) ; only the Z gets adjusted
)

(fn `UpdateTileVisual`
  (params (Data :type "/Game/TacticGame/Blueprints/Core/Grid/Utilities/S_TileData Structure"))
  (bind (_data_index _data_type) (break `/Game/TacticGame/Blueprints/Core/Grid/Utilities/S_TileData` (`local.Data`)))
  (bind (_data_index_2 _data_type_2 _data_transform _data_states) (break `/Game/TacticGame/Blueprints/Core/Grid/Utilities/S_TileData` (`local.Data`)))
  (`|ExecutionSequence`
    (:`then_0`
      ;[1 1 1] Normal Grid
      ;;[1 1 1] The first thing is to remove the old tile
      (`/Game/TacticGame/Blueprints/Core/Grid/Utilities/BP_GridMeshInst.RemoveInstance` (`self.GridMeshInst`) _data_index)
      ;;[1 1 1] The tile is created only if the type is walkable
      (if (`/Game/TacticGame/Blueprints/Core/Grid/Utilities/BFL_TileData.IsTileTypeWalkable` _data_type)
        (`/Game/TacticGame/Blueprints/Core/Grid/Utilities/BP_GridMeshInst.AddInstance` (`self.GridMeshInst`) _data_index_2 _data_type_2 _data_transform _data_states)))
    (:`then_1`
      ;[1 1 1] Tactical Grid
      (`self.UpdateTileVisual_Tactical` Data))))

(fn `UpdateTileVisual_Tactical`
  (params (Data :type "/Game/TacticGame/Blueprints/Core/Grid/Utilities/S_TileData Structure"))
  (bind (_data_index _data_type _data_transform) (break `/Game/TacticGame/Blueprints/Core/Grid/Utilities/S_TileData` (`local.Data`)))
  (bind (_data_index_2 _data_type_2 _data_transform_2) (break `/Game/TacticGame/Blueprints/Core/Grid/Utilities/S_TileData` (`local.Data`)))
  (bind (_data_index_3 _data_type_3 _data_transform_3 _data_states) (break `/Game/TacticGame/Blueprints/Core/Grid/Utilities/S_TileData` (`local.Data`)))
  (bind (_data_index_4 _data_type_4) (break `/Game/TacticGame/Blueprints/Core/Grid/Utilities/S_TileData` (`local.Data`)))
  (bind _z (.z (`.MeshSize_2_09D7913C41F06EB5C6F9088AC614A7CA` (break `/Game/TacticGame/Blueprints/Core/Grid/GridShapes/S_GridShapeData` (`/Game/TacticGame/Blueprints/Core/Grid/BP_Grid.GetCurrentShapeData` (`self.Grid`))))))
  (`|ExecutionSequence`
    (:`then_0`
      ;[1 1 1] Before the proper function code, we check if the tile we are elaborating is the lowest one for the current grid
      ; so we check if its Z location (height) is lower than our minimin, if that's the case, a new minimun is set
      (if (< (.z (.location _data_transform_2)) (`self.GridLowestZ`))
        (`self.SetGridLowestZ` (.z (.location _data_transform_2)))))
    (:`then_1`
      ;[1 1 1] De don't want to waste resource generating a tactical grid when not necessary
      ; so we condition its generation and have a flag that tells us when it's necessary to do it
      (if (`self.IsTactical`)
        ;[1 1 1] The first thing is to remove the old tile
        (`/Game/TacticGame/Blueprints/Core/Grid/Utilities/BP_GridMeshInst.RemoveInstance` (`self.GridMeshInst_Tactical`) _data_index_4)
        ;[1 1 1] For the Tactical Grid we don't display only the walkable tile, but also obstacles
        (if (`|EnumInequality` _data_type_4 "NewEnumerator0")
          (`/Game/TacticGame/Blueprints/Core/Grid/Utilities/BP_GridMeshInst.AddInstance` (`self.GridMeshInst_Tactical`) _data_index_3 _data_type_3 (`KismetMathLibrary.MakeTransform` (.location _data_transform_3) (.rotation _data_transform_3) (`KismetMathLibrary.MakeVector` (.x (.scale _data_transform_3)) (.y (.scale _data_transform_3)) (/ (+ (- (.z (.location _data_transform)) (`self.GridLowestZ`)) _z) _z))) _data_states))
        (else
          (set `self.NeedToRegenerateTacticalOnNextEnable` true))))))

(fn `UserConstructionScript`)