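; BP_GridModifier is a level-placed volume that marks a tile type for the tactical grid, such as obstacle, extra movement cost or flying units only.
; Its construction script takes the mesh and flat material from the Shape data and tints them by Type.
; It overlaps the ground trace channel, blocks the spell line-of-sight channel and is hidden in game.
; Collision responses are set after the mesh because SetStaticMesh resets them.
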(fn `UserConstructionScript`
  (bind _staticmesh (`self.StaticMesh`))
  (bind (_data_meshsize _data_mesh _data_meshmaterial _data_flatmesh _data_flatmaterial) (break `/Game/TacticGame/Blueprints/Core/Grid/GridShapes/S_GridShapeData` (`/Game/TacticGame/Blueprints/Core/Grid/GridShapes/BFL_GridShape.GetShapeData` (`self.Shape`))))
  (`StaticMeshComponent.SetStaticMesh` _staticmesh _data_mesh)
  (`PrimitiveComponent.SetMaterial` _staticmesh 0 _data_flatmaterial)
  (`MeshComponent.SetVectorParameterValueOnMaterials` _staticmesh "Color" (`KismetMathLibrary.Conv_LinearColorToVector` (select `/Game/TacticGame/Blueprints/Core/Grid/Utilities/E_TileType` (`self.Type`) :`NewEnumerator1` (struct :`R` 1.0 :`G` 1.0 :`B` 1.0 :`A` 1.0) :`NewEnumerator2` (struct :`R` 1.0 :`A` 1.0) :`NewEnumerator3` (struct :`R` 0.701961 :`G` 0.301961 :`B` 0.2 :`A` 1.0) :`NewEnumerator4` (struct :`R` 0.8 :`G` 0.3 :`B` 0.1 :`A` 1.0) :`NewEnumerator5` (struct :`R` 0.3 :`G` 0.5 :`B` 1.0 :`A` 1.0) :!type "LinearColor Structure")))
  (`MeshComponent.SetScalarParameterValueOnMaterials` _staticmesh "IsFilled" 1.0)
  ;[1 1 1 1 16] The volume should overlap the same trace channel as the ground. We have to set it after setting the mesh, because the SetStaticMesh function resetes this setting
  (`PrimitiveComponent.SetCollisionResponseToChannel` (`self.StaticMesh`) "ECC_GameTraceChannel1" "ECR_Overlap")
  ;[1 1 1] Trace channel setting for spells Line Of Sight
  (`PrimitiveComponent.SetCollisionResponseToChannel` (`self.StaticMesh`) "ECC_GameTraceChannel4" "ECR_Block")
  (`self.SetActorHiddenInGame` true))