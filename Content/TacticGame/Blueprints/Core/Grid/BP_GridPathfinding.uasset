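; Grid pathfinder for a tactics game that finds A* paths or lists reachable tiles within a max path length.
; Neighbors are filtered by type, occupancy and height step, and only square grids are handled.
; Discovered tiles stay in parallel cost-sorted arrays, with a tie-break favoring non-diagonal steps.
; FindPath runs instantly or as a gated delay loop with optional per-frame millisecond budget, reporting through dispatchers.
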(event `FindPathWithDelay`
  ;[1 1 1] SOLUTION 1: We're using a custom event
  ; The logic will be more or less the same one of the FindPath function
  ;[1 1 1] There was a problem that kept us stuck in the handmade loop if the user selected a new path to find
  ; without delay while the old one was looping with delay.
  ; To avoid that we condition the loop with a gate that we can close anytime we want.
  ; In this case we will use a custom event that will be fired if the user select a new path to find
  (`|ExecutionSequence`
    (:`then_0`
      (goto _label_3 :!via `Open`))
    (:`then_1`
      ;[1 1 1] We need to know the time used from the beginning of the loop to decide if we reached the ms limit for this frame or we can keep going, so we read the first value here
      (set `self.LoopStartTime` (`KismetMathLibrary.Now`) :!label _label)
      ;[1 1 1] The Branch will fire every time the Delay retrigger, it behaviours like a loop but with delay
      (if (> (`KismetArrayLibrary.Array_Length` (`self.DiscoveredTileIndices`)) 0) :!label _label_2
        (bind _foundtargettile (`self.AnalyseNextDiscoveredTile`))
        ;[1 1 1] TRUE = exit loop
        ; FALSE = keep looping with delay
        (if _foundtargettile
          ;[1 1 1] If a valid path from start to target was found,
          ; we take all the analysed tiles and build a path
          (bind _path (`self.GeneratePath`))
          ;[1 1 1] Path Found!
          (`self.OnPathfindingCompleted` _path) ; Call the dispatcher
          (else
            ;[1 1 1] If we don't have a time limit
            ; we simply go back to the retriggerable delay
            (if (> (`self.MaxMsPerFrame`) 0.0)
              ;[1 1 1] If we have a limit, we check if the time since the start of the loop
              ; is lesser than the limit ms we have in input
              ; TRUE: we still have time, don't wait and keep looping (no retriggerable delay and no loop start time update)
              ; FALSE: our time has run out, we need to wait for the next loop, go wait to the retriggerable delay
              (if (< (`KismetMathLibrary.GetTotalMilliseconds` (- (`KismetMathLibrary.Now`) (`self.LoopStartTime`))) (`self.MaxMsPerFrame`))
                (goto _label_2)
                (else
                  _)))
            (`KismetSystemLibrary.RetriggerableDelay` (`self.DelayBetweenIterations`))
            (`/Engine/EditorBlueprintResources/StandardMacros.Gate` true :!label _label_3
              (:`Exit`
                (goto _label)))))
        (else
          ;[1 1 1 1 16] CASE 1: No Path found!
          ; In case we analyzed the whole Discovered Tile Array and didn't find a target tile, means that the list is empty because we analysed every possible tile of the Grid
          ; CASE 2: We are interested in the Reachable tiles.
          ; In this case we can return all the Analysed Tile Array because if a Tile is analysed it means that can be reached by the unit.
          (`self.OnPathfindingCompleted` (select `bool` (`self.ReturnReachableTiles`) :`false` (`|MakeArray`) :`true` (`self.AnalysedTileIndices`))) ; Call the dispatcher
        )))))

(event `CloseDelayGate`
  ;[1 1 1] There was a problem that kept us stuck in the handmade loop if the user selected a new path to find
  ; without delay while the old one was looping with delay.
  ; To avoid that we condition the loop with a gate that we can close anytime we want.
  ; In this case we will use a custom event that will be fired if the user select a new path to find
  (goto _label_3 :!via `Close`))

(fn `AnalyseNextDiscoveredTile`
  (returns (FoundTargetTile :type Boolean))
  ;[1 1 1] Analyse starts by choosing among the discovered tiles,
  ; the one that is closest to our target tile (cheapest)
  (bind _tilepathdata (`self.PullCheapestTileOutOfDiscoveredList`))
  (bind _output_get (set `self.CurrentDiscoveredTile` _tilepathdata))
  ;[1 1 1] Since one tile is removed from the Discovered Array
  ; and added to the Analysed Array,
  ; we call the event to update texts and states on the tile
  (`self.OnPathfindingDataUpdated` (`.Index_6_EECFBC614119C7F756F2D9ADE2713DE6` (break `/Game/TacticGame/Blueprints/Core/Grid/Utilities/S_PathfindingData` _output_get)))
  ;[1 1 1] we then get all the neighbors from the cheapest tile found
  (bind _retneighbors (`self.GetValidTileNeighbors` (`.Index_6_EECFBC614119C7F756F2D9ADE2713DE6` (break `/Game/TacticGame/Blueprints/Core/Grid/Utilities/S_PathfindingData` (`self.CurrentDiscoveredTile`))) (`self.IncludeDiagonals`) (`self.ValidTileTypes`)))
  (set `self.CurrentNeighbors` _retneighbors)
  ;[1 1 1] We loop these neighbors to check if one of them is the target tile
  (while (> (`KismetArrayLibrary.Array_Length` (`self.CurrentNeighbors`)) 0)
    ;[1 1 1] If we find the target tile, we set a bool and return
    (bind _istargettile (`self.DiscoverNextNeighbor`))
    (if _istargettile
      (return true) ; Found a neighbor that is the target tile
    ))
  ;[1 1 1] If we don't find it, we simply return
  (return false) ; None of the neighbors was the target tile
)

(fn `ClearGeneratedData`
  (`BlueprintMapLibrary.Map_Clear` (`self.PathfindingData`))
  (`KismetArrayLibrary.Array_Clear` (`self.DiscoveredTileSortingCosts`))
  (`KismetArrayLibrary.Array_Clear` (`self.DiscoveredTileIndices`))
  (`KismetArrayLibrary.Array_Clear` (`self.AnalysedTileIndices`))
  ;[1 1 1] Signal listeners attached on this dispatcher
  (`self.OnPathfindingDataCleared`))

(fn `DiscoverNextNeighbor`
  (returns (IsTargetTile :type Boolean))
  (locals (CostFromStart :type Integer :default 0) (IndexInDiscovered :type Integer :default 0))
  (bind _indexindiscovered (`local.IndexInDiscovered`))
  (bind (_index _costtoentertile) (break `/Game/TacticGame/Blueprints/Core/Grid/Utilities/S_PathfindingData` (`self.Current Neighbor`)))
  ;[1 1 1] We fetch the first element of the CurrentNeighbors Array
  (set `self.Current Neighbor` (`|GetArrayItem` (`self.CurrentNeighbors`)))
  ;[1 1 1] and we remove it because it's going to be analysed right after
  (`KismetArrayLibrary.Array_Remove` (`self.CurrentNeighbors`))
  ;[1 1 1] check if the neighbor has already been analysed
  (if (not (`KismetArrayLibrary.Array_Contains` (`self.AnalysedTileIndices`) (`.Index_6_EECFBC614119C7F756F2D9ADE2713DE6` (break `/Game/TacticGame/Blueprints/Core/Grid/Utilities/S_PathfindingData` (`self.Current Neighbor`)))))
    ;[1 1 1] we then calculate the cost from start for our neighbor
    (set `local.CostFromStart` (+ (`.CostFromStart_14_A0473B64497F4AE6C8C76FB3F0BB14FE` (break `/Game/TacticGame/Blueprints/Core/Grid/Utilities/S_PathfindingData` (`self.CurrentDiscoveredTile`))) (`.CostToEnterTile_13_49557D694BA3B92363FA079C4E692538` (break `/Game/TacticGame/Blueprints/Core/Grid/Utilities/S_PathfindingData` (`self.Current Neighbor`)))))
    ;[1 1 1] Check extra - Added after we implemented the Units
    ; For each new neighbor discovered we check that we are still within the Max Path Length allowed. If not, the neighbor is invalid for our path or unreachable if we are just displaying a Unit movement range
    (if (<= (`local.CostFromStart`) (`self.MaxPathLength`))
      ;[1 1 1] we also want to know the Index corresponding to the current neighbor
      ; inside the DiscoveredTile Array
      (bind _output_get (set `local.IndexInDiscovered` (`KismetArrayLibrary.Array_Find` (`self.DiscoveredTileIndices`) (`.Index_6_EECFBC614119C7F756F2D9ADE2713DE6` (break `/Game/TacticGame/Blueprints/Core/Grid/Utilities/S_PathfindingData` (`self.Current Neighbor`))))))
      ;[1 1 1] we then check if this neighbor is a new one
      ; or we already kwen it (FIND returns -1 if not found)
      (if (not (== _output_get -1))
        ;[1 1 1] The neighbor is not a new one, so we need to check if the info about its cost that we had memorized needs to be updated or not.
        ; To do so we retrieve the info from the PathfindingData map, update the current neighbor, and compare them with the cost from start that we have
        ; this way we make sure that we have the latest data for that specific neighbor
        (bind _output_get_2 (set `self.Current Neighbor` (`BlueprintMapLibrary.Map_Find` (`self.PathfindingData`) (`.Index_6_EECFBC614119C7F756F2D9ADE2713DE6` (break `/Game/TacticGame/Blueprints/Core/Grid/Utilities/S_PathfindingData` (`self.Current Neighbor`))))))
        (if (< (`local.CostFromStart`) (`.CostFromStart_14_A0473B64497F4AE6C8C76FB3F0BB14FE` (break `/Game/TacticGame/Blueprints/Core/Grid/Utilities/S_PathfindingData` _output_get_2)))
          ;[1 1 1] We need to update. Lest first remove old information from both
          ; DiscoveredTile and SortingCost Arrays
          (`KismetArrayLibrary.Array_Remove` (`self.DiscoveredTileIndices`) _indexindiscovered)
          (`KismetArrayLibrary.Array_Remove` (`self.DiscoveredTileSortingCosts`) _indexindiscovered)
          (else
            ;[1 1 1] nothing to update about the neighbor
            ; we simply return
            (return false))))
      ;[1 1 1] If it's a new neighbor or an old one that needs to be updated
      ; we simply use DiscoverTile with fresh data/information
      (`self.DiscoverTile` (make `/Game/TacticGame/Blueprints/Core/Grid/Utilities/S_PathfindingData` _index _costtoentertile (`local.CostFromStart`) (`self.GetMinimumCostBetweenTwoTiles` (`.Index_6_EECFBC614119C7F756F2D9ADE2713DE6` (break `/Game/TacticGame/Blueprints/Core/Grid/Utilities/S_PathfindingData` (`self.Current Neighbor`))) (`self.TargetIndex`) (`self.IncludeDiagonals`)) (`.Index_6_EECFBC614119C7F756F2D9ADE2713DE6` (break `/Game/TacticGame/Blueprints/Core/Grid/Utilities/S_PathfindingData` (`self.CurrentDiscoveredTile`)))))
      ;[1 1 1] last thing to do is check if the  current neighbor is the TargetTile or not
      (if (`KismetMathLibrary.Equal_IntPointIntPoint` (`.Index_6_EECFBC614119C7F756F2D9ADE2713DE6` (break `/Game/TacticGame/Blueprints/Core/Grid/Utilities/S_PathfindingData` (`self.Current Neighbor`))) (`self.TargetIndex`))
        (return true) ; We are on the target, pathfinding stops
        (else
          (return false) ; We are not on the target, pathfinding continues
        ))
      (else
        ;;[1 1 1 1 16] nothing to update about the neighbor. We simply return
        (return false)))
    (else
      (return false))))

(fn `DiscoverTile`
  (params (TilePathData :type "/Game/TacticGame/Blueprints/Core/Grid/Utilities/S_PathfindingData Structure"))
  (bind _index (break `/Game/TacticGame/Blueprints/Core/Grid/Utilities/S_PathfindingData` TilePathData))
  ;[1 1 1] We add the tile to the PathfindingData map
  (`BlueprintMapLibrary.Map_Add` (`self.PathfindingData`) _index TilePathData)
  ;[1 1 1] We update the DiscoveredArray with the new Tile.
  ; NB. The insert must follow a precise order, the list is sorted by distance from TargetTile
  (`self.InsertTileInDiscoveredArray` (`local.TilePathData`))
  ;[1 1 1] Signals the listeners attached to this dispatcher
  (`self.OnPathfindingDataUpdated` _index))

(fn `FindPath`
  (params (Start :type "IntPoint Structure") (Target :type "IntPoint Structure") (Diagonals :type Boolean) (TileTypes :type "Array of /Game/TacticGame/Blueprints/Core/Grid/Utilities/E_TileType Enum") (Delay :type "Float (double-precision)") (MaxMs :type "Float (double-precision)") (ReturnReachables :type Boolean) (PathLenght :type Integer))
  (returns (Path :type "Array of IntPoint Structure"))
  (bind _array (`|MakeArray`))
  (bind _returnvalue (select `bool` (`self.ReturnReachableTiles`) :`false` (`|MakeArray`) :`true` (`self.AnalysedTileIndices`)))
  (set `self.StartIndex` Start)
  (set `self.TargetIndex` Target)
  (set `self.IncludeDiagonals` Diagonals)
  (set `self.ValidTileTypes` TileTypes)
  (set `self.DelayBetweenIterations` Delay)
  (set `self.MaxMsPerFrame` MaxMs)
  (set `self.ReturnReachableTiles` ReturnReachables)
  (set `self.MaxPathLength` PathLenght)
  ;[1 1 1] If there was a PathFinding with delay in action,
  ; we signal the gate to close to avoid being stuck
  (`self.CloseDelayGate`)
  (`self.ClearGeneratedData`) ; Clear old data from previous pathfinding
  ;[1 1 1] Before finding the path,
  ; We check if the Indices are valid
  (bind _isvalid (`self.IsInputDataValid`))
  (if _isvalid
    ;[1 1 1] The Algorithm starts by discovering the first Tile (StartTile added to DiscoveredArray)
    (`self.DiscoverTile` (make `/Game/TacticGame/Blueprints/Core/Grid/Utilities/S_PathfindingData` (`self.StartIndex`) 1 0 (`self.GetMinimumCostBetweenTwoTiles` (`self.StartIndex`) (`self.TargetIndex`) (`self.IncludeDiagonals`))))
    ;[1 1 1] If we need to handle Delay, we call the FindPathWithDelay custom event, and exit from FindPath
    ; otherwise we keep going with the normal flow (looping)
    (if (<= (`self.DelayBetweenIterations`) 0.0)
      ;[1 1 1] The while loop keeps analyzing tiles until there are no one left in the Discovered List (length becomes = 0)
      ; Remember that the analyse function also pulls tiles from the discovered array (the cheapest one for each loop)
      (while (> (`KismetArrayLibrary.Array_Length` (`self.DiscoveredTileIndices`)) 0)
        (bind _foundtargettile (`self.AnalyseNextDiscoveredTile`))
        ;[1 1 1] A valid path from start to target was found,
        ; so we take all the analysed tiles and  build a path
        (if _foundtargettile
          (bind _path (`self.GeneratePath`))
          ;[1 1 1] Path Found!
          (`self.OnPathfindingCompleted` _path) ; In case we need to handle Delay
          (return _path) ; No delay
        ))
      ;[1 1 1] CASE 1: No Path found!
      ; In case we analyzed the whole Discovered Tile Array and didn't find a target tile, means that the list is empty because we analysed every possible tile of the Grid
      ; CASE 2: We are interested in the Reachable tiles.
      ; In this case we can return all the Analysed Tile Array because if a Tile is analysed it means that can be reached by the unit.
      (`self.OnPathfindingCompleted` _returnvalue) ; In case we need to handle Delay
      (return _returnvalue) ; No delay
      (else
        (`self.FindPathWithDelay`)
        (return (`|MakeArray`))))
    (else
      ;[1 1 1] If the Indices are not valid, we return an empty path
      (`self.OnPathfindingCompleted` _array) ; In case we need to handle Delay
      (return _array) ; No delay
    )))

(fn `GeneratePath`
  (returns (Path :type "Array of IntPoint Structure"))
  (locals (CurrentTile :type "IntPoint Structure") (InvertedPath :type "Array of IntPoint Structure") (ReturnPath :type "Array of IntPoint Structure"))
  ;[1 1 1] To generate our path we start from the end (the Target Tile)...
  (set `local.CurrentTile` (`self.TargetIndex`))
  ;[1 1 1] ...and go all the way back to the Starting Tile
  (while (!= (`local.CurrentTile`) (`self.StartIndex`))
    ;[1 1 1] While going all the way back
    ; we build a new Inverted Array with the tiles we find in the Pathfinding Data
    (`KismetArrayLibrary.Array_Add` (`local.InvertedPath`) (`local.CurrentTile`))
    ;[1 1 1] CurrentTile is set to PreviousTile, so the loop goes backwards
    (set `local.CurrentTile` (`.PreviousIndex_12_2F9B35294E9DBD1C39976D851970B89B` (break `/Game/TacticGame/Blueprints/Core/Grid/Utilities/S_PathfindingData` (`BlueprintMapLibrary.Map_Find` (`self.PathfindingData`) (`local.CurrentTile`))))))
  ;[1 1 1] After the loop, the InvertedPath is filled from end to start
  ; so we reverse-loop it to build the final path in the correct direction
  (bind (_arrayindex _arrayelement) (`/Engine/EditorBlueprintResources/StandardMacros.ReverseForEachLoop` (`local.InvertedPath`))
    (:`LoopBody`
      (`KismetArrayLibrary.Array_Add` (`local.ReturnPath`) _arrayelement))
    (:`Completed`
      (return (`local.ReturnPath`)))))

(fn `GetMinimumCostBetweenTwoTiles`
  (params (Index1 :type "IntPoint Structure") (Index2 :type "IntPoint Structure") (Diagonals :type Boolean))
  (returns (MinCost :type Integer))
  (bind (_returnvalue_x _returnvalue_y) (break `IntPoint` (- (`local.Index1`) (`local.Index2`))))
  (bind (_returnvalue_x_2 _returnvalue_y_2) (break `IntPoint` (- (`local.Index1`) (`local.Index2`))))
  (switch `/Game/TacticGame/Blueprints/Core/Grid/GridShapes/E_GridShape` (`/Game/TacticGame/Blueprints/Core/Grid/BP_Grid.GridShape` (`self.Grid`))
    (:`NewEnumerator1`
      (if (`local.Diagonals`)
        ;[1 1 1] Cost with diagonals, is the max between the distance along X coord. and along Y coord.
        (return (`KismetMathLibrary.Max` (`KismetMathLibrary.Abs_Int` _returnvalue_x_2) (`KismetMathLibrary.Abs_Int` _returnvalue_y_2)))
        (else
          ;[1 1 1] Cost without diagonals, is the sum of the distance along X coord. and along Y coord.
          (return (+ (`KismetMathLibrary.Abs_Int` _returnvalue_x) (`KismetMathLibrary.Abs_Int` _returnvalue_y))))))))

(fn `GetNeighborIndicesForSquare`
  (params (Index :type "IntPoint Structure") (IncludeDiagonals :type Boolean))
  (returns (Neighbors :type "Array of IntPoint Structure"))
  (locals (RetNeighbors :type "Array of IntPoint Structure"))
  (bind _array (`|MakeArray` (+ (`local.Index`) (make `IntPoint` 1)) (+ (`local.Index`) (make `IntPoint` 0 1)) (+ (`local.Index`) (make `IntPoint` -1)) (+ (`local.Index`) (make `IntPoint` 0 -1))))
  (if IncludeDiagonals
    (bind _output_get (set `local.RetNeighbors` _array))
    (`KismetArrayLibrary.Array_Append` _output_get (`|MakeArray` (+ (`local.Index`) (make `IntPoint` 1 1)) (+ (`local.Index`) (make `IntPoint` -1 1)) (+ (`local.Index`) (make `IntPoint` -1 -1)) (+ (`local.Index`) (make `IntPoint` 1 -1))))
    (return (`local.RetNeighbors`))
    (else
      (return _array))))

(fn `GetNeighborsIndices`
  (params (Index :type "IntPoint Structure") (IncludeDiagonals :type Boolean))
  (returns (Neighbors :type "Array of IntPoint Structure"))
  (switch `/Game/TacticGame/Blueprints/Core/Grid/GridShapes/E_GridShape` (`/Game/TacticGame/Blueprints/Core/Grid/BP_Grid.GridShape` (`self.Grid`))
    (:`NewEnumerator1`
      (return (`self.GetNeighborIndicesForSquare` (`local.Index`) (`local.IncludeDiagonals`))))))

(fn `GetPathCost`
  (params (Path :type "Array of IntPoint Structure"))
  (returns (Cost :type Integer))
  (locals (Ret :type Integer :default 0))
  (set `local.Ret` 0) ; Reset the count
  ;[1 1 1] For each Tile in the Path, get its cost and add it to the total
  (for _array_element (`local.Path`)
    (set `local.Ret` (+ (`local.Ret`) (`/Game/TacticGame/Blueprints/Core/Grid/Utilities/BFL_TileData.GetTileTypeCost` (`.Type_8_8F74F19243475FAB39F94AA272B2F514` (break `/Game/TacticGame/Blueprints/Core/Grid/Utilities/S_TileData` (`BlueprintMapLibrary.Map_Find` (`/Game/TacticGame/Blueprints/Core/Grid/BP_Grid.GridTiles` (`self.Grid`)) _array_element)))))))
  (return (`local.Ret`)) ; Returns the cost of the whole Path
)

(fn `GetTileSortingCost`
  (params (TileData :type "/Game/TacticGame/Blueprints/Core/Grid/Utilities/S_PathfindingData Structure (by ref)"))
  (returns (Cost :type Integer))
  (bind (_index _costtoentertile _costfromstart _minimumcosttotarget _previousindex) (break `/Game/TacticGame/Blueprints/Core/Grid/Utilities/S_PathfindingData` TileData))
  (bind (_index_2 _costtoentertile_2 _costfromstart_2 _minimumcosttotarget_2) (break `/Game/TacticGame/Blueprints/Core/Grid/Utilities/S_PathfindingData` TileData))
  (return (+ (* (+ _costfromstart_2 _minimumcosttotarget_2) 2) (`KismetMathLibrary.Conv_BoolToInt` (`self.IsTileDiagonal` _index _previousindex)))))

(fn `GetValidTileNeighbors`
  (params (Index :type "IntPoint Structure") (IncludeDiagonals :type Boolean) (ValidTypes :type "Array of /Game/TacticGame/Blueprints/Core/Grid/Utilities/E_TileType Enum"))
  (returns (RetNeighbors :type "Array of /Game/TacticGame/Blueprints/Core/Grid/Utilities/S_PathfindingData Structure"))
  (locals (Data :type "/Game/TacticGame/Blueprints/Core/Grid/Utilities/S_TileData Structure") (InputData :type "/Game/TacticGame/Blueprints/Core/Grid/Utilities/S_TileData Structure") (ValidIndices :type "Array of /Game/TacticGame/Blueprints/Core/Grid/Utilities/S_PathfindingData Structure"))
  (bind (_data_index _data_type _data_transform) (break `/Game/TacticGame/Blueprints/Core/Grid/Utilities/S_TileData` (`local.Data`)))
  (bind (_inputdata_index _inputdata_type _inputdata_transform) (break `/Game/TacticGame/Blueprints/Core/Grid/Utilities/S_TileData` (`local.InputData`)))
  (bind (_data_index_2 _data_type_2) (break `/Game/TacticGame/Blueprints/Core/Grid/Utilities/S_TileData` (`local.Data`)))
  (bind (_data_index_3 _data_type_3) (break `/Game/TacticGame/Blueprints/Core/Grid/Utilities/S_TileData` (`local.Data`)))
  (bind (_data_index_4 _data_type_4 _data_transform_2 _data_states _data_unitontile) (break `/Game/TacticGame/Blueprints/Core/Grid/Utilities/S_TileData` (`local.Data`)))
  (bind (_gridtilesize_x _gridtilesize_y _gridtilesize_z) (`KismetMathLibrary.BreakVector` (`/Game/TacticGame/Blueprints/Core/Grid/BP_Grid.GridTileSize` (`self.Grid`))))
  ;[1 1 1] We need the Data for the tile corresponding to the index in Input
  ; to compare it later with its neighbors
  (set `local.InputData` (`BlueprintMapLibrary.Map_Find` (`/Game/TacticGame/Blueprints/Core/Grid/BP_Grid.GridTiles` (`self.Grid`)) (`local.Index`)))
  ;[1 1 1] Then we find neighbors indices
  (bind _neighbors (`self.GetNeighborsIndices` (`local.Index`) (`local.IncludeDiagonals`)))
  ;[1 1 1] Before returning the Neighbors Indices, we access their data to check if they need to be discarded
  (for _array_element _neighbors
    (set `local.Data` (`BlueprintMapLibrary.Map_Find` (`/Game/TacticGame/Blueprints/Core/Grid/BP_Grid.GridTiles` (`self.Grid`)) _array_element))
    ;[1 1 1] Check 1 - The tile must be in the Valid Types array
    (if (`KismetArrayLibrary.Array_Contains` (`local.ValidTypes`) _data_type_3)
      ;[1 1 1] Check 1b - Added after we implemented the Units
      ; We need to check that the Tile is free and not occupied by anothe unit.
      ; To accomplish this we check that the Unit on the neighbor is not valid (so there is none)
      (if (not (`KismetSystemLibrary.IsValid` _data_unitontile))
        ;[1 1 1] Check 2 - We compare the height (Z coordinate) of the Tile in input with its Neighbors.
        ; If the difference is too steep (bigger than the Grid Tile Size along Z),
        ; then we don't consider that neighbor valid
        (if (<= (`KismetMathLibrary.Abs` (- (`.Z` (`KismetMathLibrary.BreakVector3f` (.location _inputdata_transform))) (`.Z` (`KismetMathLibrary.BreakVector3f` (.location _data_transform))))) _gridtilesize_z)
          ;[1 1 1] All checks passed, add the index to the valid neighbors array
          ; taking into account the proper cost to enter the tile
          (`KismetArrayLibrary.Array_Add` (`local.ValidIndices`) (make `/Game/TacticGame/Blueprints/Core/Grid/Utilities/S_PathfindingData` _data_index_2 (`/Game/TacticGame/Blueprints/Core/Grid/Utilities/BFL_TileData.GetTileTypeCost` _data_type_2) 999999 999999 (`local.Index`)))))))
  ;[1 1 1] At the end, we return all the valid neighbors
  (return (`local.ValidIndices`)))

(fn `InsertTileInDiscoveredArray`
  (params (TileData :type "/Game/TacticGame/Blueprints/Core/Grid/Utilities/S_PathfindingData Structure"))
  (locals (SortingCost :type Integer :default 0))
  (bind _discoveredtilesortingcosts (`self.DiscoveredTileSortingCosts`))
  ;[1 1 1] First, we calculate the sorting cost for the Tile examined.
  (set `local.SortingCost` (`self.GetTileSortingCost` TileData))
  ;[1 1 1] We check if the SortingCost Array is empty
  (if (== (`KismetArrayLibrary.Array_Length` (`self.DiscoveredTileSortingCosts`)) 0)
    ;[1 1 1] If empty, there is no need to perform a sorted insert
    ; so we just add the Tile to both the SortingCost and DiscoveredTiles Arrays
    (`KismetArrayLibrary.Array_Add` (`self.DiscoveredTileSortingCosts`) (`local.SortingCost`) :!label _label)
    (`KismetArrayLibrary.Array_Add` (`self.DiscoveredTileIndices`) (`.Index_6_EECFBC614119C7F756F2D9ADE2713DE6` (break `/Game/TacticGame/Blueprints/Core/Grid/Utilities/S_PathfindingData` (`local.TileData`))))
    (else
      ;[1 1 1] SortingCost Array not empty. We need to perform a sorted insert!
      ;;[1 1 1] Optimization 1 - If the Sorting cost is bigger than the last element, we don't need to loop the whole array.
      ;; We can just insert the new cost/tile as last element of both arrays
      (if (>= (`local.SortingCost`) (`|GetArrayItem` _discoveredtilesortingcosts (`KismetArrayLibrary.Array_LastIndex` _discoveredtilesortingcosts)))
        (goto _label)
        (else
          ;;[1 1 1] Expensive part of the Algorithm, we must loop the array to find the right position for the insert
          (for (_array_element _array_index) (`self.DiscoveredTileSortingCosts`)
            ;;[1 1 1] As soon as we find an element of SortingCost >=
            ;; than the one we want to add, we STOP THE LOOP and insert the new one IN FRONT of it
            (if (>= _array_element (`local.SortingCost`))
              ;;[1 1 1] Insert by Index in both Arrays, and SIGNAL the BREAK of the LOOP
              (`KismetArrayLibrary.Array_Insert` (`self.DiscoveredTileSortingCosts`) (`local.SortingCost`) _array_index)
              (`KismetArrayLibrary.Array_Insert` (`self.DiscoveredTileIndices`) (`.Index_6_EECFBC614119C7F756F2D9ADE2713DE6` (break `/Game/TacticGame/Blueprints/Core/Grid/Utilities/S_PathfindingData` (`local.TileData`))) _array_index)
              (break))))))))

(fn `IsInputDataValid`
  (returns (IsValid :type Boolean))
  (bind (_index _type _transform _states _unitontile) (break `/Game/TacticGame/Blueprints/Core/Grid/Utilities/S_TileData` (`BlueprintMapLibrary.Map_Find` (`/Game/TacticGame/Blueprints/Core/Grid/BP_Grid.GridTiles` (`self.Grid`)) (`self.TargetIndex`))))
  ;[1 1 1] Check 1 - Start and Target Tile should not be the same
  (if (!= (`self.StartIndex`) (`self.TargetIndex`))
    ;[1 1 1] Check 2 - Starting and Target Tile must be walkable
    (if (`/Game/TacticGame/Blueprints/Core/Grid/BP_Grid.IsTileWalkable` (`self.Grid`) (`self.StartIndex`))
      ;[1 1 1] Check extra - Added later for Reachable Tiles.
      ; When we're just interested in reachable tiles, we don't care about the target tile (index), so we can stop here and return a valid list of reachable tiles (false branch).
      ; Otherwise (return reachable tiles == false) we keep the normal flow of execution with all the checks and the pathfinding
      (if (not (`self.ReturnReachableTiles`))
        (if (`/Game/TacticGame/Blueprints/Core/Grid/BP_Grid.IsTileWalkable` (`self.Grid`) (`self.TargetIndex`))
          ;[1 1 1] Check extra - Added after we implemented the Units
          ; We make sure that the total distance from start to finish is less or equal than the max path length allowed. This is useful both for the Unit to limit their movement and for the Reachable Tiles to limit them
          (if (<= (`self.GetMinimumCostBetweenTwoTiles` (`self.StartIndex`) (`self.TargetIndex`) (`self.IncludeDiagonals`)) (`self.MaxPathLength`))
            ;[1 1 1] Check 3 - The Target Tile must be of a valid type
            (if (`KismetArrayLibrary.Array_Contains` (`self.ValidTileTypes`) _type)
              ;[1 1 1] Check extra - Added after we implemented the Units
              ; We need to check that the Tile is free and not occupied by anothe unit.
              ; To accomplish this we check that the Unit on the neighbor is not valid (so there is none)
              (if (not (`KismetSystemLibrary.IsValid` _unitontile))
                (return true) ; Valid!
                (else
                  (return false) ; Not Valid!
                ))
              (else
                (return false) ; Not Valid!
              ))
            (else
              (return false) ; Not Valid!
            ))
          (else
            (return false) ; Not Valid!
          ))
        (else
          (return true) ; Not Valid!
        ))
      (else
        (return false) ; Not Valid!
      ))
    (else
      (return false) ; Not Valid!
    )))

(fn `IsTileDiagonal`
  (params (Index1 :type "IntPoint Structure") (Index2 :type "IntPoint Structure"))
  (returns (IsDiagonal :type Boolean))
  ;[1 1 1] We check if the second tile is among the NON-DIAGONAL neighbors of the first tile
  (bind _neighbors (`self.GetNeighborsIndices` Index1))
  (return (not (`KismetArrayLibrary.Array_Contains` _neighbors Index2))))

(fn `PullCheapestTileOutOfDiscoveredList`
  (returns (TilePathData :type "/Game/TacticGame/Blueprints/Core/Grid/Utilities/S_PathfindingData Structure"))
  (locals (TileIndex :type "IntPoint Structure"))
  ;[1 1 1] We set TileIndex with the first element (0) of the DiscoveredArray.
  ; Being sorted by cost, the first element is always the cheapest
  (set `local.TileIndex` (`|GetArrayItem` (`self.DiscoveredTileIndices`)))
  ;[1 1 1] We update the Discovered Array by removing the element.
  ; And since the 2 arrays MUST ALWAYS BE UPDATED TOGETHER
  ; we remove the cheapest element (0) from both the Indices and the SortingCost aArray
  (`KismetArrayLibrary.Array_Remove` (`self.DiscoveredTileIndices`))
  (`KismetArrayLibrary.Array_Remove` (`self.DiscoveredTileSortingCosts`))
  ;[1 1 1] The Tile is then added to the Analysed Array
  (`KismetArrayLibrary.Array_Add` (`self.AnalysedTileIndices`) (`local.TileIndex`))
  ;[1 1 1] We retrieve the Structure relative to the cheapest tile and return it
  (return (`BlueprintMapLibrary.Map_Find` (`self.PathfindingData`) (`local.TileIndex`))))

(fn `UserConstructionScript`)