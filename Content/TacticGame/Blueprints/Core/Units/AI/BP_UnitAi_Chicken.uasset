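; Unit AI for the Chicken in the tactics game, which treats the RunChickenRun spell as a fallback.
; It removes that spell from the parent's available spells, keeping it out of the normal spell choice.
; When the decision step finds no valid spell and the unit can cast RunChickenRun, it injects it into the casting data as a self-targeted cast.
; The parent's generic spellcasting flow then continues.
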(event `self.DecideWitchSpellToCast_Done`
  (bind _index (`/Game/TacticGame/Blueprints/Core/Units/BP_Unit.Index` (`self.Unit`)))
  ;[1 1 1] REMEMBER: We arrived here with the AI flow
  ; in witch we removed RunChickenRun from the available spell
  (`|ExecutionSequence`
    (:`then_0`
      ;[1 1 1] so if we didn't find a valid Spell to cast...
      (if (not (`.IsSpellValid_6_CD3DFEE64ED7C34E7FE6879B8CEAAA89` (break `/Game/TacticGame/Blueprints/Core/Units/AI/S_UnitAiSpellCastingData` (`self.AiSpellCasting`))))
        ;[1 1 1] ...we ask if the Unit is able to cast it...
        (bind _spelldata (`/Game/TacticGame/Blueprints/Core/Combat/Spells/Utilities/BFL_Spells.GetSpellDataFromSpell` "NewEnumerator10"))
        (bind _cancast (`/Game/TacticGame/Blueprints/Core/Units/BP_Unit.CanCastSpell` (`self.Unit`) _spelldata))
        (if _cancast
          ;[1 1 1] If the Unit can cast it, then we inject it manually in the Struct used to cast in the next AI flow step
          (set `self.AiSpellCasting` (make `/Game/TacticGame/Blueprints/Core/Units/AI/S_UnitAiSpellCastingData` true "NewEnumerator10" _index _index)))))
    (:`then_1`
      (`parent.DecideWitchSpellToCast_Done`) ; Continue with generic AI spellcasting
    )))

(fn `GetAvailableSpells`
  (returns (AvailableSpells :type "Array of /Game/TacticGame/Blueprints/Core/Combat/Spells/Utilities/E_Spell Enum"))
  (locals (Ret :type "Array of /Game/TacticGame/Blueprints/Core/Combat/Spells/Utilities/E_Spell Enum"))
  ;[1 1 1] We remove the RunChickenRun from the available Spell
  ; when not needed to reach the Target
  (bind _output_get (set `local.Ret` (`parent.GetAvailableSpells`)))
  (`KismetArrayLibrary.Array_RemoveItem` _output_get "NewEnumerator10")
  (return (`local.Ret`)))

(fn `UserConstructionScript`
  (`parent.UserConstructionScript`))