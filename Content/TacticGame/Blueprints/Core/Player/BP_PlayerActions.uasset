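; Player input hub for the tactics game, turning cursor hover and clicks into tile and unit selection on the CombatSystem's grid.
; Each tick it resolves the hovered unit, which widgets can override, and its tile.
; Left and right clicks, or hover changes, drive swappable action actors spawned by SetSelectedAction.
; Combat events switch move, cast-spell and wait-for-AI actions, sync selection, and manage the combat and end-screen widgets.
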(event `self.ReceiveBeginPlay`
  (bind _grid (`self.Grid`))
  (bind _combatsystem (`self.CombatSystem`))
  (bind _combatsystem_2 (`self.CombatSystem`))
  ;[1 1 1 1 16] As soon as the game begins,
  ; we set the Grid reference with the one in the CombatSystem variable
  ; NB. The CombatSystem is manually set as reference from the inspector in the Editor
  (set `self.Grid` (`/Game/TacticGame/Blueprints/Core/Combat/BP_CombatSystem.Grid` (`self.CombatSystem`)))
  ;[1 1 1 1 16] We bind on the Grid Generated and Tile Updated dispatchers to update the Grid if it gets regenerated with particular conditions
  ; Es.with a Unit selected (we need to keep also the Tile selecation in this case), etc.
  (add `/Game/TacticGame/Blueprints/Core/Grid/BP_Grid.OnGridGenerated` _grid (`|CreateDelegate` :!event `OnGridGenerated`))
  (add `/Game/TacticGame/Blueprints/Core/Grid/BP_Grid.OnTileDataUpdated` _grid (`|CreateDelegate` :!event `OnTileDataUpdated`))
  ;[1 1 1] If a Unit position changes, we need to update the Selected Tile, so we bind to the event to get notified when this happens
  (add `/Game/TacticGame/Blueprints/Core/Combat/BP_CombatSystem.OnUnitGridIndexChanged` (`self.CombatSystem`) (`|CreateDelegate` :!event `OnUnitGridIndexChanged`))
  ;[1 1 1] When the Combat starts/end we want to limit/restore the action the player can do
  (add `/Game/TacticGame/Blueprints/Core/Combat/BP_CombatSystem.OnCombatStarted` _combatsystem_2 (`|CreateDelegate` :!event `OnCombatStarted`)) ; We want be notified when the Combat starts
  (add `/Game/TacticGame/Blueprints/Core/Combat/BP_CombatSystem.OnCombatEnded` _combatsystem_2 (`|CreateDelegate` :!event `OnCombatEnded`)) ; We want be notified when the Combat ends
  ;[1 1 1] We need to know when the Units start/end their turns
  ; to keep the correct Unit selected
  (add `/Game/TacticGame/Blueprints/Core/Combat/BP_CombatSystem.OnUnitTurnStarted` _combatsystem (`|CreateDelegate` :!event `OnUnitTurnStarted`))
  (add `/Game/TacticGame/Blueprints/Core/Combat/BP_CombatSystem.OnUnitTurnEnded` _combatsystem (`|CreateDelegate` :!event `OnUnitTurnEnded`))
  ;[1 1 1] We need to know when the combat finishes
  ; to show the combat over screen
  (add `/Game/TacticGame/Blueprints/Core/Combat/BP_CombatSystem.OnCombatFinishing` (`self.CombatSystem`) (`|CreateDelegate` :!event `OnCombatFinishing`))
  ;[1 1 1] To enable mouse click for the Player Controller
  (`self.EnableInput` (`GameplayStatics.GetPlayerController` 0)))

(event `self.ReceiveTick`
  (params (DeltaSeconds :type "Float (single-precision)"))
  (`self.UpdateHoveredTileAndUnit`))

(event `Key|LeftMouseButton`
  (params (Key :type "Key Structure")))

(event `EnhancedInput|/Game/TacticGame/Blueprints/Core/Player/Inputs/IA_Actions_LeftClick`
  (params (ActionValue :type Boolean) (ElapsedSeconds :type "Float (double-precision)") (TriggeredSeconds :type "Float (double-precision)") (InputAction :type "InputAction Object Reference" :default "/Game/TacticGame/Blueprints/Core/Player/Inputs/IA_Actions_LeftClick.IA_Actions_LeftClick"))
  ;[1 1 1] Mouse left click to perform action on a tile
  (:`Triggered`
    (if ActionValue
      (`self.UpdateHoveredTileAndUnit` :!label _label) ; to force the update if player clicks too fast
      (set `self.IsLeftClickDown` true)
      (`/Engine/EditorBlueprintResources/StandardMacros.IsValid` (`self.SelectedAction_LeftClick`) ; Check if we have a selected action for the left click
        (:`Is Valid`
          (`/Game/TacticGame/Blueprints/Core/Player/Actions/BP_Action.ExecuteAction` (`self.SelectedAction_LeftClick`) (`self.HoveredTile`) :!label _label_2)))
      (else
        (set `self.IsLeftClickDown` false :!label _label_3)))))

(event `Event_SimulateLeftClickForExternalSource`
  ;[1 1 1] Mouse left click to perform action on a tile
  (`|ExecutionSequence`
    (:`then_0`
      (goto _label))
    (:`then_1`
      (goto _label_3))))

(event `Event_ExecuteActionWhenHoveredTileChanged`
  ;[1 1 1] When the mouse cursor moves on a new tile while a specific action is selected
  (`|ExecutionSequence`
    (:`then_0`
      (`/Engine/EditorBlueprintResources/StandardMacros.IsValid` (`self.SelectedAction_LeftClick`) ; Check if we have a selected action for the left click
        (:`Is Valid`
          ;[1 1 1] This action is executed on hovered, no need for the player to click
          (`/Game/TacticGame/Blueprints/Core/Player/Actions/BP_Action.ExecuteHoveredAction` (`self.SelectedAction_LeftClick`) (`self.HoveredTile`))
          (if (`self.IsLeftClickDown`)
            (goto _label_2)))))
    (:`then_1`
      (`/Engine/EditorBlueprintResources/StandardMacros.IsValid` (`self.SelectedAction_RightClick`) ; Check if we have a selected action for the right click
        (:`Is Valid`
          (`/Game/TacticGame/Blueprints/Core/Player/Actions/BP_Action.ExecuteHoveredAction` (`self.SelectedAction_RightClick`) (`self.HoveredTile`))
          (if (`self.IsRightClickDown`)
            ;[1 1 1] Mouse right click to perform action on a tile
            (`/Game/TacticGame/Blueprints/Core/Player/Actions/BP_Action.ExecuteAction` (`self.SelectedAction_RightClick`) (`self.HoveredTile`) :!label _label_4)))))))

(event `Key|RightMouseButton`
  (params (Key :type "Key Structure")))

(event `EnhancedInput|/Game/TacticGame/Blueprints/Core/Player/Inputs/IA_Actions_RightClick`
  (params (ActionValue :type Boolean) (ElapsedSeconds :type "Float (double-precision)") (TriggeredSeconds :type "Float (double-precision)") (InputAction :type "InputAction Object Reference" :default "/Game/TacticGame/Blueprints/Core/Player/Inputs/IA_Actions_RightClick.IA_Actions_RightClick"))
  ;[1 1 1] Mouse right click to perform action on a tile
  (:`Triggered`
    (if ActionValue
      (`self.UpdateHoveredTileAndUnit`) ; to force the update if player clicks too fast
      (set `self.IsRightClickDown` true)
      (`/Engine/EditorBlueprintResources/StandardMacros.IsValid` (`self.SelectedAction_RightClick`) ; Check if we have a selected action for the right click
        (:`Is Valid`
          (goto _label_4)))
      (else
        (set `self.IsRightClickDown` false)))))

(event `Key|AnyKey` :consume false
  (params (Key :type "Key Structure")))

(event `EnhancedInput|/Game/TacticGame/Blueprints/Core/Player/Inputs/IA_Actions_SelectSpell`
  (params (ActionValue :type "Float (double-precision)") (ElapsedSeconds :type "Float (double-precision)") (TriggeredSeconds :type "Float (double-precision)") (InputAction :type "InputAction Object Reference" :default "/Game/TacticGame/Blueprints/Core/Player/Inputs/IA_Actions_SelectSpell.IA_Actions_SelectSpell"))
  (bind _combatsystem (`self.CombatSystem`))
  ;[1 1 1] Select the Spell in Combat using the numbers
  (:`Triggered`
    (if (and (`/Game/TacticGame/Blueprints/Core/Combat/BP_CombatSystem.IsInCombat` _combatsystem) (not (`/Game/TacticGame/Blueprints/Core/Combat/BP_CombatSystem.IsFinishingCombat` _combatsystem)) (== (`/Game/TacticGame/Blueprints/Core/Combat/BP_CombatSystem.CurrentUnit` _combatsystem) (`self.SelectedUnit`)))
      (`/Game/TacticGame/Blueprints/Core/Combat/Spells/Widgets/WBP_ButtonList_Spell.SetSelectedSpellFromIndex` (`/Game/TacticGame/Blueprints/Core/Combat/Widgets/WBP_Combat.ButtonList_Spell` (`self.W_Combat`)) (- (`KismetMathLibrary.Round` ActionValue) 1)))))

(fn `CanHoverEmptySpace`
  (returns (TraceEmptySpace :type Boolean))
  (return (`KismetArrayLibrary.Array_Contains` (`|MakeArray` (`GameplayStatics.GetObjectClass` (`self.SelectedAction_LeftClick`)) (`GameplayStatics.GetObjectClass` (`self.SelectedAction_RightClick`))) "/Game/TacticGame/Blueprints/Core/Player/Actions/Grid/BP_Action_AddTile.BP_Action_AddTile_C")))

(fn `CanHoverGround`
  (returns (TraceForGround :type Boolean))
  (return false))

(fn `GetUnitUnderCursor`
  (params (PlayerIndex :type Integer))
  (returns (Unit :type "/Game/TacticGame/Blueprints/Core/Units/BP_Unit Object Reference"))
  (bind (_hitresult _returnvalue) (`PlayerController.GetHitResultUnderCursorByChannel` (`GameplayStatics.GetPlayerController` PlayerIndex) "TraceTypeQuery5" true))
  (if _returnvalue
    ;[1 1 1] If the mouse was on a Unit, we return it
    (bind _asbp_unit (cast `/Game/TacticGame/Blueprints/Core/Units/BP_Unit` (`.HitActor` (`GameplayStatics.BreakHitResult` _hitresult))))
    (return _asbp_unit)
    (else
      ;[1 1 1] If instead the cursor was on a tile, we try to return the Unit on that tile (if one exists)
      (bind _index (`/Game/TacticGame/Blueprints/Core/Grid/BP_Grid.GetTileIndexUnderCursor` (`self.Grid`) (`local.PlayerIndex`) (`self.CanHoverGround`) (`self.CanHoverEmptySpace`)))
      (return (`.UnitOnTile_16_1A24A24A4845A31FB93E7BBEC72A5FD3` (break `/Game/TacticGame/Blueprints/Core/Grid/Utilities/S_TileData` (`BlueprintMapLibrary.Map_Find` (`/Game/TacticGame/Blueprints/Core/Grid/BP_Grid.GridTiles` (`self.Grid`)) _index)))) ; If there is no Unit on that Tile, the return Unit will be null
    )))

(fn `OnCombatEnded`
  ;[1 1 1] Remove the combat over widget and clear its variable
  (`Widget.RemoveFromParent` (`self.W_CombatEndScreen`))
  (set `self.W_CombatEndScreen` null)
  ;[1 1 1] We deselect any pending action
  (`self.SetSelectedAction` null))

(fn `OnCombatFinishing`
  (`self.SetSelectedAction` null) ; Deselect any current action
  (`self.SetSelectedTileAndUnit` (make `IntPoint` -999 -999)) ; Deselect any eventual Tile/Unit
  ;[1 1 1] Remove the Combat UI from screen and reset the widget variable
  (`Widget.RemoveFromParent` (`self.W_Combat`))
  (set `self.W_Combat` null)
  ;[1 1 1] Show the combat over widget with the winning team
  (bind _returnvalue (`|CreateWidget` "/Game/TacticGame/Blueprints/Core/Combat/Widgets/WBP_Combat_EndScreen.WBP_Combat_EndScreen_C" null self (`/Game/TacticGame/Blueprints/Core/Combat/BP_CombatSystem.TeamIndexThatWonLastCombat` (`self.CombatSystem`))))
  (bind _output_get (set `self.W_CombatEndScreen` _returnvalue))
  (`UserWidget.AddToPlayerScreen` _output_get 0))

(fn `OnCombatStarted`
  (`self.SetSelectedAction` null) ; Deselect any current action
  (`self.SetSelectedTileAndUnit` (make `IntPoint` -999 -999)) ; Deselect any eventual Tile/Unit
  ;[1 1 1] Combat has his own UI, when it starts we create the apposite widget, set it in a variable and show UI on screen
  (bind _returnvalue (`|CreateWidget` "/Game/TacticGame/Blueprints/Core/Combat/Widgets/WBP_Combat.WBP_Combat_C" null self))
  (bind _output_get (set `self.W_Combat` _returnvalue))
  (`UserWidget.AddToPlayerScreen` _output_get 0)
  ;[1 1 1] We bind ourself to the event that notify us when a spell is selected
  (add `/Game/TacticGame/Blueprints/Core/Combat/Spells/Widgets/WBP_ButtonList_Spell.OnSelectedSpellButtonChanged` (`/Game/TacticGame/Blueprints/Core/Combat/Widgets/WBP_Combat.ButtonList_Spell` (`self.W_Combat`)) (`|CreateDelegate` :!event `OnSelectedSpellChanged`)))

(fn `OnGridGenerated`
  ;[1 1 1 1 17] After regenerating the grid we check if the player had a Tile selected
  (if (`/Game/TacticGame/Blueprints/Core/Grid/BP_Grid.IsIndexValid` (`self.Grid`) (`self.SelectedTile`))
    (`self.SetSelectedTileAndUnit` (`self.SelectedTile`) true) ; If still valid, we reselct the same Tile
    (else
      (`self.SetSelectedTileAndUnit` (make `IntPoint` -999 -999) true) ; Othrwise we deselect it
    )))

(fn `OnSelectedSpellChanged`
  (params (Button :type "/Game/TacticGame/Blueprints/Core/Combat/Spells/Widgets/WBP_Button_Spell Object Reference"))
  (`/Engine/EditorBlueprintResources/StandardMacros.IsValid` Button ; Check that the Spell button is valid
    (:`Is Valid`
      (`self.SetSelectedAction` "/Game/TacticGame/Blueprints/Core/Player/Actions/Combat/BP_Action_Cbt_CastSpell.BP_Action_Cbt_CastSpell_C") ; OK, set the action to Cbt_CastSpell
      ;[1 1 1] After the Action is set, we also set the selected Spell inside the Action
      (bind _asbp_action_cbt_cast_spell (cast `/Game/TacticGame/Blueprints/Core/Player/Actions/Combat/BP_Action_Cbt_CastSpell` (`self.SelectedAction_LeftClick`)))
      (`/Game/TacticGame/Blueprints/Core/Player/Actions/Combat/BP_Action_Cbt_CastSpell.SetSpell` _asbp_action_cbt_cast_spell (`/Game/TacticGame/Blueprints/Core/Combat/Spells/Widgets/WBP_Button_Spell.Spell` (`local.Button`))))
    (:`Is Not Valid`
      (if (!= (`GameplayStatics.GetObjectClass` (`self.SelectedAction_LeftClick`)) "/Game/TacticGame/Blueprints/Core/Player/Actions/Combat/BP_Action_Cbt_Move.BP_Action_Cbt_Move_C")
        (`self.SetSelectedAction` "/Game/TacticGame/Blueprints/Core/Player/Actions/Combat/BP_Action_Cbt_Move.BP_Action_Cbt_Move_C") ; KO, go back in action Cbt_Move
      ))))

(fn `OnTileDataUpdated`
  (params (Index :type "IntPoint Structure"))
  (if (`KismetMathLibrary.Equal_IntPointIntPoint` Index (`self.SelectedTile`))
    (`self.OnGridGenerated`)))

(fn `OnUnitGridIndexChanged`
  (params (Unit :type "/Game/TacticGame/Blueprints/Core/Units/BP_Unit Object Reference"))
  ;[1 1 1] If the moved Unit is the one Selected
  (if (== Unit (`self.SelectedUnit`))
    ;[1 1 1] We update the Tile selection with the one the Unit reached with its movement
    (`self.SetSelectedTileAndUnit` (`/Game/TacticGame/Blueprints/Core/Units/BP_Unit.Index` Unit))))

(fn `OnUnitTurnEnded`
  (params (Unit :type "/Game/TacticGame/Blueprints/Core/Units/BP_Unit Object Reference"))
  (`self.SetSelectedTileAndUnit` (make `IntPoint` -999 -999)) ; Deselect the Unit that ended its turn
  ;[1 1 1] Unlink the spellbar with the unit. Reset the spellbar
  (`/Game/TacticGame/Blueprints/Core/Combat/Spells/Widgets/WBP_ButtonList_Spell.LinkUnitToSpellsList` (`/Game/TacticGame/Blueprints/Core/Combat/Widgets/WBP_Combat.ButtonList_Spell` (`self.W_Combat`)) null))

(fn `OnUnitTurnStarted`
  (params (Unit :type "/Game/TacticGame/Blueprints/Core/Units/BP_Unit Object Reference"))
  ;[1 1 1] Is the Unit handled by a valid AI?
  ; YES - Activate AI, put the Player in WaitForTurn
  ; NO - Player gets the controls
  (`/Engine/EditorBlueprintResources/StandardMacros.IsValid` (`/Game/TacticGame/Blueprints/Core/Units/BP_Unit.Ai` (`local.Unit`))
    (:`Is Valid`
      (if (!= (`GameplayStatics.GetObjectClass` (`self.SelectedAction_LeftClick`)) "/Game/TacticGame/Blueprints/Core/Player/Actions/Combat/BP_Action_Cbt_WaitForTurn.BP_Action_Cbt_WaitForTurn_C")
        (`self.SetSelectedAction` "/Game/TacticGame/Blueprints/Core/Player/Actions/Combat/BP_Action_Cbt_WaitForTurn.BP_Action_Cbt_WaitForTurn_C") ; Player put in Wait for Turn
      ))
    (:`Is Not Valid`
      ;[1 1 1] The Unit in play gets selected
      (`self.SetSelectedTileAndUnit` (`/Game/TacticGame/Blueprints/Core/Units/BP_Unit.Index` (`local.Unit`)))
      ;[1 1 1] The Action assigned at the start of each player turn is the ActionCbtMove
      (`self.SetSelectedAction` "/Game/TacticGame/Blueprints/Core/Player/Actions/Combat/BP_Action_Cbt_Move.BP_Action_Cbt_Move_C")
      ;[1 1 1] Link the spellbar with the unit.
      ; Every turn the spellbar shows the spell available to the Unit in play
      (`/Game/TacticGame/Blueprints/Core/Combat/Spells/Widgets/WBP_ButtonList_Spell.LinkUnitToSpellsList` (`/Game/TacticGame/Blueprints/Core/Combat/Widgets/WBP_Combat.ButtonList_Spell` (`self.W_Combat`)) (`self.SelectedUnit`)))))

(fn `SetHoveredUnitOverride`
  (params (Unit :type "/Game/TacticGame/Blueprints/Core/Units/BP_Unit Object Reference"))
  (set `self.HoveredUnitOverride` Unit)
  (`self.UpdateHoveredTileAndUnit`))

(fn `SetSelectedAction`
  (params (LeftAction :type "/Game/TacticGame/Blueprints/Core/Player/Actions/BP_Action Class Reference") (RightAction :type "/Game/TacticGame/Blueprints/Core/Player/Actions/BP_Action Class Reference"))
  (bind _selectedaction_leftclick (`self.SelectedAction_LeftClick`))
  (bind _selectedaction_rightclick (`self.SelectedAction_RightClick`))
  (`|ExecutionSequence`
    (:`then_0`
      ;[1 1 1] If there was already an action associated with the left click...
      (`/Engine/EditorBlueprintResources/StandardMacros.IsValid` _selectedaction_leftclick
        (:`Is Valid`
          ;[1 1 1] We destroy it (the old one)
          (`self.K2_DestroyActor` _selectedaction_leftclick)
          ;[1 1 1] And set it to None (no input)
          (set `self.SelectedAction_LeftClick` null))
        (:`Is Not Valid`
          _))
      ;[1 1 1] Resolved the old action (invalid or destroyed)
      ; We check if the new one in input is valid
      (if (`KismetSystemLibrary.IsValidClass` (`local.LeftAction`))
        ;[1 1 1] If valid we are gonna use it to spawn a new actor of this class
        (bind _returnvalue (`|SpawnActorFromClass` (`local.LeftAction`) (`KismetMathLibrary.MakeTransform` (0.0 0.0 0.0)) "AlwaysSpawn" "MultiplyWithRoot" null self null))
        ;[1 1 1] and set the new action
        (set `self.SelectedAction_LeftClick` _returnvalue)))
    (:`then_1`
      ;[1 1 1] If there was already an action associated with the right click...
      (`/Engine/EditorBlueprintResources/StandardMacros.IsValid` _selectedaction_rightclick
        (:`Is Valid`
          ;[1 1 1] We destroy it (the old one)
          (`self.K2_DestroyActor` _selectedaction_rightclick)
          ;[1 1 1] And set it to None (no input)
          (set `self.SelectedAction_RightClick` null))
        (:`Is Not Valid`
          _))
      ;[1 1 1] Resolved the old action (invalid or destroyed)
      ; We check if the new one in input is valid
      (if (`KismetSystemLibrary.IsValidClass` (`local.RightAction`))
        ;[1 1 1] If valid we are gonna use it to spawn a new actor of this class
        (bind _returnvalue_2 (`|SpawnActorFromClass` (`local.RightAction`) (`KismetMathLibrary.MakeTransform` (0.0 0.0 0.0)) "AlwaysSpawn" "MultiplyWithRoot" null self null))
        ;[1 1 1] and set the new action
        (set `self.SelectedAction_RightClick` _returnvalue_2)))
    (:`then_2`
      ;[1 1 1] Signal all the blueprints bound to the dispatcher
      (`self.OnSelectedActionsChanged` (`self.SelectedAction_LeftClick`) (`self.SelectedAction_RightClick`)))))

(fn `SetSelectedTileAndUnit`
  (params (Index :type "IntPoint Structure") (Force :type Boolean))
  (locals (NewUnit :type "/Game/TacticGame/Blueprints/Core/Units/BP_Unit Object Reference"))
  (bind _selectedunit (`self.SelectedUnit`))
  (`|ExecutionSequence`
    (:`then_0`
      ;[1 1 1] First thing first, we compare the index in input with the one from the selected tile, to check if they are different
      (if (or (!= (`self.SelectedTile`) (`local.Index`)) (`local.Force`))
        ;[1 1 1] If they are the different, we remove the Selected state on Previous Tile...
        (`/Game/TacticGame/Blueprints/Core/Grid/BP_Grid.RemoveStateFromTile` (`self.Grid`) (`self.SelectedTile`) "NewEnumerator2")
        ;[1 1 1] ...then update the selected Tile
        (set `self.SelectedTile` (`local.Index`))
        ;[1 1 1] ...and finally update the State for that Tile
        (`/Game/TacticGame/Blueprints/Core/Grid/BP_Grid.AddStateToTile` (`self.Grid`) (`self.SelectedTile`) "NewEnumerator2")
        (else
          ;[1 1 1] If they are the same, we wanna simply deselect the Tile.
          ; So we remove the Selected state on the Tile...
          (`/Game/TacticGame/Blueprints/Core/Grid/BP_Grid.RemoveStateFromTile` (`self.Grid`) (`self.SelectedTile`) "NewEnumerator2")
          ;[1 1 1] ...then update the selected Tile
          ; with an invalid one (-999,-999)
          (set `self.SelectedTile` (make `IntPoint` -999 -999))))
      (`self.OnSelectedTileChanged` (`self.SelectedTile`)) ; Notify tile selection change (es. for reachable tiles)
    )
    (:`then_1`
      ;[1 1 1] We get the Unit on the selected Tile of the grid and put it into a local variable
      (set `local.NewUnit` (`.UnitOnTile_16_1A24A24A4845A31FB93E7BBEC72A5FD3` (break `/Game/TacticGame/Blueprints/Core/Grid/Utilities/S_TileData` (`BlueprintMapLibrary.Map_Find` (`/Game/TacticGame/Blueprints/Core/Grid/BP_Grid.GridTiles` (`self.Grid`)) (`self.SelectedTile`)))))
      ;[1 1 1] As done for the Tile, we compare the Unit on the selected Tile with the old selected Unit, to check if they are different
      (if (or (!= (`self.SelectedUnit`) (`local.NewUnit`)) (`local.Force`))
        (`|ExecutionSequence`
          (:`then_0`
            ;[1 1 1] Old Unit deselection
            (`/Engine/EditorBlueprintResources/StandardMacros.IsValid` _selectedunit
              (:`Is Valid`
                (`/Game/TacticGame/Blueprints/Core/Units/BP_Unit.SetIsSelected` _selectedunit false))))
          (:`then_1`
            ;[1 1 1] New Unit selection
            (bind _output_get (set `self.SelectedUnit` (`local.NewUnit`)))
            (`/Engine/EditorBlueprintResources/StandardMacros.IsValid` _output_get
              (:`Is Valid`
                (`/Game/TacticGame/Blueprints/Core/Units/BP_Unit.SetIsSelected` _output_get true)))))))))

(fn `UpdateHoveredTileAndUnit`
  (locals (NewIndex :type "IntPoint Structure") (UnitLocal :type "/Game/TacticGame/Blueprints/Core/Units/BP_Unit Object Reference"))
  (bind _hoveredunit (`self.HoveredUnit`))
  (bind _hoveredunit_2 (`self.HoveredUnit`))
  (`|ExecutionSequence`
    (:`then_0`
      ;[1 1 1 1 14] Before using the default HoveredUnit we wanna check if the Player is hovering a UnitButton in the Combat Widget or in the UnitTurnList.
      ; In any of these cases, we override the Hovered Unit with the one in the Widget (we're basically considering the Widget before the Grid under the Mouse)
      (`/Engine/EditorBlueprintResources/StandardMacros.IsValid` (`self.HoveredUnitOverride`)
        (:`Is Valid`
          (set `local.UnitLocal` (`self.HoveredUnitOverride`)))
        (:`Is Not Valid`
          ;[1 1 1] Check that we are hovering a different unit and not always the same one
          (bind _unit (`self.GetUnitUnderCursor` 0))
          (set `local.UnitLocal` _unit)))
      (if (!= (`local.UnitLocal`) (`self.HoveredUnit`))
        (`|ExecutionSequence`
          (:`then_0`
            ;[1 1 1] Unhovering the old unit
            (`/Engine/EditorBlueprintResources/StandardMacros.IsValid` _hoveredunit_2
              (:`Is Valid`
                (`/Game/TacticGame/Blueprints/Core/Units/BP_Unit.SetIsHovered` _hoveredunit_2 false))))
          (:`then_1`
            ;[1 1 1] Hovering the new one
            (bind _output_get (set `self.HoveredUnit` (`local.UnitLocal`)))
            (`/Engine/EditorBlueprintResources/StandardMacros.IsValid` _output_get
              (:`Is Valid`
                (`/Game/TacticGame/Blueprints/Core/Units/BP_Unit.SetIsHovered` _output_get true)))))))
    (:`then_1`
      ;[1 1 1] If a Unit is hovered, we ignore the eventual Tile hovered and always select the index of the Tile under the Unit hovered
      (`/Engine/EditorBlueprintResources/StandardMacros.IsValid` _hoveredunit
        (:`Is Valid`
          (set `local.NewIndex` (`/Game/TacticGame/Blueprints/Core/Units/BP_Unit.Index` _hoveredunit)))
        (:`Is Not Valid`
          ;[1 1 1] If no Unit is hovered, than we use the hovered Tile index
          (bind _index (`/Game/TacticGame/Blueprints/Core/Grid/BP_Grid.GetTileIndexUnderCursor` (`self.Grid`) 0 (`self.CanHoverGround`) (`self.CanHoverEmptySpace`)))
          (set `local.NewIndex` _index)))
      ;[1 1 1] Performance Optimization
      ; we update the hovered tile only if its a different one from the previous hovered one
      (if (!= (`local.NewIndex`) (`self.HoveredTile`))
        ;[1 1 1] Remove the hovered state from the old tile
        (`/Game/TacticGame/Blueprints/Core/Grid/BP_Grid.RemoveStateFromTile` (`self.Grid`) (`self.HoveredTile`) "NewEnumerator1")
        ;[1 1 1] Update the hovered state to the new tile
        (bind _output_get_2 (set `self.HoveredTile` (`local.NewIndex`)))
        (`/Game/TacticGame/Blueprints/Core/Grid/BP_Grid.AddStateToTile` (`self.Grid`) _output_get_2 "NewEnumerator1")
        ;[1 1 1] Signal the Event listening for the hovered tile changed
        (`self.Event_ExecuteActionWhenHoveredTileChanged`)
        ;[1 1 1] Signal the game of Hovered Tile change
        (`self.OnHoveredTileChanged` (`self.HoveredTile`))))))

(fn `UserConstructionScript`)