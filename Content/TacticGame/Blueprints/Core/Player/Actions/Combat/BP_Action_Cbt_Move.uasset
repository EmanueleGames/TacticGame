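; Combat player action that previews and executes movement for the turn's selected unit on the tactics grid.
; Hovering shows the hovered unit's reachable tiles, or the selected unit's plus a path to the hovered tile.
; Pathfinding completion callbacks mark tiles and cache the path, which execution passes to CombatSystem.
; Walk start/finish events suspend and refresh previews, and EndPlay clears both tile states.
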(event `self.ReceiveBeginPlay`
  (bind _selectedunit (`/Game/TacticGame/Blueprints/Core/Player/BP_PlayerActions.SelectedUnit` (`self.PlayerActions`)))
  (`parent.ReceiveBeginPlay`)
  ;[1 1 1] We hook to the Event that notify us whenever Reachables generation is complete
  ; could be the Reachables of any Unit on the Grid, it depends on the Unit hovered / selected
  (add `/Game/TacticGame/Blueprints/Core/Grid/BP_GridPathfinding.OnPathfindingCompleted` (`/Game/TacticGame/Blueprints/Core/Grid/BP_Grid.GridPathfinding_Reachables` (`/Game/TacticGame/Blueprints/Core/Player/BP_PlayerActions.Grid` (`self.PlayerActions`))) (`|CreateDelegate` :!event `OnPathfindingCompleted_Reachables`))
  ;[1 1 1] We hook to the Event that notify us whenever the path generation is complete
  ; this only works for the selected Unit, the other ones can't move when it's not their turn
  (add `/Game/TacticGame/Blueprints/Core/Grid/BP_GridPathfinding.OnPathfindingCompleted` (`/Game/TacticGame/Blueprints/Core/Grid/BP_Grid.GridPathfinding` (`/Game/TacticGame/Blueprints/Core/Player/BP_PlayerActions.Grid` (`self.PlayerActions`))) (`|CreateDelegate` :!event `OnPathfindingCompleted_Path`))
  ;[1 1 1] Since we want to sync functionality like "keep the path visible until its fully walked" or "as soon as the Unit finishes walking, generate new reachables"... We hook to the proper events to be notified
  (add `/Game/TacticGame/Blueprints/Core/Units/BP_Unit.OnUnitStartedWalking` _selectedunit (`|CreateDelegate` :!event `OnUnitStartedWalking`))
  (add `/Game/TacticGame/Blueprints/Core/Units/BP_Unit.OnUnitFinishedWalking` _selectedunit (`|CreateDelegate` :!event `OnUnitFinishedWalking`))
  ;[1 1 1] We make sure to generate the reachables for the selected Unit at the beginning of each turn (different turn = different Unit)
  (`self.GenerateReachables` (`/Game/TacticGame/Blueprints/Core/Player/BP_PlayerActions.SelectedUnit` (`self.PlayerActions`))))

(event `self.ReceiveEndPlay`
  (params (EndPlayReason :type "EEndPlayReason Enum" :default "Destroyed"))
  (bind _grid (`/Game/TacticGame/Blueprints/Core/Player/BP_PlayerActions.Grid` (`self.PlayerActions`)))
  ;[1 1 1] To keep consistency when the Action is deleted from the game (exit combat)
  ; We are performing some clean-up in the EndPlay event
  (`parent.ReceiveEndPlay` EndPlayReason)
  (`/Game/TacticGame/Blueprints/Core/Grid/BP_Grid.ClearStateFromTiles` _grid "NewEnumerator7") ; Clear any pending Reachable
  (`/Game/TacticGame/Blueprints/Core/Grid/BP_Grid.ClearStateFromTiles` _grid "NewEnumerator4") ; Clear any pending Path
)

(fn `ExecuteAction`
  (params (Index :type "IntPoint Structure"))
  (bind _playeractions (`self.PlayerActions`))
  (`parent.ExecuteAction` Index)
  ;[1 1 1] Unit movement on left click
  (if (> (`KismetArrayLibrary.Array_Length` (`self.GeneratedPath`)) 0)
    (`/Game/TacticGame/Blueprints/Core/Combat/BP_CombatSystem.MoveUnit` (`/Game/TacticGame/Blueprints/Core/Player/BP_PlayerActions.CombatSystem` _playeractions) (`/Game/TacticGame/Blueprints/Core/Player/BP_PlayerActions.SelectedUnit` _playeractions) (`self.GeneratedPath`)) ; ask the CombatSystem to move the Unit
    (`KismetArrayLibrary.Array_Clear` (`self.GeneratedPath`)) ; Clear the Path just walked, for consistency
  ))

(fn `ExecuteHoveredAction`
  (params (Index :type "IntPoint Structure"))
  (bind _playeractions (`self.PlayerActions`))
  (bind _hoveredunit (`/Game/TacticGame/Blueprints/Core/Player/BP_PlayerActions.HoveredUnit` _playeractions))
  (`parent.ExecuteHoveredAction` Index)
  ;[1 1 1] Hovered actions are not executed while a Unit is currently moving
  (if (not (`self.IsUnitWalking`))
    ;[1 1 1] During each turn, if the player hovers a valid Unit we display that Unit reachables,
    ; otherwise we display the reachables for the selected Unit (the one in play for that turn)
    (`/Engine/EditorBlueprintResources/StandardMacros.IsValid` _hoveredunit
      (:`Is Valid`
        (`self.GenerateReachables` _hoveredunit)
        ;[1 1 1 1 16] Personal initiative!!!!
        ; It may happen that during a Unit turn the player is hovering its reachable tiles and finding a path among them
        ; If another Unit is on one of the reachables and it hovered, we display his reachable instead but the old path is still there so we clear it
        (`/Game/TacticGame/Blueprints/Core/Grid/BP_Grid.ClearStateFromTiles` (`/Game/TacticGame/Blueprints/Core/Player/BP_PlayerActions.Grid` (`self.PlayerActions`)) "NewEnumerator4") ; Clear old Path
        (`KismetArrayLibrary.Array_Clear` (`self.GeneratedPath`)) ; Clear old saved Path, to avoid using it for an invalid movement
      )
      (:`Is Not Valid`
        (`self.GenerateReachables` (`/Game/TacticGame/Blueprints/Core/Player/BP_PlayerActions.SelectedUnit` _playeractions))
        ;[1 1 1] The Path instead is generated only for the selected Unit
        (`self.GeneratePath`)))))

(fn `GeneratePath`
  (bind _selectedunit (`/Game/TacticGame/Blueprints/Core/Player/BP_PlayerActions.SelectedUnit` (`self.PlayerActions`)))
  (bind ((`ValidTileTypes_3_929725CE49027623BFBC479EBA9580D6` _validtiletypes) (`CanMoveDiagonally_7_7E720D6645739EC9FF74959433CD15E1` _canmovediagonally) (`MP_Current_10_FB397B3D409E5FAEA964D8A44B0876D5` _mp_current)) (break `/Game/TacticGame/Blueprints/Core/Units/Utilities/S_UnitData_Stats` (`.Stats_8_1FF4029D4CCC943B93A92087BC3004A2` (break `/Game/TacticGame/Blueprints/Core/Units/Utilities/S_UnitData` (`/Game/TacticGame/Blueprints/Core/Units/BP_Unit.UnitData` _selectedunit)))))
  ;[1 1 1] new Path creation
  (`/Game/TacticGame/Blueprints/Core/Grid/BP_Grid.ClearStateFromTiles` (`/Game/TacticGame/Blueprints/Core/Player/BP_PlayerActions.Grid` (`self.PlayerActions`)) "NewEnumerator4") ; Clear old Path
  (`KismetArrayLibrary.Array_Clear` (`self.GeneratedPath`)) ; Clear old saved Path, to avoid using it for an invalid movement
  (`/Game/TacticGame/Blueprints/Core/Grid/BP_GridPathfinding.FindPath` (`/Game/TacticGame/Blueprints/Core/Grid/BP_Grid.GridPathfinding` (`/Game/TacticGame/Blueprints/Core/Player/BP_PlayerActions.Grid` (`self.PlayerActions`))) (`/Game/TacticGame/Blueprints/Core/Units/BP_Unit.Index` _selectedunit) (`/Game/TacticGame/Blueprints/Core/Player/BP_PlayerActions.HoveredTile` (`self.PlayerActions`)) _canmovediagonally _validtiletypes 0.1 15.0 false _mp_current) ; Find the new Path
)

(fn `GenerateReachables`
  (params (Unit :type "/Game/TacticGame/Blueprints/Core/Units/BP_Unit Object Reference"))
  (bind _currentunitforreachables (`self.CurrentUnitForReachables`))
  (bind ((`ValidTileTypes_3_929725CE49027623BFBC479EBA9580D6` _validtiletypes) (`CanMoveDiagonally_7_7E720D6645739EC9FF74959433CD15E1` _canmovediagonally) (`MP_Current_10_FB397B3D409E5FAEA964D8A44B0876D5` _mp_current)) (break `/Game/TacticGame/Blueprints/Core/Units/Utilities/S_UnitData_Stats` (`.Stats_8_1FF4029D4CCC943B93A92087BC3004A2` (break `/Game/TacticGame/Blueprints/Core/Units/Utilities/S_UnitData` (`/Game/TacticGame/Blueprints/Core/Units/BP_Unit.UnitData` _currentunitforreachables)))))
  ;[1 1 1] Since we could hover on many Unit in succession with our mouse, before generating the Reachables, we make sure that the Unit is in fact different from the one we generated the Reachables before (stored in a variables)
  (if (!= Unit (`self.CurrentUnitForReachables`))
    (set `self.CurrentUnitForReachables` Unit) ; Different, update the Unit we're displaying
    ;[1 1 1] new Reachables creation
    (`/Game/TacticGame/Blueprints/Core/Grid/BP_Grid.ClearStateFromTiles` (`/Game/TacticGame/Blueprints/Core/Player/BP_PlayerActions.Grid` (`self.PlayerActions`)) "NewEnumerator7") ; Clear old reachables
    (`/Game/TacticGame/Blueprints/Core/Grid/BP_GridPathfinding.FindPath` (`/Game/TacticGame/Blueprints/Core/Grid/BP_Grid.GridPathfinding_Reachables` (`/Game/TacticGame/Blueprints/Core/Player/BP_PlayerActions.Grid` (`self.PlayerActions`))) (`/Game/TacticGame/Blueprints/Core/Units/BP_Unit.Index` _currentunitforreachables) (make `IntPoint` -999 -999) _canmovediagonally _validtiletypes 0.1 15.0 true _mp_current) ; Find the new Reachables
  ))

(fn `OnPathfindingCompleted_Path`
  (params (Path :type "Array of IntPoint Structure"))
  ;[1 1 1 1 16] We save the Path into a variable so, if the player decides to move along that path, we have it ready and don't have to recalculate it
  ; (it is done on every new Tile hovered)
  (bind _output_get (set `self.GeneratedPath` Path))
  ;[1 1 1] When the pathfinding is complete, we add the InPath state to the correct tiles
  (for _array_element _output_get
    (`/Game/TacticGame/Blueprints/Core/Grid/BP_Grid.AddStateToTile` (`/Game/TacticGame/Blueprints/Core/Player/BP_PlayerActions.Grid` (`self.PlayerActions`)) _array_element "NewEnumerator4")))

(fn `OnPathfindingCompleted_Reachables`
  (params (Reachables :type "Array of IntPoint Structure"))
  ;[1 1 1 1 16] We don't wanna show reachables while Unit is walking (could happens if the FindPath for the reachables takes too much time)
  (if (not (`self.IsUnitWalking`))
    ;[1 1 1] When the pathfinding is complete, we add the Reachable state to the correct tiles
    (for _array_element Reachables
      (`/Game/TacticGame/Blueprints/Core/Grid/BP_Grid.AddStateToTile` (`/Game/TacticGame/Blueprints/Core/Player/BP_PlayerActions.Grid` (`self.PlayerActions`)) _array_element "NewEnumerator7"))))

(fn `OnUnitFinishedWalking`
  (params (Unit :type "/Game/TacticGame/Blueprints/Core/Units/BP_Unit Object Reference"))
  (set `self.IsUnitWalking` false) ; flag variable FALSE
  (`self.ExecuteHoveredAction` (`/Game/TacticGame/Blueprints/Core/Player/BP_PlayerActions.HoveredTile` (`self.PlayerActions`))) ; Execute the hovered action\n(could be to generate a new path or new reachables)
)

(fn `OnUnitStartedWalking`
  (params (Unit :type "/Game/TacticGame/Blueprints/Core/Units/BP_Unit Object Reference"))
  (set `self.IsUnitWalking` true) ; flag variable TRUE
  (`/Game/TacticGame/Blueprints/Core/Grid/BP_Grid.ClearStateFromTiles` (`/Game/TacticGame/Blueprints/Core/Player/BP_PlayerActions.Grid` (`self.PlayerActions`)) "NewEnumerator7") ; ...Clear the Reachables, they're no valid anymore
  (set `self.CurrentUnitForReachables` null) ; set CurrentUnitForReachable as invalid\n(at least until the Unit stops)
)

(fn `UserConstructionScript`
  (`parent.UserConstructionScript`))