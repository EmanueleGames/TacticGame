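; Combat player action that previews a selected spell's range on the grid and casts it from the selected tile onto the executed tile.
; SetSpell caches the spell's cast and AoE data, then paints range tiles obtained from the CombatSystem as grid states.
; Hovering redraws the AoE pattern for in-range tiles, or just the hovered tile without one.
; Execution delegates to CombatSystem and deselects the spell button; EndPlay clears both indicators.
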(event `self.ReceiveEndPlay`
  (params (EndPlayReason :type "EEndPlayReason Enum" :default "Destroyed"))
  (bind _grid (`/Game/TacticGame/Blueprints/Core/Player/BP_PlayerActions.Grid` (`self.PlayerActions`)))
  (`parent.ReceiveEndPlay` EndPlayReason)
  ;[1 1 1] Clear eventual deferred old indicators
  (`/Game/TacticGame/Blueprints/Core/Grid/BP_Grid.ClearStateFromTiles` _grid "NewEnumerator8")
  (`/Game/TacticGame/Blueprints/Core/Grid/BP_Grid.ClearStateFromTiles` _grid "NewEnumerator9"))

(fn `ExecuteAction`
  (params (Index :type "IntPoint Structure"))
  (bind _playeractions (`self.PlayerActions`))
  (bind _w_combat (`/Game/TacticGame/Blueprints/Core/Player/BP_PlayerActions.W_Combat` (`self.PlayerActions`)))
  (`parent.ExecuteAction` Index)
  (`/Game/TacticGame/Blueprints/Core/Combat/BP_CombatSystem.CastSpell` (`/Game/TacticGame/Blueprints/Core/Player/BP_PlayerActions.CombatSystem` _playeractions) (`self.Spell`) (`/Game/TacticGame/Blueprints/Core/Player/BP_PlayerActions.SelectedTile` _playeractions) (`local.Index`))
  ;[1 1 1] After casting a spell we deselect the Button
  (`/Engine/EditorBlueprintResources/StandardMacros.IsValid` _w_combat ; Widget is destroyed during the FinishingCombat phase
    (:`Is Valid`
      (`/Game/TacticGame/Blueprints/Core/Combat/Spells/Widgets/WBP_ButtonList_Spell.SetSelectedSpellFromIndex` (`/Game/TacticGame/Blueprints/Core/Combat/Widgets/WBP_Combat.ButtonList_Spell` _w_combat) -1) ; -1 means deselect
    )))

(fn `ExecuteHoveredAction`
  (params (Index :type "IntPoint Structure"))
  (`parent.ExecuteHoveredAction` Index)
  (`self.ShowSpellRangePatternAoe`))

(fn `SetSpell`
  (params (Spell :type "/Game/TacticGame/Blueprints/Core/Combat/Spells/Utilities/E_Spell Enum" :default "NewEnumerator0"))
  (bind _grid (`/Game/TacticGame/Blueprints/Core/Player/BP_PlayerActions.Grid` (`self.PlayerActions`)))
  (bind _output_get (set `self.Spell` Spell))
  ;[1 1 1] is the Spell valid?
  (if (`|EnumInequality` _output_get "NewEnumerator0")
    ;[1 1 1] Spell is valid, lets start by saving its info in two variables
    (bind _spelldata (`/Game/TacticGame/Blueprints/Core/Combat/Spells/Utilities/BFL_Spells.GetSpellDataFromSpell` (`self.Spell`)))
    (bind ((`Cast_8_748526A74251AD731B2C90902CCB0787` _cast) (`CastAoe_11_E2D808754BFAA919D9F7AFA1E6870B0D` _castaoe)) (break `/Game/TacticGame/Blueprints/Core/Combat/Spells/Utilities/S_SpellData` _spelldata))
    (set `self.Cast` _cast)
    (set `self.CastAoe` _castaoe)
    ;[1 1 1] Show on the Grid the indicators for the new selected spell
    (`self.ShowSpellRangePattern`)
    (else
      ;[1 1 1] Spell is not valid, clear all indicator from the Grid
      (`/Game/TacticGame/Blueprints/Core/Grid/BP_Grid.ClearStateFromTiles` _grid "NewEnumerator8")
      (`/Game/TacticGame/Blueprints/Core/Grid/BP_Grid.ClearStateFromTiles` _grid "NewEnumerator9"))))

(fn `ShowSpellRangePattern`
  (bind _playeractions (`self.PlayerActions`))
  (bind _grid (`/Game/TacticGame/Blueprints/Core/Player/BP_PlayerActions.Grid` (`self.PlayerActions`)))
  (`|ExecutionSequence`
    (:`then_0`
      ;[1 1 1] Clear old indicators
      (`/Game/TacticGame/Blueprints/Core/Grid/BP_Grid.ClearStateFromTiles` _grid "NewEnumerator8")
      (`/Game/TacticGame/Blueprints/Core/Grid/BP_Grid.ClearStateFromTiles` _grid "NewEnumerator9")
      ;[1 1 1] Get new indicators
      (bind _rangeindices (`/Game/TacticGame/Blueprints/Core/Combat/BP_CombatSystem.GetSpellRange` (`/Game/TacticGame/Blueprints/Core/Player/BP_PlayerActions.CombatSystem` _playeractions) (`/Game/TacticGame/Blueprints/Core/Player/BP_PlayerActions.SelectedTile` _playeractions) (`self.Cast`)))
      ;[1 1 1] Add the new indicators to the Grid
      (for _array_element _rangeindices
        (`/Game/TacticGame/Blueprints/Core/Grid/BP_Grid.AddStateToTile` (`/Game/TacticGame/Blueprints/Core/Player/BP_PlayerActions.Grid` (`self.PlayerActions`)) _array_element "NewEnumerator8")))
    (:`then_1`
      (`self.ShowSpellRangePatternAoe`) ; Update the indicators for the AoE spells
    )))

(fn `ShowSpellRangePatternAoe`
  (bind _playeractions (`self.PlayerActions`))
  ;[1 1 1] Clear the previous Spell Range Pattern
  (`/Game/TacticGame/Blueprints/Core/Grid/BP_Grid.ClearStateFromTiles` (`/Game/TacticGame/Blueprints/Core/Player/BP_PlayerActions.Grid` (`self.PlayerActions`)) "NewEnumerator9")
  ;[1 1 1] When the player is casting an AoE spell, we need to check if the Tile he wants to originate the spell from (the one he is hovering) is among the tiles of the SpellRange
  (if (`KismetArrayLibrary.Array_Contains` (`.IntPointArray_3_D0EC34214CC66367B6C657B38B50F0D6` (break `/Game/TacticGame/Blueprints/Core/Grid/Utilities/S_IntPointArray` (`BlueprintMapLibrary.Map_Find` (`/Game/TacticGame/Blueprints/Core/Grid/BP_Grid.TileStateToIndices` (`/Game/TacticGame/Blueprints/Core/Player/BP_PlayerActions.Grid` (`self.PlayerActions`))) "NewEnumerator8"))) (`/Game/TacticGame/Blueprints/Core/Player/BP_PlayerActions.HoveredTile` (`self.PlayerActions`)))
    ;[1 1 1] We make sure that the AoE has a pattern to draw on the grid
    (if (`|EnumInequality` (`.RangePattern_3_8F2F620549BE101B8A88079D92F4C347` (break `/Game/TacticGame/Blueprints/Core/Combat/Spells/Utilities/S_SpellData_Cast` (`self.CastAoe`))) "NewEnumerator0")
      ;[1 1 1] Then we can ask the combat system to give us the AoE target indices...
      (bind _rangeindices (`/Game/TacticGame/Blueprints/Core/Combat/BP_CombatSystem.GetSpellRange` (`/Game/TacticGame/Blueprints/Core/Player/BP_PlayerActions.CombatSystem` _playeractions) (`/Game/TacticGame/Blueprints/Core/Player/BP_PlayerActions.HoveredTile` _playeractions) (`self.CastAoe`)))
      ;[1 1 1] ...and for each of them we set the tile state to IsSpellRangeAoE
      (for _array_element _rangeindices
        (`/Game/TacticGame/Blueprints/Core/Grid/BP_Grid.AddStateToTile` (`/Game/TacticGame/Blueprints/Core/Player/BP_PlayerActions.Grid` (`self.PlayerActions`)) _array_element "NewEnumerator9"))
      (else
        ;[1 1 1] If there is no pattern, like a not AoE spell with a single target tile
        ; we show the appropriate color only on the hovered tile
        (`/Game/TacticGame/Blueprints/Core/Grid/BP_Grid.AddStateToTile` (`/Game/TacticGame/Blueprints/Core/Player/BP_PlayerActions.Grid` (`self.PlayerActions`)) (`/Game/TacticGame/Blueprints/Core/Player/BP_PlayerActions.HoveredTile` (`self.PlayerActions`)) "NewEnumerator9")))))

(fn `UserConstructionScript`
  (`parent.UserConstructionScript`))