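; Combat player action for waiting on a turn that highlights the movement range of the hovered unit, or of the selected unit in play when none is hovered.
; Hovering triggers a time-budgeted reachables pathfinding search from the unit's movement stats, skipped if the unit is unchanged.
; A completion callback bound on BeginPlay marks the returned grid tiles with a reachable state, which is cleared on unit change and EndPlay.
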(event `self.ReceiveBeginPlay`
  (`parent.ReceiveBeginPlay`)
  ;[1 1 1] We hook to the Event that notify us whenever Reachables generation is complete
  ; could be the Reachables of any Unit on the Grid, it depends on the Unit hovered / selected
  (add `/Game/TacticGame/Blueprints/Core/Grid/BP_GridPathfinding.OnPathfindingCompleted` (`/Game/TacticGame/Blueprints/Core/Grid/BP_Grid.GridPathfinding_Reachables` (`/Game/TacticGame/Blueprints/Core/Player/BP_PlayerActions.Grid` (`self.PlayerActions`))) (`|CreateDelegate` :!event `OnPathfindingCompleted_Reachables`)))

(event `self.ReceiveEndPlay`
  (params (EndPlayReason :type "EEndPlayReason Enum" :default "Destroyed"))
  ;[1 1 1] To keep consistency when the Action is deleted from the game (exit combat)
  ; We are performing some clean-up in the EndPlay event
  (`parent.ReceiveEndPlay` EndPlayReason)
  (`/Game/TacticGame/Blueprints/Core/Grid/BP_Grid.ClearStateFromTiles` (`/Game/TacticGame/Blueprints/Core/Player/BP_PlayerActions.Grid` (`self.PlayerActions`)) "NewEnumerator7") ; Clear any pending Reachable
)

(fn `ExecuteHoveredAction`
  (params (Index :type "IntPoint Structure"))
  (bind _playeractions (`self.PlayerActions`))
  (bind _hoveredunit (`/Game/TacticGame/Blueprints/Core/Player/BP_PlayerActions.HoveredUnit` _playeractions))
  (`parent.ExecuteHoveredAction` Index)
  ;[1 1 1] During each turn, if the player hovers a valid Unit we display that Unit reachables,
  ; otherwise we display the reachables for the selected Unit (the one in play for that turn)
  (`/Engine/EditorBlueprintResources/StandardMacros.IsValid` _hoveredunit
    (:`Is Valid`
      (`self.GenerateReachables` _hoveredunit))
    (:`Is Not Valid`
      (`self.GenerateReachables` (`/Game/TacticGame/Blueprints/Core/Player/BP_PlayerActions.SelectedUnit` _playeractions)))))

(fn `GenerateReachables`
  (params (Unit :type "/Game/TacticGame/Blueprints/Core/Units/BP_Unit Object Reference"))
  (bind _currentunitforreachables (`self.CurrentUnitForReachables`))
  (bind ((`ValidTileTypes_3_929725CE49027623BFBC479EBA9580D6` _validtiletypes) (`CanMoveDiagonally_7_7E720D6645739EC9FF74959433CD15E1` _canmovediagonally) (`MP_Current_10_FB397B3D409E5FAEA964D8A44B0876D5` _mp_current)) (break `/Game/TacticGame/Blueprints/Core/Units/Utilities/S_UnitData_Stats` (`.Stats_8_1FF4029D4CCC943B93A92087BC3004A2` (break `/Game/TacticGame/Blueprints/Core/Units/Utilities/S_UnitData` (`/Game/TacticGame/Blueprints/Core/Units/BP_Unit.UnitData` _currentunitforreachables)))))
  ;[1 1 1] Since we could hover on many Unit in succession with our mouse, before generating the Reachables, we make sure that the Unit is in fact different from the one we generated the Reachables before (stored in a variables)
  (if (!= Unit (`self.CurrentUnitForReachables`))
    (set `self.CurrentUnitForReachables` Unit) ; Different, update the Unit we're displaying
    ;[1 1 1] new Reachables creation
    (`/Game/TacticGame/Blueprints/Core/Grid/BP_Grid.ClearStateFromTiles` (`/Game/TacticGame/Blueprints/Core/Player/BP_PlayerActions.Grid` (`self.PlayerActions`)) "NewEnumerator7") ; Clear old reachables
    (`/Engine/EditorBlueprintResources/StandardMacros.IsValid` _currentunitforreachables
      (:`Is Valid`
        (`/Game/TacticGame/Blueprints/Core/Grid/BP_GridPathfinding.FindPath` (`/Game/TacticGame/Blueprints/Core/Grid/BP_Grid.GridPathfinding_Reachables` (`/Game/TacticGame/Blueprints/Core/Player/BP_PlayerActions.Grid` (`self.PlayerActions`))) (`/Game/TacticGame/Blueprints/Core/Units/BP_Unit.Index` _currentunitforreachables) (make `IntPoint` -999 -999) _canmovediagonally _validtiletypes 0.1 15.0 true _mp_current) ; Find the new Reachables
      ))))

(fn `OnPathfindingCompleted_Reachables`
  (params (Reachables :type "Array of IntPoint Structure"))
  ;[1 1 1] When the pathfinding is complete, we add the Reachable state to the correct tiles
  (for _array_element Reachables
    (`/Game/TacticGame/Blueprints/Core/Grid/BP_Grid.AddStateToTile` (`/Game/TacticGame/Blueprints/Core/Player/BP_PlayerActions.Grid` (`self.PlayerActions`)) _array_element "NewEnumerator7")))

(fn `UserConstructionScript`
  (`parent.UserConstructionScript`))