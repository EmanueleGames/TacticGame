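; BP_Action_AddRemoveUnitFromCombat is a combat setup player action that adds or removes a unit on a chosen grid tile.
; When adding, it checks the tile type against the unit type's valid tiles, clears any existing occupant, then spawns a BP_Unit and registers it with the Combat System with team and AI settings.
; Removal shares that clearing path, unregistering the tile's unit and destroying its actor.
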(fn `ExecuteAction`
  (params (Index :type "IntPoint Structure"))
  (locals (Unit :type "/Game/TacticGame/Blueprints/Core/Units/BP_Unit Object Reference"))
  (if (`self.IsAddingUnit`)
    ;[1 1 1] We need to check if we're allowed to spawn that Specific Unit on that Specific Tile
    ; So we compare the chosen tile with theTileTypes allowed by that kind of unit
    (bind _unitdata (`/Game/TacticGame/Blueprints/Core/Units/Utilities/BFL_Units.GetDefaultDataFromUnitType` (`self.UnitType`)))
    (if (`KismetArrayLibrary.Array_Contains` (`.ValidTileTypes_3_929725CE49027623BFBC479EBA9580D6` (break `/Game/TacticGame/Blueprints/Core/Units/Utilities/S_UnitData_Stats` (`.Stats_8_1FF4029D4CCC943B93A92087BC3004A2` (break `/Game/TacticGame/Blueprints/Core/Units/Utilities/S_UnitData` _unitdata)))) (`.Type_8_8F74F19243475FAB39F94AA272B2F514` (break `/Game/TacticGame/Blueprints/Core/Grid/Utilities/S_TileData` (`BlueprintMapLibrary.Map_Find` (`/Game/TacticGame/Blueprints/Core/Grid/BP_Grid.GridTiles` (`/Game/TacticGame/Blueprints/Core/Player/BP_PlayerActions.Grid` (`self.PlayerActions`))) (`local.Index`)))))
      ;[1 1 1] Before proceding with the Unit spawn,
      ; we branch in the remove path to despawn any possible old unit found on the same tile
      (`|ExecutionSequence`
        (:`then_0`
          ;[1 1 1] We access the grid data at corresponding index, and check if there is a unit on that tile (is valid)
          (bind _output_get (set `local.Unit` (`.UnitOnTile_16_1A24A24A4845A31FB93E7BBEC72A5FD3` (break `/Game/TacticGame/Blueprints/Core/Grid/Utilities/S_TileData` (`BlueprintMapLibrary.Map_Find` (`/Game/TacticGame/Blueprints/Core/Grid/BP_Grid.GridTiles` (`/Game/TacticGame/Blueprints/Core/Player/BP_PlayerActions.Grid` (`self.PlayerActions`))) (`local.Index`)))) :!label _label))
          (`/Engine/EditorBlueprintResources/StandardMacros.IsValid` _output_get
            (:`Is Valid`
              ;[1 1 1] If there is a Unit, we remove it from the combat system
              (`/Game/TacticGame/Blueprints/Core/Combat/BP_CombatSystem.RemoveUnitFromCombat` (`/Game/TacticGame/Blueprints/Core/Player/BP_PlayerActions.CombatSystem` (`self.PlayerActions`)) (`local.Unit`))
              (`self.K2_DestroyActor` (`local.Unit`)) ; Destroy the Unit Actor
            )))
        (:`then_1`
          ;[1 1 1] Creating an instance of BP_Unit with proper type
          (bind _returnvalue (`|SpawnActorFromClass` "/Game/TacticGame/Blueprints/Core/Units/BP_Unit.BP_Unit_C" (`KismetMathLibrary.MakeTransform` (0.0 0.0 0.0)) "AlwaysSpawn" "MultiplyWithRoot" null (`self.UnitType`) null))
          ;[1 1 1] And add the new Unit to the Combat System
          (`/Game/TacticGame/Blueprints/Core/Combat/BP_CombatSystem.AddUnitInCombat` (`/Game/TacticGame/Blueprints/Core/Player/BP_PlayerActions.CombatSystem` (`self.PlayerActions`)) _returnvalue (`local.Index`) (`self.TeamIndex`) (`self.UseAi`)))))
    (else
      (goto _label))))

(fn `UserConstructionScript`
  (`parent.UserConstructionScript`))