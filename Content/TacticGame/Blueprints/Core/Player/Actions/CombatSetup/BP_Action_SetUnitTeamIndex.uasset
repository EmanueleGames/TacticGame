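; Player action for combat setup that assigns a team index to the unit standing on a selected grid tile.
; ExecuteAction looks up the tile by index in the Grid's GridTiles map and checks that its UnitOnTile is valid.
; It then passes that unit and the action's TeamIndex to the CombatSystem's SetUnitTeamIndex, reaching both Grid and CombatSystem through PlayerActions.
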(fn `ExecuteAction`
  (params (Index :type "IntPoint Structure"))
  (bind ((`UnitOnTile_16_1A24A24A4845A31FB93E7BBEC72A5FD3` _unitontile)) (break `/Game/TacticGame/Blueprints/Core/Grid/Utilities/S_TileData` (`BlueprintMapLibrary.Map_Find` (`/Game/TacticGame/Blueprints/Core/Grid/BP_Grid.GridTiles` (`/Game/TacticGame/Blueprints/Core/Player/BP_PlayerActions.Grid` (`self.PlayerActions`))) (`local.Index`))))
  ;[1 1 1] Is there a valid Unit on the clicked Tile?
  (`/Engine/EditorBlueprintResources/StandardMacros.IsValid` _unitontile
    (:`Is Valid`
      ;[1 1 1] Put that Unit on the TeamIndex in input
      (`/Game/TacticGame/Blueprints/Core/Combat/BP_CombatSystem.SetUnitTeamIndex` (`/Game/TacticGame/Blueprints/Core/Player/BP_PlayerActions.CombatSystem` (`self.PlayerActions`)) _unitontile (`self.TeamIndex`)))))

(fn `UserConstructionScript`
  (`parent.UserConstructionScript`))