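; Combat setup player action that previews a spell's range and area of effect on the tactics grid.
; Executing the action rebuilds the range tiles from the selected tile using the combat system's GetSpellRange, then refreshes the AoE preview.
; Hovering redraws only the AoE preview, shown when the hovered tile lies within the spell range.
; The AoE preview marks the CastAoe pattern around that tile, or just the tile itself when no pattern is set.
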(fn `ExecuteAction`
  (params (Index :type "IntPoint Structure"))
  (`parent.ExecuteAction` Index)
  (`self.ShowSpellRangePattern`))

(fn `ExecuteHoveredAction`
  (params (Index :type "IntPoint Structure"))
  (`parent.ExecuteHoveredAction` Index)
  ;[1 1 1] After each time we hover a new Tile,
  ; we also update the Spell Range Pattern for AoE spell
  (`self.ShowSpellRangePatternAoe`))

(fn `ShowSpellRangePattern`
  (bind _playeractions (`self.PlayerActions`))
  (bind _playeractions_2 (`self.PlayerActions`))
  (`|ExecutionSequence`
    (:`then_0`
      ;[1 1 1] Clear the previous Spell Range Pattern
      (`/Game/TacticGame/Blueprints/Core/Grid/BP_Grid.ClearStateFromTiles` (`/Game/TacticGame/Blueprints/Core/Player/BP_PlayerActions.Grid` (`self.PlayerActions`)) "NewEnumerator8")
      ;[1 1 1] We make sure we're casting from a valid Origin Index
      (if (`/Game/TacticGame/Blueprints/Core/Grid/BP_Grid.IsIndexValid` (`/Game/TacticGame/Blueprints/Core/Player/BP_PlayerActions.Grid` _playeractions_2) (`/Game/TacticGame/Blueprints/Core/Player/BP_PlayerActions.SelectedTile` _playeractions_2))
        ;[1 1 1] Then we can ask the combat system to give us the target indices...
        (bind _rangeindices (`/Game/TacticGame/Blueprints/Core/Combat/BP_CombatSystem.GetSpellRange` (`/Game/TacticGame/Blueprints/Core/Player/BP_PlayerActions.CombatSystem` _playeractions) (`/Game/TacticGame/Blueprints/Core/Player/BP_PlayerActions.SelectedTile` _playeractions) (`self.Cast`)))
        ;[1 1 1] ...and for each of them we set the tile state to IsSpellRange
        (for _array_element _rangeindices
          (`/Game/TacticGame/Blueprints/Core/Grid/BP_Grid.AddStateToTile` (`/Game/TacticGame/Blueprints/Core/Player/BP_PlayerActions.Grid` (`self.PlayerActions`)) _array_element "NewEnumerator8"))))
    (:`then_1`
      ;[1 1 1] After each time we update the Spell Range Pattern, we also update the Spell Range Pattern for AoE spell
      (`self.ShowSpellRangePatternAoe`))))

(fn `ShowSpellRangePatternAoe`
  (bind _playeractions (`self.PlayerActions`))
  ;[1 1 1] Clear the previous Spell Range Pattern
  (`/Game/TacticGame/Blueprints/Core/Grid/BP_Grid.ClearStateFromTiles` (`/Game/TacticGame/Blueprints/Core/Player/BP_PlayerActions.Grid` (`self.PlayerActions`)) "NewEnumerator9")
  ;[1 1 1] When the player is casting an AoE spell, we need to check if the Tile he wants to originate the spell from (the one he is hovering) is among the tiles of the SpellRange
  (if (`KismetArrayLibrary.Array_Contains` (`.IntPointArray_3_D0EC34214CC66367B6C657B38B50F0D6` (break `/Game/TacticGame/Blueprints/Core/Grid/Utilities/S_IntPointArray` (`BlueprintMapLibrary.Map_Find` (`/Game/TacticGame/Blueprints/Core/Grid/BP_Grid.TileStateToIndices` (`/Game/TacticGame/Blueprints/Core/Player/BP_PlayerActions.Grid` (`self.PlayerActions`))) "NewEnumerator8"))) (`/Game/TacticGame/Blueprints/Core/Player/BP_PlayerActions.HoveredTile` (`self.PlayerActions`)))
    ;[1 1 1] We make sure that the AoE has a pattern to draw on the grid
    (if (`|EnumInequality` (`.RangePattern_3_8F2F620549BE101B8A88079D92F4C347` (break `/Game/TacticGame/Blueprints/Core/Combat/Spells/Utilities/S_SpellData_Cast` (`self.CastAoe`))) "NewEnumerator0")
      ;[1 1 1] Then we can ask the combat system to give us the AoE target indices...
      (bind _rangeindices (`/Game/TacticGame/Blueprints/Core/Combat/BP_CombatSystem.GetSpellRange` (`/Game/TacticGame/Blueprints/Core/Player/BP_PlayerActions.CombatSystem` _playeractions) (`/Game/TacticGame/Blueprints/Core/Player/BP_PlayerActions.HoveredTile` _playeractions) (`self.CastAoe`)))
      ;[1 1 1] ...and for each of them we set the tile state to IsSpellRangeAoE
      (for _array_element _rangeindices
        (`/Game/TacticGame/Blueprints/Core/Grid/BP_Grid.AddStateToTile` (`/Game/TacticGame/Blueprints/Core/Player/BP_PlayerActions.Grid` (`self.PlayerActions`)) _array_element "NewEnumerator9"))
      (else
        ;[1 1 1] If there is no pattern, like a not AoE spell with a single target tile
        ; we show the appropriate color only on the hovered tile
        (`/Game/TacticGame/Blueprints/Core/Grid/BP_Grid.AddStateToTile` (`/Game/TacticGame/Blueprints/Core/Player/BP_PlayerActions.Grid` (`self.PlayerActions`)) (`/Game/TacticGame/Blueprints/Core/Player/BP_PlayerActions.HoveredTile` (`self.PlayerActions`)) "NewEnumerator9")))))

(fn `UserConstructionScript`
  (`parent.UserConstructionScript`))