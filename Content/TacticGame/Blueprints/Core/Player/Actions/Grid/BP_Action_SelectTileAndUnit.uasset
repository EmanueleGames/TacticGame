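; BP_Action_SelectTileAndUnit is a player grid action, derived from BP_Action, that selects a tile and unit.
; Its ExecuteAction override passes the tile index to PlayerActions.SetSelectedTileAndUnit without forcing.
; On End Play, such as when the Select Tile button is toggled off, it executes with an out-of-range sentinel index to clear the selection.
; End Play replaces Destroyed to avoid editor warnings.
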(event `self.ReceiveEndPlay`
  (params (EndPlayReason :type "EEndPlayReason Enum" :default "Destroyed"))
  ;[1 1 1] We use Event End Play and not Event Destroyed because the last is also called in the editor
  ; giving ug few warnings when closing the blueprint
  ;;[1 1 1 1 16] When the button Select Tile is toggled off
  ;; the Destroy is called and we want to reset the eventual Selected Tile
  ;; To do so, we select an invalid tile (-999,-999)
  (`self.ExecuteAction` (make `IntPoint` -999 -999)))

(fn `ExecuteAction`
  (params (Index :type "IntPoint Structure"))
  (`/Game/TacticGame/Blueprints/Core/Player/BP_PlayerActions.SetSelectedTileAndUnit` (`self.PlayerActions`) Index false))

(fn `UserConstructionScript`
  (`parent.UserConstructionScript`))