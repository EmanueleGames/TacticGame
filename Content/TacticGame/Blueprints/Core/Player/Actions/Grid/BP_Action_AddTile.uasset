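; BP_Action_AddTile is a player grid action that adds a new tile at a given grid index.
; ExecuteAction skips indices the Grid already holds, then traces for ground at that index's location to set the tile's height.
; It adds the tile through the player actions' Grid, using the grid's tile scale and a fixed tile type.
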(fn `ExecuteAction`
  (params (Index :type "IntPoint Structure"))
  (bind _grid (`/Game/TacticGame/Blueprints/Core/Player/BP_PlayerActions.Grid` (`self.PlayerActions`)))
  (if (not (`/Game/TacticGame/Blueprints/Core/Grid/BP_Grid.IsIndexValid` (`/Game/TacticGame/Blueprints/Core/Player/BP_PlayerActions.Grid` (`self.PlayerActions`)) (`local.Index`)))
    ;[1 1 1] Adjust the Z of the tile based on ground level
    (bind (_tiletype _outlocation) (`/Game/TacticGame/Blueprints/Core/Grid/BP_Grid.TraceForGround` (`/Game/TacticGame/Blueprints/Core/Player/BP_PlayerActions.Grid` (`self.PlayerActions`)) (`/Game/TacticGame/Blueprints/Core/Grid/BP_Grid.GetTileLocationFromGridIndex` _grid (`local.Index`))))
    (`/Game/TacticGame/Blueprints/Core/Grid/BP_Grid.AddGridTile` (`/Game/TacticGame/Blueprints/Core/Player/BP_PlayerActions.Grid` (`self.PlayerActions`)) (make `/Game/TacticGame/Blueprints/Core/Grid/Utilities/S_TileData` (`local.Index`) "NewEnumerator1" (`KismetMathLibrary.MakeTransform` _outlocation (struct) (`/Game/TacticGame/Blueprints/Core/Grid/BP_Grid.GetTileScale` _grid))))))

(fn `UserConstructionScript`
  (`parent.UserConstructionScript`))