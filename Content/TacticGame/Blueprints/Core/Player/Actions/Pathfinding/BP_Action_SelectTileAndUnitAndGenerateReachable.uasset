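; Player action for the tactics grid that, on execution, runs the parent action and then highlights the tiles reachable from the selected tile.
; It runs an asynchronous reachables search using the selected unit's stats, or its own pathfinding options when no unit is selected.
; A completion callback tags the returned tiles with a grid state.
; With a unit selected, walk events clear the highlight on departure and regenerate it on arrival.
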(fn `ExecuteAction`
  (params (Index :type "IntPoint Structure"))
  (`parent.ExecuteAction` Index)
  (`self.GenerateReachable`))

(fn `GenerateReachable`
  (bind _selectedunit (`/Game/TacticGame/Blueprints/Core/Player/BP_PlayerActions.SelectedUnit` (`self.PlayerActions`)))
  (bind (_validtiletypes _canmovediagonally _availablespells _hp_current _hp_max _mp_current) (break `/Game/TacticGame/Blueprints/Core/Units/Utilities/S_UnitData_Stats` (`.Stats_8_1FF4029D4CCC943B93A92087BC3004A2` (break `/Game/TacticGame/Blueprints/Core/Units/Utilities/S_UnitData` (`/Game/TacticGame/Blueprints/Core/Units/BP_Unit.UnitData` (`/Game/TacticGame/Blueprints/Core/Player/BP_PlayerActions.SelectedUnit` (`self.PlayerActions`)))))))
  ;[1 1 1] Clear old reachable array
  (`/Game/TacticGame/Blueprints/Core/Grid/BP_Grid.ClearStateFromTiles` (`/Game/TacticGame/Blueprints/Core/Player/BP_PlayerActions.Grid` (`self.PlayerActions`)) "NewEnumerator7")
  ;[1 1 1] Before calling FindPath, we attach ourself to the dispatcher that will signal us
  ; when the function is done building our reachable array
  (add `/Game/TacticGame/Blueprints/Core/Grid/BP_GridPathfinding.OnPathfindingCompleted` (`/Game/TacticGame/Blueprints/Core/Grid/BP_Grid.GridPathfinding_Reachables` (`/Game/TacticGame/Blueprints/Core/Player/BP_PlayerActions.Grid` (`self.PlayerActions`))) (`|CreateDelegate` :!event `OnPathfindingCompleted`))
  ;[1 1 1 1 16] We check if we have a valid unit selected.
  ; - VALID UNIT: we calculate the reachable based on the Unit data (max step, flying, etc.)
  ; - INVALID UNIT: we calculate the reachable based on the Widget options (max step, flying, etc.)
  (`/Engine/EditorBlueprintResources/StandardMacros.IsValid` (`/Game/TacticGame/Blueprints/Core/Player/BP_PlayerActions.SelectedUnit` (`self.PlayerActions`))
    (:`Is Valid`
      ;[1 1 1] Since we need to update the reachable tiles array when the unit moves, we bind to the proper events.
      ; - OnUnitStartedWalking will let us to clear the old reachable tile whem movement starts
      ; - OnUnitFinishedWalking will let us build the new reachable array when the unit stops
      (add `/Game/TacticGame/Blueprints/Core/Units/BP_Unit.OnUnitStartedWalking` _selectedunit (`|CreateDelegate` :!event `OnUnitStartedWalking`))
      (add `/Game/TacticGame/Blueprints/Core/Units/BP_Unit.OnUnitFinishedWalking` _selectedunit (`|CreateDelegate` :!event `OnUnitFinishedWalking`))
      ;[1 1 1] Find the new array of reachable tiles based on Unit Data
      (`/Game/TacticGame/Blueprints/Core/Grid/BP_GridPathfinding.FindPath` (`/Game/TacticGame/Blueprints/Core/Grid/BP_Grid.GridPathfinding_Reachables` (`/Game/TacticGame/Blueprints/Core/Player/BP_PlayerActions.Grid` (`self.PlayerActions`))) (`/Game/TacticGame/Blueprints/Core/Player/BP_PlayerActions.SelectedTile` (`self.PlayerActions`)) (make `IntPoint` -999 -999) _canmovediagonally _validtiletypes 0.0 0.0 true _mp_current))
    (:`Is Not Valid`
      ;[1 1 1] Find the new array of reachable tiles based on Pathfinding widget
      (`/Game/TacticGame/Blueprints/Core/Grid/BP_GridPathfinding.FindPath` (`/Game/TacticGame/Blueprints/Core/Grid/BP_Grid.GridPathfinding_Reachables` (`/Game/TacticGame/Blueprints/Core/Player/BP_PlayerActions.Grid` (`self.PlayerActions`))) (`/Game/TacticGame/Blueprints/Core/Player/BP_PlayerActions.SelectedTile` (`self.PlayerActions`)) (make `IntPoint` -999 -999) (`self.IncludeDiagonals`) (select `bool` (`self.IncludeFlyingOnly`) :`false` (`|MakeArray` "NewEnumerator1" "NewEnumerator3" "NewEnumerator4" :!type "/Game/TacticGame/Blueprints/Core/Grid/Utilities/E_TileType Enum") :`true` (`|MakeArray` "NewEnumerator1" "NewEnumerator3" "NewEnumerator4" "NewEnumerator5" :!type "/Game/TacticGame/Blueprints/Core/Grid/Utilities/E_TileType Enum")) (`self.DelayBetweenIterations`) (`self.MaxMsPerFrame`) true (`self.MaxPathLength`)))))

(fn `OnPathfindingCompleted`
  (params (Path :type "Array of IntPoint Structure (by ref)"))
  (for _array_element Path
    (`/Game/TacticGame/Blueprints/Core/Grid/BP_Grid.AddStateToTile` (`/Game/TacticGame/Blueprints/Core/Player/BP_PlayerActions.Grid` (`self.PlayerActions`)) _array_element "NewEnumerator7")))

(fn `OnUnitFinishedWalking`
  (params (Unit :type "/Game/TacticGame/Blueprints/Core/Units/BP_Unit Object Reference"))
  ;[1 1 1] When the unit arrives in a new tile
  ; generate the corresponding new reachable
  (`self.GenerateReachable`))

(fn `OnUnitStartedWalking`
  (params (Unit :type "/Game/TacticGame/Blueprints/Core/Units/BP_Unit Object Reference"))
  ;[1 1 1] When the unit moves, the old reachable are no more valid, lets clear them
  (`/Game/TacticGame/Blueprints/Core/Grid/BP_Grid.ClearStateFromTiles` (`/Game/TacticGame/Blueprints/Core/Player/BP_PlayerActions.Grid` (`self.PlayerActions`)) "NewEnumerator7"))

(fn `UserConstructionScript`
  (`parent.UserConstructionScript`))