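; BP_Action child for the tactics grid that marks the valid neighbors of a given tile.
; ExecuteAction clears the previous neighbor state, queries GridPathfinding with an optional diagonals setting and a set of allowed tile types, then adds that state to each result.
; EndPlay executes the action on an invalid index, so the highlighted neighbors reset when the action is toggled off and destroyed.
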(event `self.ReceiveEndPlay`
  (params (EndPlayReason :type "EEndPlayReason Enum" :default "Destroyed"))
  ;[1 1 1] We use Event End Play and not Event Destroyed because the last is also called in the editor
  ; giving ug few warnings when closing the blueprint
  ;;[1 1 1 1 16] When the button Show Tile Neighbors Tile is toggled off
  ;; the Destroy is called and we want to reset the eventual Selected Tile
  ;; To do so, we select an invalid tile (-999,-999)
  (`self.ExecuteAction` (make `IntPoint` -999 -999)))

(fn `ExecuteAction`
  (params (Index :type "IntPoint Structure"))
  ;[1 1 1] Clear old neighbors
  (`/Game/TacticGame/Blueprints/Core/Grid/BP_Grid.ClearStateFromTiles` (`/Game/TacticGame/Blueprints/Core/Player/BP_PlayerActions.Grid` (`self.PlayerActions`)) "NewEnumerator3")
  ;[1 1 1] Find the new neighbors
  (bind _retneighbors (`/Game/TacticGame/Blueprints/Core/Grid/BP_GridPathfinding.GetValidTileNeighbors` (`/Game/TacticGame/Blueprints/Core/Grid/BP_Grid.GridPathfinding` (`/Game/TacticGame/Blueprints/Core/Player/BP_PlayerActions.Grid` (`self.PlayerActions`))) Index (`self.IncludeDiagonals`) (`|MakeArray` "NewEnumerator1" "NewEnumerator3" "NewEnumerator4" "NewEnumerator5" :!type "/Game/TacticGame/Blueprints/Core/Grid/Utilities/E_TileType Enum")))
  ;[1 1 1] Add the IsNeighbor state to them
  (for _array_element _retneighbors
    (`/Game/TacticGame/Blueprints/Core/Grid/BP_Grid.AddStateToTile` (`/Game/TacticGame/Blueprints/Core/Player/BP_PlayerActions.Grid` (`self.PlayerActions`)) (break `/Game/TacticGame/Blueprints/Core/Grid/Utilities/S_PathfindingData` _array_element) "NewEnumerator3")))

(fn `UserConstructionScript`
  (`parent.UserConstructionScript`))