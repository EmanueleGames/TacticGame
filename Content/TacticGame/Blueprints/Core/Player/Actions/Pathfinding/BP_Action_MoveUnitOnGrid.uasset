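; Player action, a child of BP_Action, that moves the selected unit to a target tile for debugging, resetting its movement points after each move.
; ExecuteAction requests a path using the unit's movement stats and binds to pathfinding-completed and walk-finished events.
; On completion, if the selection is unchanged, it highlights the path and has CombatSystem move the unit.
; The highlight clears when walking finishes; EndPlay executes with an invalid tile to reset.
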(event `self.ReceiveEndPlay`
  (params (EndPlayReason :type "EEndPlayReason Enum" :default "Destroyed"))
  ;[1 1 1] We use Event End Play and not Event Destroyed because the last is also called in the editor
  ; giving ug few warnings when closing the blueprint
  ;;[1 1 1 1 16] When the button Find Path To Target is toggled off
  ;; the Destroy is called and we want to reset the eventual Selected Tile
  ;; To do so, we select an invalid tile (-999,-999)
  (`self.ExecuteAction` (make `IntPoint` -999 -999)))

(fn `ExecuteAction`
  (params (Index :type "IntPoint Structure"))
  (bind (_validtiletypes _canmovediagonally _availablespells _hp_current _hp_max _mp_current) (break `/Game/TacticGame/Blueprints/Core/Units/Utilities/S_UnitData_Stats` (`.Stats_8_1FF4029D4CCC943B93A92087BC3004A2` (break `/Game/TacticGame/Blueprints/Core/Units/Utilities/S_UnitData` (`/Game/TacticGame/Blueprints/Core/Units/BP_Unit.UnitData` (`self.CurrentUnit`))))))
  ;[1 1 1] Clear old path
  (`/Game/TacticGame/Blueprints/Core/Grid/BP_Grid.ClearStateFromTiles` (`/Game/TacticGame/Blueprints/Core/Player/BP_PlayerActions.Grid` (`self.PlayerActions`)) "NewEnumerator4")
  ;[1 1 1] We make sure to have a valid Unit selected
  (bind _output_get (set `self.CurrentUnit` (`/Game/TacticGame/Blueprints/Core/Player/BP_PlayerActions.SelectedUnit` (`self.PlayerActions`))))
  (`/Engine/EditorBlueprintResources/StandardMacros.IsValid` _output_get
    (:`Is Valid`
      ;[1 1 1] We hook ourself to the event to get notified when the movement is over
      (add `/Game/TacticGame/Blueprints/Core/Units/BP_Unit.OnUnitFinishedWalking` (`self.CurrentUnit`) (`|CreateDelegate` :!event `OnUnitFinishedWalking`))
      ;[1 1 1] Before calling FindPath, we attach ourself to the dispatcher that will signal us
      ; when the function is done building our path
      (add `/Game/TacticGame/Blueprints/Core/Grid/BP_GridPathfinding.OnPathfindingCompleted` (`/Game/TacticGame/Blueprints/Core/Grid/BP_Grid.GridPathfinding` (`/Game/TacticGame/Blueprints/Core/Player/BP_PlayerActions.Grid` (`self.PlayerActions`))) (`|CreateDelegate` :!event `OnPathfindingCompleted`))
      ;[1 1 1] Find the new path
      (`/Game/TacticGame/Blueprints/Core/Grid/BP_GridPathfinding.FindPath` (`/Game/TacticGame/Blueprints/Core/Grid/BP_Grid.GridPathfinding` (`/Game/TacticGame/Blueprints/Core/Player/BP_PlayerActions.Grid` (`self.PlayerActions`))) (`/Game/TacticGame/Blueprints/Core/Player/BP_PlayerActions.SelectedTile` (`self.PlayerActions`)) (`local.Index`) _canmovediagonally _validtiletypes 0.0 0.0 false _mp_current))))

(fn `OnPathfindingCompleted`
  (params (Path :type "Array of IntPoint Structure"))
  (bind _currentunit (`self.CurrentUnit`))
  ;[1 1 1] If finding the path took too much time we check if the selected Unit is still valid again. All this because the player could have deselected or chose another one during the pathfinding
  (`/Engine/EditorBlueprintResources/StandardMacros.IsValid` (`self.CurrentUnit`)
    (:`Is Valid`
      ;[1 1 1 1 16] We compare the CurrentUnit (the one in execution) with the SelectedUnit.
      ; This because if the player chages selection during the pathfinding, we don't wanna to execute the rest of the code.
      (if (== (`self.CurrentUnit`) (`/Game/TacticGame/Blueprints/Core/Player/BP_PlayerActions.SelectedUnit` (`self.PlayerActions`)))
        (for _array_element (`local.Path`)
          (`/Game/TacticGame/Blueprints/Core/Grid/BP_Grid.AddStateToTile` (`/Game/TacticGame/Blueprints/Core/Player/BP_PlayerActions.Grid` (`self.PlayerActions`)) _array_element "NewEnumerator4"))
        ;[1 1 1] Pathfinding completed, time to set the move duration and ask the CombatSystem to move the Unit
        (set `/Game/TacticGame/Blueprints/Core/Units/BP_Unit.MoveDurationPerTile` (`self.MoveDuration`) _currentunit)
        (`/Game/TacticGame/Blueprints/Core/Combat/BP_CombatSystem.MoveUnit` (`/Game/TacticGame/Blueprints/Core/Player/BP_PlayerActions.CombatSystem` (`self.PlayerActions`)) _currentunit (`local.Path`))
        ;[1 1 1] Since this is a Debugging action, we reset the Unit movement after each move
        ; no need to limit it like in Combat turns
        (`/Game/TacticGame/Blueprints/Core/Units/BP_Unit.ResetMp` (`self.CurrentUnit`))))))

(fn `OnUnitFinishedWalking`
  (params (Unit :type "/Game/TacticGame/Blueprints/Core/Units/BP_Unit Object Reference"))
  (if (== Unit (`self.CurrentUnit`))
    ;[1 1 1] Ok, then we can delete the path drawn on the tiles
    (`/Game/TacticGame/Blueprints/Core/Grid/BP_Grid.ClearStateFromTiles` (`/Game/TacticGame/Blueprints/Core/Player/BP_PlayerActions.Grid` (`self.PlayerActions`)) "NewEnumerator4")))

(fn `UserConstructionScript`
  (`parent.UserConstructionScript`))