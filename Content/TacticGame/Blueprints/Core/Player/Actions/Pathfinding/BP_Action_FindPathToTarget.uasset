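; Player action, child of BP_Action, that finds a path on the tactics grid from the selected tile to a target tile and marks it.
; ExecuteAction clears the old path state and calls GridPathfinding's FindPath with options for diagonals, flying-only tiles, length and per-frame pacing.
; The OnPathfindingCompleted callback applies the path state to each returned tile.
; Selection changes and EndPlay execute the action on an invalid tile to clear the path.
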(event `self.ReceiveBeginPlay`
  (add `/Game/TacticGame/Blueprints/Core/Player/BP_PlayerActions.OnSelectedTileChanged` (`self.PlayerActions`) (delegate `OnSelectedTileChanged`)) ; we want be notified on Tile Selection to remove the old path
)

(event `OnSelectedTileChanged`
  (params (Index :type "IntPoint Structure"))
  ;[1 1 1 1 16] When we change tile selection
  ; We want to reset the eventual Selected Tile
  ; To do so, we select an invalid tile (-999,-999)
  (`self.ExecuteAction` (make `IntPoint` -999 -999)))

(event `self.ReceiveEndPlay`
  (params (EndPlayReason :type "EEndPlayReason Enum" :default "Destroyed"))
  ;[1 1 1] We use Event End Play and not Event Destroyed because the last is also called in the editor
  ; giving ug few warnings when closing the blueprint
  ;;[1 1 1 1 16] When the button Find Path To Target is toggled off
  ;; the Destroy is called and we want to reset the eventual Selected Tile
  ;; To do so, we select an invalid tile (-999,-999)
  (`self.ExecuteAction` (make `IntPoint` -999 -999)))

(fn `ExecuteAction`
  (params (Index :type "IntPoint Structure"))
  ;[1 1 1] Clear old path
  (`/Game/TacticGame/Blueprints/Core/Grid/BP_Grid.ClearStateFromTiles` (`/Game/TacticGame/Blueprints/Core/Player/BP_PlayerActions.Grid` (`self.PlayerActions`)) "NewEnumerator4")
  ;[1 1 1] Before calling FindPath, we attach ourself to the dispatcher that will signal us
  ; when the function is done building our path
  (add `/Game/TacticGame/Blueprints/Core/Grid/BP_GridPathfinding.OnPathfindingCompleted` (`/Game/TacticGame/Blueprints/Core/Grid/BP_Grid.GridPathfinding` (`/Game/TacticGame/Blueprints/Core/Player/BP_PlayerActions.Grid` (`self.PlayerActions`))) (`|CreateDelegate` :!event `OnPathfindingCompleted`))
  ;[1 1 1] Find the new path
  (`/Game/TacticGame/Blueprints/Core/Grid/BP_GridPathfinding.FindPath` (`/Game/TacticGame/Blueprints/Core/Grid/BP_Grid.GridPathfinding` (`/Game/TacticGame/Blueprints/Core/Player/BP_PlayerActions.Grid` (`self.PlayerActions`))) (`/Game/TacticGame/Blueprints/Core/Player/BP_PlayerActions.SelectedTile` (`self.PlayerActions`)) Index (`self.IncludeDiagonals`) (select `bool` (`self.IncludeFlyingOnly`) :`false` (`|MakeArray` "NewEnumerator1" "NewEnumerator3" "NewEnumerator4" :!type "/Game/TacticGame/Blueprints/Core/Grid/Utilities/E_TileType Enum") :`true` (`|MakeArray` "NewEnumerator1" "NewEnumerator3" "NewEnumerator4" "NewEnumerator5" :!type "/Game/TacticGame/Blueprints/Core/Grid/Utilities/E_TileType Enum")) (`self.DelayBetweenIterations`) (`self.MaxMsPerFrame`) false (`self.MaxPathLength`)))

(fn `OnPathfindingCompleted`
  (params (Path :type "Array of IntPoint Structure"))
  (for _array_element Path
    (`/Game/TacticGame/Blueprints/Core/Grid/BP_Grid.AddStateToTile` (`/Game/TacticGame/Blueprints/Core/Player/BP_PlayerActions.Grid` (`self.PlayerActions`)) _array_element "NewEnumerator4")))

(fn `UserConstructionScript`
  (`parent.UserConstructionScript`))