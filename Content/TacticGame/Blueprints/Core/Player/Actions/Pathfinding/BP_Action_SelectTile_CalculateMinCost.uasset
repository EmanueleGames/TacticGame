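; Player action for the tactics grid that extends tile selection by computing the minimum cost from every tile to the selected one.
; ExecuteAction runs the parent behaviour, then clears GridPathfinding's generated data.
; If the selected tile is valid, it discovers every grid tile with zero cost from start and its minimum cost to the selection, optionally counting diagonals.
; It runs no path search, only this per-tile estimate.
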(fn `ExecuteAction`
  (params (Index :type "IntPoint Structure"))
  (bind _playeractions (`self.PlayerActions`))
  (bind _playeractions_2 (`self.PlayerActions`))
  (bind _grid (`/Game/TacticGame/Blueprints/Core/Player/BP_PlayerActions.Grid` _playeractions))
  ;[1 1 1] This BP Action is child of Select Tile and Unit, so when selected we want to keep the parent behaviour and do also other things
  (`parent.ExecuteAction` Index)
  ;[1 1 1] We clear generated data before we create new one
  (`/Game/TacticGame/Blueprints/Core/Grid/BP_GridPathfinding.ClearGeneratedData` (`/Game/TacticGame/Blueprints/Core/Grid/BP_Grid.GridPathfinding` (`/Game/TacticGame/Blueprints/Core/Player/BP_PlayerActions.Grid` (`self.PlayerActions`))))
  ;[1 1 1] Check if index is valid
  (if (`/Game/TacticGame/Blueprints/Core/Grid/BP_Grid.IsIndexValid` (`/Game/TacticGame/Blueprints/Core/Player/BP_PlayerActions.Grid` _playeractions_2) (`/Game/TacticGame/Blueprints/Core/Player/BP_PlayerActions.SelectedTile` _playeractions_2))
    ;[1 1 1] we get every Tile on the Grid
    (bind _keys (`BlueprintMapLibrary.Map_Keys` (`/Game/TacticGame/Blueprints/Core/Grid/BP_Grid.GridTiles` _grid)))
    ;[1 1 1] We then loop on every Tile and Discover it, generating pathfinding data.
    ; At the same time we generate the cost between every looped Tile and the selected one
    (for _array_element _keys
      (`/Game/TacticGame/Blueprints/Core/Grid/BP_GridPathfinding.DiscoverTile` (`/Game/TacticGame/Blueprints/Core/Grid/BP_Grid.GridPathfinding` (`/Game/TacticGame/Blueprints/Core/Player/BP_PlayerActions.Grid` (`self.PlayerActions`))) (make `/Game/TacticGame/Blueprints/Core/Grid/Utilities/S_PathfindingData` _array_element 1 0 (`/Game/TacticGame/Blueprints/Core/Grid/BP_GridPathfinding.GetMinimumCostBetweenTwoTiles` (`/Game/TacticGame/Blueprints/Core/Grid/BP_Grid.GridPathfinding` _grid) _array_element (`/Game/TacticGame/Blueprints/Core/Player/BP_PlayerActions.SelectedTile` _playeractions) (`self.IncludeDiagonals`)))))))

(fn `UserConstructionScript`
  (`parent.UserConstructionScript`))