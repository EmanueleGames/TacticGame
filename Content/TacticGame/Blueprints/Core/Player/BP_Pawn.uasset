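; BP_Pawn is the player's camera pawn for the tactics game, handling panning, zooming and yaw rotation.
; Enhanced Input actions, mapped on BeginPlay, update target location, rotation and a clamped spring arm length.
; Tick interpolates the actor transform and arm length toward those targets for smooth motion.
; A separate event applies a yaw step for main menu rotation, and the old axis input events are empty, deprecated stubs.
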(event `self.ReceiveBeginPlay`
  ;[1 1 1] Variables starting values
  (set `self.LocationDesired` (`self.K2_GetActorLocation`))
  (set `self.ZoomValue` (`SpringArmComponent.TargetArmLength` (`self.SpringArm`)))
  (set `self.RotationDesired` (`self.K2_GetActorRotation`))
  ;[1 1 1] Set the Input Mapping Context relative to our Enhanced Inputs
  (message `EnhancedInputSubsystemInterface.AddMappingContext` (pcsubsystem `EnhancedInputLocalPlayerSubsystem` (cast `PlayerController` (`self.GetOwner`) :!pure true)) "/Game/TacticGame/Blueprints/Core/Player/Inputs/IMC_Default.IMC_Default" 0 (struct)))

(event `self.ReceiveTick`
  (params (DeltaSeconds :type "Float (single-precision)"))
  (bind _springarm (`self.SpringArm`))
  ;[1 1 1] Interpolation to final values
  (set `SpringArmComponent.TargetArmLength` (`KismetMathLibrary.FInterpTo` (`SpringArmComponent.TargetArmLength` _springarm) (`self.ZoomValue`) DeltaSeconds (`self.ZoomInterpSpeed`)) _springarm)
  (`self.K2_SetActorLocation` (`KismetMathLibrary.VInterpTo` (`self.K2_GetActorLocation`) (`self.LocationDesired`) DeltaSeconds (`self.LocationInterpSpeed`)))
  (`self.K2_SetActorRotation` (`KismetMathLibrary.RInterpTo` (`self.K2_GetActorRotation`) (`self.RotationDesired`) DeltaSeconds (`self.RotationInterpSpeed`))))

(event `InputAxis|InputAxis_Zoom`
  (params (AxisValue :type "Float (single-precision)")))

(event `EnhancedInput|/Game/TacticGame/Blueprints/Core/Player/Inputs/IA_Camera_Zoom`
  (params (ActionValue :type "Float (double-precision)") (ElapsedSeconds :type "Float (double-precision)") (TriggeredSeconds :type "Float (double-precision)") (InputAction :type "InputAction Object Reference" :default "/Game/TacticGame/Blueprints/Core/Player/Inputs/IA_Camera_Zoom.IA_Camera_Zoom"))
  ;[1 1 1] Enhanced Input to set variables
  (:`Triggered`
    (set `self.ZoomValue` (`KismetMathLibrary.FClamp` (+ (`self.ZoomValue`) (* ActionValue (`self.ZoomSpeed`))) (`self.ZoomMin`) (`self.ZoomMax`)))))

(event `InputAxis|InputAxis_Forward`
  (params (AxisValue :type "Float (single-precision)")))

(event `EnhancedInput|/Game/TacticGame/Blueprints/Core/Player/Inputs/IA_Camera_Move`
  (params (ActionValue :type "Vector2D Structure") (ElapsedSeconds :type "Float (double-precision)") (TriggeredSeconds :type "Float (double-precision)") (InputAction :type "InputAction Object Reference" :default "/Game/TacticGame/Blueprints/Core/Player/Inputs/IA_Camera_Move.IA_Camera_Move"))
  (bind (_returnvalue_x _returnvalue_y) (`KismetMathLibrary.BreakVector2D` (`KismetMathLibrary.Normal2D` ActionValue)))
  ;[1 1 1] Enhanced Input to set variables
  (:`Triggered`
    (set `self.LocationDesired` (+ (* (* _returnvalue_x (`self.LocationSpeed`)) (`self.GetActorForwardVector`)) (`self.LocationDesired`) (* (* _returnvalue_y (`self.LocationSpeed`)) (`self.GetActorRightVector`))))))

(event `InputAxis|InputAxis_Right`
  (params (AxisValue :type "Float (single-precision)")))

(event `InputAction|InputAction_RotationRight`
  (params (Key :type "Key Structure")))

(event `EnhancedInput|/Game/TacticGame/Blueprints/Core/Player/Inputs/IA_Camera_Rotate`
  (params (ActionValue :type "Float (double-precision)") (ElapsedSeconds :type "Float (double-precision)") (TriggeredSeconds :type "Float (double-precision)") (InputAction :type "InputAction Object Reference" :default "/Game/TacticGame/Blueprints/Core/Player/Inputs/IA_Camera_Rotate.IA_Camera_Rotate"))
  ;[1 1 1] Enhanced Input to set variables
  (:`Triggered`
    (set `self.RotationDesired` (`KismetMathLibrary.ComposeRotators` (`self.RotationDesired`) (`KismetMathLibrary.MakeRotator` 0.0 0.0 (* ActionValue (`self.RotationSpeed`)))))))

(event `InputAction|InputAction_RotationLeft`
  (params (Key :type "Key Structure")))

(event `Event_MainMenuRotation`
  ;[1 1 1] By Finn - For MainMenu rotation
  (set `self.RotationDesired` (`self.K2_GetActorRotation`))
  (set `self.RotationDesired` (`KismetMathLibrary.ComposeRotators` (`self.RotationDesired`) (`KismetMathLibrary.MakeRotator` 0.0 0.0 (`self.RotationSpeedMainMenu`)))))

(fn `UserConstructionScript`)