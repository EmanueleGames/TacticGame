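; Base actor for a spell's visual animation in the tactics grid combat, with a default play event meant to be overridden per spell.
; On BeginPlay it spawns one BP_AnimatedShape per attacked tile, using the grid's shape mesh with randomized red tint and play rate, growing from the origin tile toward its target.
; Each arrival broadcasts a tile hit; the last broadcasts completion and destroys the actor.
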(event `self.ReceiveBeginPlay`
  (`self.Event_PlaySpellAnimation`))

(event `Event_PlaySpellAnimation`
  (bind (_transform_location _transform_rotation) (`KismetMathLibrary.BreakTransform` (`self.GetTileTransform` (`self.OriginIndex`))))
  (bind (_meshsize _mesh _meshmaterial) (break `/Game/TacticGame/Blueprints/Core/Grid/GridShapes/S_GridShapeData` (`/Game/TacticGame/Blueprints/Core/Grid/BP_Grid.GetCurrentShapeData` (`self.Grid`))))
  ;[1 1 1] In case the spell is an AoE
  ; we have to loop on all the Target Tiles
  (for _array_element (`self.AttackIndexes`)
    (bind _returnvalue (`|SpawnActorFromClass` "/Game/TacticGame/Blueprints/Core/Combat/Spells/SpellAnimations/Components/BP_AnimatedShape.BP_AnimatedShape_C" (`KismetMathLibrary.MakeTransform` (0.0 0.0 0.0)) "AlwaysSpawn" "MultiplyWithRoot" null _mesh _meshmaterial (* (struct :`R` 0.671875 :`G` 0.018865 :`A` 1.0) (`KismetMathLibrary.RandomFloatInRange` 0.5 1.5)) (`KismetMathLibrary.MakeTransform` _transform_location _transform_rotation (0.01 0.01 0.01)) (`self.GetTileTransform` _array_element) (`KismetMathLibrary.RandomFloatInRange` 0.5 1.0) _array_element null))
    ;[1 1 1] We need to be notified when the animation is completed to destroy the instance of this Blueprint used to perform the animation
    (add `/Game/TacticGame/Blueprints/Core/Combat/Spells/SpellAnimations/Components/BP_AnimatedShape.OnShapeAnimationCompleted` _returnvalue (delegate `OnShapeAnimationCompleted`))))

(event `OnShapeAnimationCompleted`
  (params (AnimatedShape :type "/Game/TacticGame/Blueprints/Core/Combat/Spells/SpellAnimations/Components/BP_AnimatedShape Object Reference"))
  (bind _index (`/Game/TacticGame/Blueprints/Core/Combat/Spells/SpellAnimations/Components/BP_AnimatedShape.Index` AnimatedShape))
  (bind _attackindexes (`self.AttackIndexes`))
  ;[1 1 1] This notify the eventual Units hit by the spell to play their Hit animation when the spell reaches the Target Tile
  (`self.OnSpellAnimationHitTile` self _index)
  ;[1 1 1 1 16] To keep track of all the tiles examined/still to process of the current attack,
  ; we remove the Tile just processed from the AttackedIndices
  (`KismetArrayLibrary.Array_RemoveItem` _attackindexes _index)
  ;[1 1 1] When all the AttackIndices have been processed
  ; it means we're done with the spell
  (if (== (`KismetArrayLibrary.Array_Length` _attackindexes) 0)
    (`self.Event_CompleteSpellAnimation`) ; Notify the end of the animation
  ))

(event `Event_CompleteSpellAnimation`
  (`self.OnSpellAnimationCompleted` self) ; Used to notify the end of the Spell Animation
  ;[1 1 1] After all the notification
  ; we can safely destroy the actor
  (`self.K2_DestroyActor`))

(fn `GetTileTransform`
  (params (Index :type "IntPoint Structure (by ref)"))
  (returns (Transform :type "Transform Structure"))
  (return (`.Transform_7_D016BDCC41B32F0EC4D85EB94D99E603` (break `/Game/TacticGame/Blueprints/Core/Grid/Utilities/S_TileData` (`BlueprintMapLibrary.Map_Find` (`/Game/TacticGame/Blueprints/Core/Grid/BP_Grid.GridTiles` (`self.Grid`)) Index)))))

(fn `UserConstructionScript`)