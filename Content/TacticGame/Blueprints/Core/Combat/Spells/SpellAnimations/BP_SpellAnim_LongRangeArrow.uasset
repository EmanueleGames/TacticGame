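; BP_SpellAnim_LongRangeArrow is a spell animation that flies an arrow in an arc from the origin tile to the target tile.
; It overrides the play event to face the target, then a timeline lerps position with a height offset while driving pitch and scale on a child component.
; Past a playback threshold it fires the tile-hit notification once, and completes the spell animation when the timeline finishes.
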(event `self.Event_PlaySpellAnimation`
  (bind _anim_rotationscale (`self.Anim_RotationScale`))
  (bind _transform_location (`KismetMathLibrary.BreakTransform` (`self.GetTileTransform` (`self.OriginIndex`))))
  (bind _transform_location_2 (`KismetMathLibrary.BreakTransform` (`self.GetTileTransform` (`self.TargetIndex`))))
  (bind _transform_location_3 (`KismetMathLibrary.BreakTransform` (`self.GetTileTransform` (`self.OriginIndex`))))
  ;[1 1 1] We position and orient the arrow from the OriginIndex to the TargetIndex
  (`self.K2_SetActorLocationAndRotation` _transform_location_3 (`KismetMathLibrary.FindLookAtRotation` (`KismetMathLibrary.Conv_Vector2DToVector` (`KismetMathLibrary.Conv_IntPointToVector2D` (`self.OriginIndex`))) (`KismetMathLibrary.Conv_Vector2DToVector` (`KismetMathLibrary.Conv_IntPointToVector2D` (`self.TargetIndex`)))))
  (bind (_direction _actorlocationalpha _locationz _rotationy _scale) (`Timeline|Timeline_LongArrow` :!via `PlayFromStart`)
    (:`Update`
      ;[1 1 1] We give the arrow a projectile motion, it reaches the target like a curve
      (`self.K2_SetActorLocation` (+ (`KismetMathLibrary.VLerp` _transform_location _transform_location_2 _actorlocationalpha) (`KismetMathLibrary.MakeVector` 0.0 0.0 _locationz)))
      ;[1 1 1] We make arrow point in the correct direction during its curve
      (`SceneComponent.K2_SetRelativeRotation` _anim_rotationscale (`KismetMathLibrary.MakeRotator` 0.0 _rotationy) false false)
      ;[1 1 1] Arrow gets slighly bigger moving
      (`SceneComponent.SetRelativeScale3D` _anim_rotationscale (`KismetMathLibrary.Conv_DoubleToVector` _scale))
      ;[1 1 1] At the proper time during the timeline (depends on the spell)
      (if (>= (`TimelineComponent.GetPlaybackPosition` (`self.Timeline_LongArrow`)) 0.65)
        ;[1 1 1] Notify (just once) that we hit the tile (so the Unit can play the Hit animation)
        (`/Engine/EditorBlueprintResources/StandardMacros.DoOnce` false
          (:`Completed`
            (`self.OnSpellAnimationHitTile` self (`self.TargetIndex`))))))
    (:`Finished`
      ;[1 1 1] Responsable to destroy the BP when Animation ends
      (`self.Event_CompleteSpellAnimation`))))

(fn `UserConstructionScript`
  (`parent.UserConstructionScript`))