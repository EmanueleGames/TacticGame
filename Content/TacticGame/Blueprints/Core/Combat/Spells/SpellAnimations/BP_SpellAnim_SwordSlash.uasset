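; Spell animation actor that plays a sword slash from the caster's tile toward a target tile in the tactics game.
; Overrides the play event to place the actor at the origin tile facing the target, then runs a timeline that pitches and scales the sword.
; Partway through the swing it fires the hit-tile notification once so the unit can react, then completes the animation when the timeline finishes.
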(event `self.Event_PlaySpellAnimation`
  (bind _anim_rotationscale (`self.Anim_RotationScale`))
  (bind _transform_location (`KismetMathLibrary.BreakTransform` (`self.GetTileTransform` (`self.OriginIndex`))))
  ;[1 1 1] We position and orient the sword from the OriginIndex to the TargetIndex
  (`self.K2_SetActorLocationAndRotation` _transform_location (`KismetMathLibrary.FindLookAtRotation` (`KismetMathLibrary.Conv_Vector2DToVector` (`KismetMathLibrary.Conv_IntPointToVector2D` (`self.OriginIndex`))) (`KismetMathLibrary.Conv_Vector2DToVector` (`KismetMathLibrary.Conv_IntPointToVector2D` (`self.TargetIndex`)))))
  (bind (_direction _rotationy _scale) (`Timeline|Timeline_SwordSwing` :!via `PlayFromStart`)
    (:`Update`
      ;[1 1 1] During the Timeline the animation will rotate and scale the Sword Mesh
      (`SceneComponent.K2_SetRelativeRotation` _anim_rotationscale (`KismetMathLibrary.MakeRotator` 0.0 _rotationy) false false) ; The swing is animated only along the Y axis
      (`SceneComponent.SetRelativeScale3D` _anim_rotationscale (`KismetMathLibrary.Conv_DoubleToVector` _scale)) ; For the scale, we make it bigger first, then smaller
      ;[1 1 1] At the proper time during the timeline (depends on the spell)
      (if (>= (`TimelineComponent.GetPlaybackPosition` (`self.Timeline_SwordSwing`)) 0.4)
        ;[1 1 1] Notify (just once) that we hit the tile (so the Unit can play the Hit animation)
        (`/Engine/EditorBlueprintResources/StandardMacros.DoOnce` false
          (:`Completed`
            (`self.OnSpellAnimationHitTile` self (`self.TargetIndex`))))))
    (:`Finished`
      ;[1 1 1] Responsable to destroy the BP when Animation ends
      (`self.Event_CompleteSpellAnimation`))))

(fn `UserConstructionScript`
  (`parent.UserConstructionScript`))