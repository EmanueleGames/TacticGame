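; Spell animation actor for Dark Wave, a point-blank area spell that appears on the target tile in the tactics game.
; A timeline scales the wave and fades the opacity of its three mesh layers, which the construction script tints in dark purple shades.
; Shortly into playback, a DoOnce reports a hit on every attacked tile so units can react.
; When the timeline finishes, it completes the spell animation.
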(event `self.Event_PlaySpellAnimation`
  (bind _transform_location (`KismetMathLibrary.BreakTransform` (`self.GetTileTransform` (`self.TargetIndex`))))
  ;[1 1 1] We position the Wave on the Target Tile (Point Blank AoE)
  (`self.K2_SetActorLocation` _transform_location)
  (bind (_direction _opacity _scale) (`Timeline|Timeline_DarkWave` :!via `PlayFromStart`)
    (:`Update`
      ;[1 1 1] We animate the Wave scaling it
      (`SceneComponent.SetRelativeScale3D` (`self.Anim_Scale`) _scale)
      ;[1 1 1] And we play with the opacity to animate the Wave
      (`MeshComponent.SetScalarParameterValueOnMaterials` (`self.StaticMesh_Inner`) "Opacity" _opacity)
      (`MeshComponent.SetScalarParameterValueOnMaterials` (`self.StaticMesh_Middle`) "Opacity" _opacity)
      (`MeshComponent.SetScalarParameterValueOnMaterials` (`self.StaticMesh_Outer`) "Opacity" _opacity)
      ;[1 1 1] At the proper time during the timeline (depends on the spell)
      (if (>= (`TimelineComponent.GetPlaybackPosition` (`self.Timeline_DarkWave`)) 0.2)
        ;[1 1 1] Notify (just once) that we hit the tile (so the Unit can play the Hit animation)
        (`/Engine/EditorBlueprintResources/StandardMacros.DoOnce` false
          (:`Completed`
            (for _array_element (`self.AttackIndexes`)
              (`self.OnSpellAnimationHitTile` self _array_element))))))
    (:`Finished`
      ;[1 1 1] Responsable to destroy the BP when Animation ends
      (`self.Event_CompleteSpellAnimation`))))

(fn `UserConstructionScript`
  (`parent.UserConstructionScript`)
  (`MeshComponent.SetVectorParameterValueOnMaterials` (`self.StaticMesh_Inner`) "Color" (`KismetMathLibrary.Conv_LinearColorToVector` (struct :`R` 0.129412 :`B` 0.14902 :`A` 1.0)))
  (`MeshComponent.SetVectorParameterValueOnMaterials` (`self.StaticMesh_Middle`) "Color" (`KismetMathLibrary.Conv_LinearColorToVector` (struct :`R` 0.063322 :`B` 0.072917 :`A` 1.0)))
  (`MeshComponent.SetVectorParameterValueOnMaterials` (`self.StaticMesh_Outer`) "Color" (`KismetMathLibrary.Conv_LinearColorToVector` (struct :`R` 0.018092 :`B` 0.020833 :`A` 1.0))))