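; Debug overlay actor for the tactics grid that shows per-tile text and pathfinding state colors.
; It binds to BP_Grid and GridPathfinding dispatchers, keeping debug updates out of the game loop.
; Toggle setters refresh all tiles, using one TextRenderActor per index, scaled to tile size and longest entry, for indices, type and pathfinding costs.
; Discovered and analysed pathfinding tiles are marked through grid tile states.
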(event `self.ReceiveBeginPlay`
  (bind _gridpathfinding (`/Game/TacticGame/Blueprints/Core/Grid/BP_Grid.GridPathfinding` (`self.Grid`)))
  (bind _gridpathfinding_2 (`/Game/TacticGame/Blueprints/Core/Grid/BP_Grid.GridPathfinding` (`self.Grid`)))
  (bind _returnvalue (`GameplayStatics.GetActorOfClass` "/Game/TacticGame/Blueprints/Core/Grid/BP_Grid.BP_Grid_C"))
  (bind _output_get (set `self.Grid` _returnvalue))
  ;[1 1 1] Since the text containing the tile indices are only for debug use,
  ; we add them by using events.
  ; We listen to these three events (whose dispatchers are in the BP_Grid)
  ; to get notified everytime a tile is added/removed/modified or the grid is destroyed
  (add `/Game/TacticGame/Blueprints/Core/Grid/BP_Grid.OnTileDataUpdated` _output_get (`|CreateDelegate` :!event `UpdateTextOnTile`))
  (add `/Game/TacticGame/Blueprints/Core/Grid/BP_Grid.OnTileStateUpdated` _output_get (`|CreateDelegate` :!event `UpdateStateOnTile`))
  (add `/Game/TacticGame/Blueprints/Core/Grid/BP_Grid.OnGridDestroyed` _output_get (`|CreateDelegate` :!event `ClearAllTextActors`))
  ;[1 1 1] Same reason as before. We only use Tile States for debug use, so we add them with events
  ; We listen to these two events (whose dispatchers are in the BP_GridPathfinding)
  ; to get notified everytime the states/colors needs to be updated
  (add `/Game/TacticGame/Blueprints/Core/Grid/BP_GridPathfinding.OnPathfindingDataUpdated` _gridpathfinding_2 (`|CreateDelegate` :!event `UpdateStateOnTile`))
  (add `/Game/TacticGame/Blueprints/Core/Grid/BP_GridPathfinding.OnPathfindingDataCleared` _gridpathfinding_2 (`|CreateDelegate` :!event `UpdateStateOnAllTiles`))
  ;[1 1 1] Same reason as before. We only use Text Actors for debug use, so we add them with events
  ; We listen to these two events (whose dispatchers are in the BP_GridPathfinding)
  ; to get notified everytime the text needs to be updated
  (add `/Game/TacticGame/Blueprints/Core/Grid/BP_GridPathfinding.OnPathfindingDataUpdated` _gridpathfinding (`|CreateDelegate` :!event `UpdateTextOnTile`))
  (add `/Game/TacticGame/Blueprints/Core/Grid/BP_GridPathfinding.OnPathfindingDataCleared` _gridpathfinding (`|CreateDelegate` :!event `UpdateTextOnAllTiles`)))

(fn `ClearAllTextActors`
  ;[1 1 1] Clear all the map of Indices and TextActors, and destroy all the corresponding TextActors.
  ; Useful when we destroy the entire grid
  (bind _values (`BlueprintMapLibrary.Map_Values` (`self.SpawnedTexts`)))
  (for _array_element _values
    (`self.K2_DestroyActor` _array_element))
  (`BlueprintMapLibrary.Map_Clear` (`self.SpawnedTexts`)))

(fn `DestroyTextActor`
  (params (Index :type "IntPoint Structure"))
  (locals (Actor :type "TextRenderActor Object Reference"))
  ;[1 1 1] If we find a valid entry in our map for the index in input
  (bind _output_get (set `local.Actor` (`BlueprintMapLibrary.Map_Find` (`self.SpawnedTexts`) Index)))
  (`/Engine/EditorBlueprintResources/StandardMacros.IsValid` _output_get
    (:`Is Valid`
      ;[1 1 1] we destroy the actor and remove the entry from the map
      (`self.K2_DestroyActor` _output_get)
      (`BlueprintMapLibrary.Map_Remove` (`self.SpawnedTexts`) (`local.Index`)))))

(fn `GetTextActor`
  (params (Index :type "IntPoint Structure"))
  (returns (TextRenderedActor :type "TextRenderActor Object Reference"))
  (locals (TextActor :type "TextRenderActor Object Reference"))
  (bind _textactor (`local.TextActor`))
  (bind _textrender (`TextRenderActor.TextRender` (`local.TextActor`)))
  ;[1 1 1] First, we look for an entry in our map for the index in input
  (bind _output_get (set `local.TextActor` (`BlueprintMapLibrary.Map_Find` (`self.SpawnedTexts`) Index)))
  (`/Engine/EditorBlueprintResources/StandardMacros.IsValid` _output_get ; Since we don't wanna spawn a second Text actor for the same index, we check if it's valid
    (:`Is Valid`
      ;[1 1 1] It's valid, we just return it
      (return (`local.TextActor`)))
    (:`Is Not Valid`
      ;[1 1 1] Not valid, we spawn a new TextActor
      (bind _returnvalue (`|SpawnActorFromClass` "/Script/Engine.TextRenderActor" (`KismetMathLibrary.MakeTransform` (0.0 0.0 0.0)) "AlwaysSpawn" "MultiplyWithRoot" null null))
      (set `local.TextActor` _returnvalue)
      ;[1 1 1] add it to the map
      (`BlueprintMapLibrary.Map_Add` (`self.SpawnedTexts`) (`local.Index`) (`local.TextActor`))
      (`self.SetActorTickEnabled` _textactor false) ; Disabling the tick
      (`self.SetActorEnableCollision` _textactor false) ; Disabling the collision
      ;[1 1 1] Center the text both horizontally and vertically
      (`TextRenderComponent.SetHorizontalAlignment` _textrender "EHTA_Center")
      (`TextRenderComponent.SetVerticalAlignment` _textrender "EVRTA_TextCenter")
      ;[1 1 1] and return it
      (return (`local.TextActor`)))))

(fn `SetShowTileState`
  (params (ShowDiscoveredTiles :type Boolean) (ShowAnalysedTiles :type Boolean))
  (set `self.ShowDiscoveredTiles` ShowDiscoveredTiles)
  (set `self.ShowAnalysedTiles` ShowAnalysedTiles)
  (`self.UpdateStateOnAllTiles`))

(fn `SetShowTileTexts`
  (params (ShowTileIndices :type Boolean) (ShowCostToEnterTile :type Boolean) (ShowMinCostToTarget :type Boolean) (ShowCostFromStart :type Boolean) (ShowSortOrder :type Boolean) (ShowTileType :type Boolean))
  ;[1 1 1] We check what info the user wants on the Tile, there are 5 possible checkboxes
  (set `self.ShowTileIndices` ShowTileIndices)
  (set `self.ShowCostToEnterTile` ShowCostToEnterTile)
  (set `self.ShowMinCostToTarget` ShowMinCostToTarget)
  (set `self.ShowCostFromStart` ShowCostFromStart)
  (set `self.ShowSortOrder` ShowSortOrder)
  (set `self.ShowTileType` ShowTileType)
  (`self.UpdateTextOnAllTiles`) ; Updates Text Actor based on checkboxes
)

(fn `UpdateStateOnAllTiles`
  (bind _grid (`self.Grid`))
  ;[1 1 1] Is there at least one state to show?
  (if (or (`self.ShowDiscoveredTiles`) (`self.ShowAnalysedTiles`))
    ;[1 1 1] Update the State for every Tile o the Grid
    (bind _keys (`BlueprintMapLibrary.Map_Keys` (`/Game/TacticGame/Blueprints/Core/Grid/BP_Grid.GridTiles` (`self.Grid`))))
    (for _array_element _keys
      (`self.UpdateStateOnTile` _array_element))
    (else
      ;[1 1 1] Clear every Discovered or Analaysed
      (`/Game/TacticGame/Blueprints/Core/Grid/BP_Grid.ClearStateFromTiles` _grid "NewEnumerator5")
      (`/Game/TacticGame/Blueprints/Core/Grid/BP_Grid.ClearStateFromTiles` _grid "NewEnumerator6"))))

(fn `UpdateStateOnTile`
  (params (Index :type "IntPoint Structure"))
  (`|ExecutionSequence`
    (:`then_0`
      (if (`self.ShowDiscoveredTiles`)
        (if (`KismetArrayLibrary.Array_Contains` (`/Game/TacticGame/Blueprints/Core/Grid/BP_GridPathfinding.DiscoveredTileIndices` (`/Game/TacticGame/Blueprints/Core/Grid/BP_Grid.GridPathfinding` (`self.Grid`))) (`local.Index`))
          ;[1 1 1] Update Discovered status
          (`/Game/TacticGame/Blueprints/Core/Grid/BP_Grid.AddStateToTile` (`self.Grid`) (`local.Index`) "NewEnumerator5")
          (else
            (`/Game/TacticGame/Blueprints/Core/Grid/BP_Grid.RemoveStateFromTile` (`self.Grid`) (`local.Index`) "NewEnumerator5" :!label _label)))
        (else
          (goto _label))))
    (:`then_1`
      (if (`self.ShowAnalysedTiles`)
        (if (`KismetArrayLibrary.Array_Contains` (`/Game/TacticGame/Blueprints/Core/Grid/BP_GridPathfinding.AnalysedTileIndices` (`/Game/TacticGame/Blueprints/Core/Grid/BP_Grid.GridPathfinding` (`self.Grid`))) (`local.Index`))
          ;[1 1 1] Update Analysed status
          (`/Game/TacticGame/Blueprints/Core/Grid/BP_Grid.AddStateToTile` (`self.Grid`) (`local.Index`) "NewEnumerator6")
          (else
            (`/Game/TacticGame/Blueprints/Core/Grid/BP_Grid.RemoveStateFromTile` (`self.Grid`) (`local.Index`) "NewEnumerator6" :!label _label_2)))
        (else
          (goto _label_2))))))

(fn `UpdateTextOnAllTiles`
  ;[1 1 1] If anything needs to be displayed
  (if (`self.WantToDisplayAnyText`)
    (bind _keys (`BlueprintMapLibrary.Map_Keys` (`/Game/TacticGame/Blueprints/Core/Grid/BP_Grid.GridTiles` (`self.Grid`))))
    (for _array_element _keys
      (`self.UpdateTextOnTile` _array_element))
    (else
      (`self.ClearAllTextActors`) ; Nothing to display, clear all the TextActors
    )))

(fn `UpdateTextOnTile`
  (params (Index :type "IntPoint Structure"))
  (locals (TileData :type "/Game/TacticGame/Blueprints/Core/Grid/Utilities/S_TileData Structure") (TextActor :type "TextRenderActor Object Reference") (Text :type "Array of String") (TextLengths :type "Array of Integer") (PathfindingData :type "/Game/TacticGame/Blueprints/Core/Grid/Utilities/S_PathfindingData Structure"))
  (bind (_tiledata_index _tiledata_type _tiledata_transform) (break `/Game/TacticGame/Blueprints/Core/Grid/Utilities/S_TileData` (`local.TileData`)))
  (bind (_tiledata_index_2 _tiledata_type_2) (break `/Game/TacticGame/Blueprints/Core/Grid/Utilities/S_TileData` (`local.TileData`)))
  (bind (_index_x _index_y) (break `IntPoint` (`local.Index`)))
  (bind (_tiledata_index_3 _tiledata_type_3) (break `/Game/TacticGame/Blueprints/Core/Grid/Utilities/S_TileData` (`local.TileData`)))
  (bind (_index _costtoentertile _costfromstart _minimumcosttotarget) (break `/Game/TacticGame/Blueprints/Core/Grid/Utilities/S_PathfindingData` (`local.PathfindingData`)))
  (bind (_index_2 _costtoentertile_2 _costfromstart_2) (break `/Game/TacticGame/Blueprints/Core/Grid/Utilities/S_PathfindingData` (`local.PathfindingData`)))
  (bind _returnvalue (`|GetEnumeratorNameAsString` _tiledata_type_3))
  (bind _gridpathfinding (`/Game/TacticGame/Blueprints/Core/Grid/BP_Grid.GridPathfinding` (`self.Grid`)))
  (bind (_gridtilesize_x _gridtilesize_y) (`KismetMathLibrary.BreakVector` (`/Game/TacticGame/Blueprints/Core/Grid/BP_Grid.GridTileSize` (`self.Grid`))))
  (bind (_value _returnvalue_2) (`BlueprintMapLibrary.Map_Find` (`/Game/TacticGame/Blueprints/Core/Grid/BP_Grid.GridTiles` (`self.Grid`)) (`local.Index`)))
  (bind _returnvalue_3 (`KismetStringLibrary.Concat_StrStr` (`KismetStringLibrary.Conv_IntToString` _index_x) "," (`KismetStringLibrary.Conv_IntToString` _index_y)))
  (bind _returnvalue_4 (`KismetArrayLibrary.Array_Find` (`/Game/TacticGame/Blueprints/Core/Grid/BP_GridPathfinding.DiscoveredTileIndices` _gridpathfinding) (`local.Index`)))
  (bind (_value_2 _returnvalue_5) (`BlueprintMapLibrary.Map_Find` (`/Game/TacticGame/Blueprints/Core/Grid/BP_GridPathfinding.PathfindingData` (`/Game/TacticGame/Blueprints/Core/Grid/BP_Grid.GridPathfinding` (`self.Grid`))) (`local.Index`)))
  (bind _returnvalue_6 (`KismetStringLibrary.Concat_StrStr` "Enter: " (`KismetStringLibrary.Conv_IntToString` (`.CostToEnterTile_13_49557D694BA3B92363FA079C4E692538` (break `/Game/TacticGame/Blueprints/Core/Grid/Utilities/S_PathfindingData` (`local.PathfindingData`))))))
  (bind _returnvalue_7 (`KismetStringLibrary.Concat_StrStr` "Min: " (`KismetStringLibrary.Conv_IntToString` _minimumcosttotarget)))
  (bind _returnvalue_8 (`KismetStringLibrary.Concat_StrStr` "Start: " (`KismetStringLibrary.Conv_IntToString` _costfromstart_2)))
  (bind _returnvalue_9 (`KismetStringLibrary.Concat_StrStr` "Sort: " (`KismetStringLibrary.Conv_IntToString` _returnvalue_4) "(" (`KismetStringLibrary.Conv_IntToString` (`|GetArrayItem` (`/Game/TacticGame/Blueprints/Core/Grid/BP_GridPathfinding.DiscoveredTileSortingCosts` _gridpathfinding) _returnvalue_4)) ")"))
  (if (`self.WantToDisplayAnyText`)
    (if _returnvalue_2
      ;[1 1 1] ... and put it in a local var
      (set `local.TileData` _value)
      ;[1 1 1] We check if the tile is walkable (no text on unwalkable ones)
      (if (`/Game/TacticGame/Blueprints/Core/Grid/Utilities/BFL_TileData.IsTileTypeWalkable` _tiledata_type_2)
        (`|ExecutionSequence`
          (:`then_0`
            (`|ExecutionSequence`
              (:`then_0`
                (if (`self.ShowTileIndices`)
                  ;[1 1 1] Add the Indices to the Text Array
                  (`KismetArrayLibrary.Array_Add` (`local.Text`) _returnvalue_3)
                  ;[1 1 1] For every text in the Array, we have a twin array containing the length of these
                  (`KismetArrayLibrary.Array_Add` (`local.TextLengths`) (`KismetStringLibrary.Len` _returnvalue_3))))
              (:`then_1`
                (if (`self.ShowTileType`)
                  ;[1 1 1] Add the Tile Type to the Text Array
                  (if (`|EnumInequality` _tiledata_type_3 "NewEnumerator1")
                    (`KismetArrayLibrary.Array_Add` (`local.Text`) _returnvalue)
                    ;[1 1 1] For every text in the Array, we have a twin array containing the length of these
                    (`KismetArrayLibrary.Array_Add` (`local.TextLengths`) (`KismetStringLibrary.Len` _returnvalue)))))
              (:`then_2`
                (if (or (`self.ShowCostToEnterTile`) (`self.ShowMinCostToTarget`) (`self.ShowCostFromStart`) (`self.ShowSortOrder`))
                  ;[1 1 1] Retrieve the pathfinding data to show
                  (if _returnvalue_5
                    (set `local.PathfindingData` _value_2)
                    (`|ExecutionSequence`
                      (:`then_0`
                        ;[1 1 1] Cost to enter tile
                        (if (`self.ShowCostToEnterTile`)
                          (`KismetArrayLibrary.Array_Add` (`local.Text`) _returnvalue_6)
                          ;[1 1 1] For every text in the Array, we have a twin array containing the length of these
                          (`KismetArrayLibrary.Array_Add` (`local.TextLengths`) (`KismetStringLibrary.Len` _returnvalue_6))))
                      (:`then_1`
                        ;[1 1 1] Min cost to target
                        (if (`self.ShowMinCostToTarget`)
                          (if (!= _minimumcosttotarget 999999)
                            (`KismetArrayLibrary.Array_Add` (`local.Text`) _returnvalue_7)
                            (`KismetArrayLibrary.Array_Add` (`local.TextLengths`) (`KismetStringLibrary.Len` _returnvalue_7)))))
                      (:`then_2`
                        ;[1 1 1] Cost from start
                        (if (`self.ShowCostFromStart`)
                          (if (!= _costfromstart_2 999999)
                            (`KismetArrayLibrary.Array_Add` (`local.Text`) _returnvalue_8)
                            (`KismetArrayLibrary.Array_Add` (`local.TextLengths`) (`KismetStringLibrary.Len` _returnvalue_8)))))
                      (:`then_3`
                        ;[1 1 1] Sort Order
                        (if (`self.ShowSortOrder`)
                          (if (!= _returnvalue_4 -1)
                            (`KismetArrayLibrary.Array_Add` (`local.Text`) _returnvalue_9)
                            (`KismetArrayLibrary.Array_Add` (`local.TextLengths`) (`KismetStringLibrary.Len` _returnvalue_9)))))))))))
          (:`then_1`
            ;[1 1 1] Before doing anything we check if there is some text in the array to display
            (if (> (`KismetArrayLibrary.Array_Length` (`local.Text`)) 0)
              ;[1 1 1] We get the text actor corresponding to that index
              (bind _textrenderedactor (`self.GetTextActor` (`local.Index`)))
              (set `local.TextActor` _textrenderedactor)
              ;[1 1 1] we combine the texts in the array and set the combined string on the TextActor
              (`TextRenderComponent.K2_SetText` (`TextRenderActor.TextRender` (`local.TextActor`)) (`KismetTextLibrary.Conv_StringToText` (`KismetStringLibrary.JoinStringArray` (`local.Text`) " \n")))
              ;[1 1 1] And finally we move the TextActor to the corresponding Tile location
              ; and position, scale and orient it properly
              (`self.K2_SetActorTransform` (`local.TextActor`) (`KismetMathLibrary.MakeTransform` (+ (.location _tiledata_transform) (0.0 0.0 1.0)) (struct :`Pitch` 90.0 :`Yaw` 180.0) (`KismetMathLibrary.Conv_DoubleToVector` (/ _gridtilesize_y (* (`.MaxValue` (`KismetMathLibrary.MaxOfIntArray` (`local.TextLengths`))) 15.0)))) false false)
              (else
                ;[1 1 1] Nothing to show, destroy the Text Actor
                (`self.DestroyTextActor` (`local.Index`))))))
        (else
          ;[1 1 1] If the tile does not exist or it's not walkable,
          ; we destroy the TextActor cos we don't want it there
          (`self.DestroyTextActor` (`local.Index`) :!label _label)))
      (else
        (goto _label)))))

(fn `UserConstructionScript`)

(fn `WantToDisplayAnyText`
  (returns (SomethingToDisplay :type Boolean))
  ;[1 1 1] If any of the 5 checkboxes is ticked, then we show something
  (return (or (`self.ShowTileIndices`) (`self.ShowCostToEnterTile`) (`self.ShowMinCostToTarget`) (`self.ShowCostFromStart`) (`self.ShowSortOrder`) (`self.ShowTileType`))))