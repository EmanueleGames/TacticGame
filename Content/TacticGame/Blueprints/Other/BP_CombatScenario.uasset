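; BP_CombatScenario is a level-placed actor that quick-starts a predefined combat on BeginPlay and returns to the main menu when that combat ends.
; Its construction script pre-spawns the grid in the editor, centred on the actor, and maps units to tiles by location.
; Separate helpers derive teams from team numbers in placed units' display names and assign every team after the first to AI.
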(event `self.ReceiveBeginPlay`
  (add `/Game/TacticGame/Blueprints/Core/Combat/BP_CombatSystem.OnCombatEnded` (`self.CombatSystem`) (delegate `OnCombatEnded`)) ; We need to know when combat is over
  (`/Game/TacticGame/Blueprints/Core/Combat/BP_CombatSystem.QuickStartCombat` (`self.CombatSystem`) (`self.GridData`) (`self.UnitsData`) self))

(event `OnCombatEnded`
  ;[1 1 1] We check if the Combat that just ended was started from a CombatScenario
  ; (and not from a Combat Debug Menu)
  (if (== (`/Game/TacticGame/Blueprints/Core/Combat/BP_CombatSystem.ObjectThatStartedCombat` (`self.CombatSystem`)) self)
    (`GameplayStatics.OpenLevel` "L_MainMenu")))

(fn `BuildAiListBasedOnTeamIndexes`
  (locals (AiUnits :type "Array of /Game/TacticGame/Blueprints/Core/Units/BP_Unit Object Reference"))
  (for (_array_element _array_index) (`.UnitTeams_12_9D9EF9D941EDB98BDC7BDE9F390F2C33` (break `/Game/TacticGame/Blueprints/Core/Combat/Utilities/S_QuickCombat_UnitTeams` (`self.UnitsData`)))
    ;[1 1 1] If the Team is not the first one, then assign AI to it
    (if (!= _array_index 0)
      (`KismetArrayLibrary.Array_Append` (`local.AiUnits`) (`.UnitArray_5_BEF553954C5D7EB6C9912FB3D4D40761` (break `/Game/TacticGame/Blueprints/Core/Combat/Utilities/S_UnitArray` _array_element)))))
  (setmembers `/Game/TacticGame/Blueprints/Core/Combat/Utilities/S_QuickCombat_UnitTeams` :`StructRef` (`self.UnitsData`) :`UnitsControlledByAi` (`local.AiUnits`)) ; Return all the AI Teams
)

(fn `BuildDesiredGridIndexesBasedOnUnitLocations`
  (locals (DesiredIndexes :type "Map of /Game/TacticGame/Blueprints/Core/Units/BP_Unit Object Reference to IntPoint Structure"))
  (for _array_element (`.UnitTeams_12_9D9EF9D941EDB98BDC7BDE9F390F2C33` (break `/Game/TacticGame/Blueprints/Core/Combat/Utilities/S_QuickCombat_UnitTeams` (`self.UnitsData`)))
    (for _array_element_2 (`.UnitArray_5_BEF553954C5D7EB6C9912FB3D4D40761` (break `/Game/TacticGame/Blueprints/Core/Combat/Utilities/S_UnitArray` _array_element))
      ;[1 1 1 1 16] Get the closest Index to snap the Unit to inside the Grid bounds
      (bind _index (`/Game/TacticGame/Blueprints/Core/Grid/BP_Grid.GetTileIndexFromWorldLocation` (`/Game/TacticGame/Blueprints/Core/Combat/BP_CombatSystem.Grid` (`self.CombatSystem`)) (`self.K2_GetActorLocation` _array_element_2)))
      ;[1 1 1 1 16] Add the Index info in the return Structure
      (`BlueprintMapLibrary.Map_Add` (`local.DesiredIndexes`) _array_element_2 _index)))
  (setmembers `/Game/TacticGame/Blueprints/Core/Combat/Utilities/S_QuickCombat_UnitTeams` :`StructRef` (`self.UnitsData`) :`UnitDesiredIndexes` (`local.DesiredIndexes`)) ; Return all the found Grid Indexes
)

(fn `BuildTeamsBasedOnUnitNames`
  (locals (Unit :type "/Game/TacticGame/Blueprints/Core/Units/BP_Unit Object Reference") (TeamIndex :type Integer) (UnitsTeams :type "Array of /Game/TacticGame/Blueprints/Core/Combat/Utilities/S_UnitArray Structure"))
  ;[1 1 1] Get all the Unit Actors placed in the scene and loop them
  (bind _outactors (`GameplayStatics.GetAllActorsOfClass` "/Game/TacticGame/Blueprints/Core/Units/BP_Unit.BP_Unit_C"))
  (for _array_element _outactors
    (set `local.Unit` _array_element)
    ;[1 1 1] Get the Unit's Team included in the Unit display name
    (set `local.TeamIndex` (`KismetStringLibrary.Conv_StringToInt` (`KismetStringLibrary.Split` (`.RightS` (`KismetStringLibrary.Split` (`KismetSystemLibrary.GetDisplayName` (`local.Unit`)) "Team")) "_")))
    ;[1 1 1] Do we have enough Teams in the UnitsTeams Array?
    ; (NB. UnitsTeams is an array of array, one array for each Team)
    (if (< (`KismetArrayLibrary.Array_Length` (`local.UnitsTeams`)) (+ (`local.TeamIndex`) 1))
      ;[1 1 1] Not enough Teams - The Array must be resized
      (`KismetArrayLibrary.Array_Resize` (`local.UnitsTeams`) (+ (`local.TeamIndex`) 1)))
    (`KismetArrayLibrary.Array_Add` (`.UnitArray_5_BEF553954C5D7EB6C9912FB3D4D40761` (break `/Game/TacticGame/Blueprints/Core/Combat/Utilities/S_UnitArray` (`|GetArrayItem` (`local.UnitsTeams`) (`local.TeamIndex`)))) (`local.Unit`)))
  (`KismetArrayLibrary.Array_RemoveItem` (`local.UnitsTeams`)) ; Removes empty groups
  ;[1 1 1] Update the final Structure with the non-empty Teams
  (setmembers `/Game/TacticGame/Blueprints/Core/Combat/Utilities/S_QuickCombat_UnitTeams` :`StructRef` (`self.UnitsData`) :`UnitTeams` (`local.UnitsTeams`)))

(fn `SpawnGrid`
  (bind _combatsystem (`self.CombatSystem`))
  (bind (_generategridbeforestartingcombat _centerlocation _tilesize _tilecount _shape _useenvironment) (break `/Game/TacticGame/Blueprints/Core/Combat/Utilities/S_QuickCombat_Grid` (`self.GridData`)))
  (bind _grid (`/Game/TacticGame/Blueprints/Core/Combat/BP_CombatSystem.Grid` _combatsystem))
  (`/Engine/EditorBlueprintResources/StandardMacros.IsValid` _combatsystem
    (:`Is Valid`
      (`/Engine/EditorBlueprintResources/StandardMacros.IsValid` _grid
        (:`Is Valid`
          (`/Game/TacticGame/Blueprints/Core/Grid/BP_Grid.SpawnGrid` _grid _centerlocation _tilesize _tilecount _shape _useenvironment))))))

(fn `UserConstructionScript`
  ;[1 1 1 1 16] We only generate the Grid in the Editor
  ; (in Game the Grid is already there from the Editor)
  (if (not (`/Game/TacticGame/Blueprints/Core/Utilities/BFL_Utilities.IsInGame`))
    (setmembers `/Game/TacticGame/Blueprints/Core/Combat/Utilities/S_QuickCombat_Grid` :`StructRef` (`self.GridData`) :`CenterLocation` (`self.K2_GetActorLocation`))
    (`self.SpawnGrid`)
    (`self.BuildDesiredGridIndexesBasedOnUnitLocations`)))