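; Main menu controller that shows the W_MainMenu widget over a streamed-in L_Square level used as a backdrop.
; On BeginPlay it adds the widget, loads the level, triggers the background reveal, then slows BP_Pawn's rotation interpolation and re-triggers its menu camera rotation on a long delay loop.
; An unconnected chain for cycling square, hexagon and triangle backdrop levels with show/hide transitions never runs.
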(event `self.ReceiveBeginPlay`
  (bind _pawn (`self.Pawn`))
  (bind _returnvalue (`|CreateWidget` "/Game/Blueprints/Other/MainMenu/W_MainMenu.W_MainMenu_C"))
  (bind _output_get (set `self.W_MainMenu` _returnvalue))
  (`UserWidget.AddToViewport` _output_get 0)
  ;[1 1 1] By Finn - Camera rotation
  (bind _returnvalue_2 (`GameplayStatics.GetActorOfClass` "/Game/Blueprints/Core/Player/BP_Pawn.BP_Pawn_C"))
  (set `self.Pawn` _returnvalue_2)
  (`GameplayStatics.LoadStreamLevel` "L_Square" true)
  (`/Game/Blueprints/Other/MainMenu/W_MainMenu.Event_ShowBackground` (`self.W_MainMenu`))
  ;[1 1 1] By Finn - Camera rotation
  (`KismetSystemLibrary.Delay` 1.0)
  (set `/Game/Blueprints/Core/Player/BP_Pawn.RotationInterpSpeed` 0.02 _pawn)
  (`/Game/Blueprints/Core/Player/BP_Pawn.Event_MainMenuRotation` _pawn :!label _label)
  (`KismetSystemLibrary.Delay` 200.0)
  (goto _label))

(fn `UserConstructionScript`)