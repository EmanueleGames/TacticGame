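; BP_PlayerActions handles mouse interaction with the BP_Grid, tracking hovered and selected tiles and units.
; Tick updates hover from cursor traces, with a hovered unit overriding the tile under the cursor.
; Left and right clicks execute swappable action actors spawned by SetSelectedAction, repeating on each newly hovered tile while held.
; Grid regeneration and selected-tile updates force a reselect to keep tile and unit selection in sync.
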(event `self.ReceiveBeginPlay`
  (bind _grid (`self.Grid`))
  ;[1 1 1] As soon as the game begins,
  ; we get the first actor of class BP_Grid that we find
  ; and use it as reference parameter for the player actions
  (bind _returnvalue (`GameplayStatics.GetActorOfClass` "/Game/Blueprints/Core/Grid/BP_Grid.BP_Grid_C"))
  (set `self.Grid` _returnvalue)
  ;[1 1 1 1 16] We bind on the Grid Generated and Tile Updated dispatchers to update the Grid if it gets regenerated with particular conditions
  ; Es.with a Unit selected (we need to keep also the Tile selecation in this case), etc.
  (add `/Game/Blueprints/Core/Grid/BP_Grid.OnGridGenerated` _grid (`|CreateDelegate` :!event `OnGridGenerated`))
  (add `/Game/Blueprints/Core/Grid/BP_Grid.OnTileDataUpdated` _grid (`|CreateDelegate` :!event `OnTileDataUpdated`))
  ;[1 1 1] As soon as the game begins,
  ; we get the first actor of class BP_CombatSystem that we find
  ; and use it as reference parameter for the combat system
  (bind _returnvalue_2 (`GameplayStatics.GetActorOfClass` "/Game/Blueprints/Core/Combat/BP_CombatSystem.BP_CombatSystem_C"))
  (set `self.CombatSystem` _returnvalue_2)
  ;[1 1 1] To enable mouse click for the Player Controller
  (`self.EnableInput` (`GameplayStatics.GetPlayerController` 0)))

(event `self.ReceiveTick`
  (params (DeltaSeconds :type "Float (single-precision)"))
  (`self.UpdateHoveredTileAndUnit`))

(event `Key|LeftMouseButton`
  (params (Key :type "Key Structure"))
  ;[1 1 1] Mouse left click to perform action on a tile
  (:`Pressed`
    (`self.UpdateHoveredTileAndUnit`) ; to force the update if player clicks too fast
    (set `self.IsLeftClickDown` true)
    (`/Engine/EditorBlueprintResources/StandardMacros.IsValid` (`self.SelectedAction_LeftClick`) :!label _label ; Check if we have a selected action for the left click
      (:`Is Valid`
        (`/Game/Blueprints/Core/Player/Actions/BP_Action.ExecuteAction` (`self.SelectedAction_LeftClick`) (`self.HoveredTile`)))))
  (:`Released`
    (set `self.IsLeftClickDown` false)))

(event `OnHoveredTileChanged`
  ;[1 1 1] When the mouse cursor moves on a new tile while a button is kept pressed
  (`|ExecutionSequence`
    (:`then_0`
      (if (`self.IsLeftClickDown`)
        (goto _label)))
    (:`then_1`
      (if (`self.IsRightClickDown`)
        ;[1 1 1] Mouse right click to perform action on a tile
        (`/Engine/EditorBlueprintResources/StandardMacros.IsValid` (`self.SelectedAction_RightClick`) :!label _label_2 ; Check if we have a selected action for the right click
          (:`Is Valid`
            (`/Game/Blueprints/Core/Player/Actions/BP_Action.ExecuteAction` (`self.SelectedAction_RightClick`) (`self.HoveredTile`))))))))

(event `Key|RightMouseButton`
  (params (Key :type "Key Structure"))
  ;[1 1 1] Mouse right click to perform action on a tile
  (:`Pressed`
    (`self.UpdateHoveredTileAndUnit`) ; to force the update if player clicks too fast
    (set `self.IsRightClickDown` true)
    (goto _label_2))
  (:`Released`
    (set `self.IsRightClickDown` false)))

(fn `GetUnitUnderCursor`
  (params (PlayerIndex :type Integer))
  (returns (Unit :type "/Game/Blueprints/Core/Units/BP_Unit Object Reference"))
  (bind (_hitresult _returnvalue) (`PlayerController.GetHitResultUnderCursorByChannel` (`GameplayStatics.GetPlayerController` PlayerIndex) "TraceTypeQuery5" false))
  (if _returnvalue
    ;[1 1 1] If the mouse was on a Unit, we return it
    (bind _asbp_unit (cast `/Game/Blueprints/Core/Units/BP_Unit` (`.HitActor` (`GameplayStatics.BreakHitResult` _hitresult))))
    (return _asbp_unit)
    (else
      ;[1 1 1] If instead the cursor was on a tile, we try to return the Unit on that tile (if one exists)
      (bind _index (`/Game/Blueprints/Core/Grid/BP_Grid.GetTileIndexUnderCursor` (`self.Grid`) (`local.PlayerIndex`)))
      (return (`.UnitOnTile_16_1A24A24A4845A31FB93E7BBEC72A5FD3` (break `/Game/Blueprints/Core/Grid/Utilities/S_TileData` (`BlueprintMapLibrary.Map_Find` (`/Game/Blueprints/Core/Grid/BP_Grid.GridTiles` (`self.Grid`)) _index)))) ; If there is no Unit on that Tile, the return Unit will be null
    )))

(fn `OnGridGenerated`
  ;[1 1 1 1 17] After regenerating the grid we check if the player had a Tile selected
  (if (`/Game/Blueprints/Core/Grid/BP_Grid.IsIndexValid` (`self.Grid`) (`self.SelectedTile`))
    (`self.SetSelectedTileAndUnit` (`self.SelectedTile`) true) ; If still valid, we reselct the same Tile
    (else
      (`self.SetSelectedTileAndUnit` (make `IntPoint` -999 -999) true) ; Othrwise we deselect it
    )))

(fn `OnTileDataUpdated`
  (params (Index :type "IntPoint Structure"))
  (if (`KismetMathLibrary.Equal_IntPointIntPoint` Index (`self.SelectedTile`))
    (`self.OnGridGenerated`)))

(fn `SetSelectedAction`
  (params (LeftAction :type "/Game/Blueprints/Core/Player/Actions/BP_Action Class Reference") (RightAction :type "/Game/Blueprints/Core/Player/Actions/BP_Action Class Reference"))
  (bind _selectedaction_leftclick (`self.SelectedAction_LeftClick`))
  (bind _selectedaction_rightclick (`self.SelectedAction_RightClick`))
  (`|ExecutionSequence`
    (:`then_0`
      ;[1 1 1] If there was already an action associated with the left click...
      (`/Engine/EditorBlueprintResources/StandardMacros.IsValid` _selectedaction_leftclick
        (:`Is Valid`
          ;[1 1 1] We destroy it (the old one)
          (`self.K2_DestroyActor` _selectedaction_leftclick)
          ;[1 1 1] And set it to None (no input)
          (set `self.SelectedAction_LeftClick` null))
        (:`Is Not Valid`
          _))
      ;[1 1 1] Resolved the old action (invalid or destroyed)
      ; We check if the new one in input is valid
      (if (`KismetSystemLibrary.IsValidClass` (`local.LeftAction`))
        ;[1 1 1] If valid we are gonna use it to spawn a new actor of this class
        (bind _returnvalue (`|SpawnActorFromClass` (`local.LeftAction`) (`KismetMathLibrary.MakeTransform` (0.0 0.0 0.0)) "AlwaysSpawn" "MultiplyWithRoot" null self null))
        ;[1 1 1] and set the new action
        (set `self.SelectedAction_LeftClick` _returnvalue)))
    (:`then_1`
      ;[1 1 1] If there was already an action associated with the right click...
      (`/Engine/EditorBlueprintResources/StandardMacros.IsValid` _selectedaction_rightclick
        (:`Is Valid`
          ;[1 1 1] We destroy it (the old one)
          (`self.K2_DestroyActor` _selectedaction_rightclick)
          ;[1 1 1] And set it to None (no input)
          (set `self.SelectedAction_RightClick` null))
        (:`Is Not Valid`
          _))
      ;[1 1 1] Resolved the old action (invalid or destroyed)
      ; We check if the new one in input is valid
      (if (`KismetSystemLibrary.IsValidClass` (`local.RightAction`))
        ;[1 1 1] If valid we are gonna use it to spawn a new actor of this class
        (bind _returnvalue_2 (`|SpawnActorFromClass` (`local.RightAction`) (`KismetMathLibrary.MakeTransform` (0.0 0.0 0.0)) "AlwaysSpawn" "MultiplyWithRoot" null self null))
        ;[1 1 1] and set the new action
        (set `self.SelectedAction_RightClick` _returnvalue_2)))
    (:`then_2`
      ;[1 1 1] Signal all the blueprints bound to the dispatcher
      (`self.OnSelectedActionsChanged` (`self.SelectedAction_LeftClick`) (`self.SelectedAction_RightClick`)))))

(fn `SetSelectedTileAndUnit`
  (params (Index :type "IntPoint Structure") (Force :type Boolean))
  (locals (NewUnit :type "/Game/Blueprints/Core/Units/BP_Unit Object Reference"))
  (bind _selectedunit (`self.SelectedUnit`))
  (`|ExecutionSequence`
    (:`then_0`
      ;[1 1 1] First thing first, we compare the index in input with the one from the selected tile, to check if they are different
      (if (or (!= (`self.SelectedTile`) (`local.Index`)) (`local.Force`))
        ;[1 1 1] If they are the different, we remove the Selected state on Previous Tile...
        (`/Game/Blueprints/Core/Grid/BP_Grid.RemoveStateFromTile` (`self.Grid`) (`self.SelectedTile`) "NewEnumerator2")
        ;[1 1 1] ...then update the selected Tile
        (set `self.SelectedTile` (`local.Index`))
        ;[1 1 1] ...and finally update the State for that Tile
        (`/Game/Blueprints/Core/Grid/BP_Grid.AddStateToTile` (`self.Grid`) (`self.SelectedTile`) "NewEnumerator2")
        (else
          ;[1 1 1] If they are the same, we wanna simply deselect the Tile.
          ; So we remove the Selected state on the Tile...
          (`/Game/Blueprints/Core/Grid/BP_Grid.RemoveStateFromTile` (`self.Grid`) (`self.SelectedTile`) "NewEnumerator2")
          ;[1 1 1] ...then update the selected Tile
          ; with an invalid one (-999,-999)
          (set `self.SelectedTile` (make `IntPoint` -999 -999)))))
    (:`then_1`
      ;[1 1 1] We get the Unit on the selected Tile of the grid and put it into a local variable
      (set `local.NewUnit` (`.UnitOnTile_16_1A24A24A4845A31FB93E7BBEC72A5FD3` (break `/Game/Blueprints/Core/Grid/Utilities/S_TileData` (`BlueprintMapLibrary.Map_Find` (`/Game/Blueprints/Core/Grid/BP_Grid.GridTiles` (`self.Grid`)) (`self.SelectedTile`)))))
      ;[1 1 1] As done for the Tile, we compare the Unit on the selected Tile with the old selected Unit, to check if they are different
      (if (or (!= (`self.SelectedUnit`) (`local.NewUnit`)) (`local.Force`))
        (`|ExecutionSequence`
          (:`then_0`
            ;[1 1 1] Old Unit deselection
            (`/Engine/EditorBlueprintResources/StandardMacros.IsValid` _selectedunit
              (:`Is Valid`
                (`/Game/Blueprints/Core/Units/BP_Unit.SetIsSelected` _selectedunit false))))
          (:`then_1`
            ;[1 1 1] New Unit selection
            (bind _output_get (set `self.SelectedUnit` (`local.NewUnit`)))
            (`/Engine/EditorBlueprintResources/StandardMacros.IsValid` _output_get
              (:`Is Valid`
                (`/Game/Blueprints/Core/Units/BP_Unit.SetIsSelected` _output_get true)))))))))

(fn `UpdateHoveredTileAndUnit`
  (locals (NewIndex :type "IntPoint Structure"))
  (bind _hoveredunit (`self.HoveredUnit`))
  (bind _hoveredunit_2 (`self.HoveredUnit`))
  (`|ExecutionSequence`
    (:`then_0`
      ;[1 1 1] Check that we are hovering a different unit and not always the same one
      (bind _unit (`self.GetUnitUnderCursor` 0))
      (if (!= _unit (`self.HoveredUnit`))
        (`|ExecutionSequence`
          (:`then_0`
            ;[1 1 1] Unhovering the old unit
            (`/Engine/EditorBlueprintResources/StandardMacros.IsValid` _hoveredunit_2
              (:`Is Valid`
                (`/Game/Blueprints/Core/Units/BP_Unit.SetIsHovered` _hoveredunit_2 false))))
          (:`then_1`
            ;[1 1 1] Hovering the new one
            (bind _output_get (set `self.HoveredUnit` _unit))
            (`/Engine/EditorBlueprintResources/StandardMacros.IsValid` _output_get
              (:`Is Valid`
                (`/Game/Blueprints/Core/Units/BP_Unit.SetIsHovered` _output_get true)))))))
    (:`then_1`
      ;[1 1 1] If a Unit is hovered, we ignore the eventual Tile hovered and always select the index of the Tile under the Unit hovered
      (`/Engine/EditorBlueprintResources/StandardMacros.IsValid` _hoveredunit
        (:`Is Valid`
          (set `local.NewIndex` (`/Game/Blueprints/Core/Units/BP_Unit.Index` _hoveredunit)))
        (:`Is Not Valid`
          ;[1 1 1] If no Unit is hovered, than we use the hovered Tile index
          (bind _index (`/Game/Blueprints/Core/Grid/BP_Grid.GetTileIndexUnderCursor` (`self.Grid`) 0))
          (set `local.NewIndex` _index)))
      ;[1 1 1] Performance Optimization
      ; we update the hovered tile only if its a different one from the previous hovered one
      (if (!= (`local.NewIndex`) (`self.HoveredTile`))
        ;[1 1 1] Remove the hovered state from the old tile
        (`/Game/Blueprints/Core/Grid/BP_Grid.RemoveStateFromTile` (`self.Grid`) (`self.HoveredTile`) "NewEnumerator1")
        ;[1 1 1] Update the hovered state to the new tile
        (bind _output_get_2 (set `self.HoveredTile` (`local.NewIndex`)))
        (`/Game/Blueprints/Core/Grid/BP_Grid.AddStateToTile` (`self.Grid`) _output_get_2 "NewEnumerator1")
        ;[1 1 1] Signal the Event listening for the hovered tile changed
        (`self.OnHoveredTileChanged`)))))

(fn `UserConstructionScript`)