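; Player camera pawn with smoothed panning, stepped rotation and spring arm zoom.
; Axis inputs shift a target location along the actor's forward and right vectors and adjust a clamped target arm length.
; Left and right rotation actions turn a target rotation in 45-degree steps.
; Tick interpolates actor location, rotation and arm length toward those targets, which BeginPlay seeds from the starting state.
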(event `self.ReceiveBeginPlay`
  (set `self.LocationPos` (`self.K2_GetActorLocation`))
  (set `self.ZoomValue` (`SpringArmComponent.TargetArmLength` (`self.SpringArm`)))
  (set `self.RotationView` (`self.K2_GetActorRotation`)))

(event `self.ReceiveTick`
  (params (DeltaSeconds :type "Float (single-precision)"))
  (bind _springarm (`self.SpringArm`))
  (set `SpringArmComponent.TargetArmLength` (`KismetMathLibrary.FInterpTo` (`SpringArmComponent.TargetArmLength` _springarm) (`self.ZoomValue`) DeltaSeconds 2.0) _springarm)
  (`self.K2_SetActorLocation` (`KismetMathLibrary.VInterpTo` (`self.K2_GetActorLocation`) (`self.LocationPos`) DeltaSeconds 5.0))
  (`self.K2_SetActorRotation` (`KismetMathLibrary.RInterpTo` (`self.K2_GetActorRotation`) (`self.RotationView`) DeltaSeconds 5.0)))

(event `InputAxis|InputAxis_Zoom`
  (params (AxisValue :type "Float (single-precision)"))
  (set `self.ZoomValue` (`KismetMathLibrary.FClamp` (+ (`self.ZoomValue`) (* AxisValue 50.0)) 200.0 2500.0)))

(event `InputAxis|InputAxis_Forward`
  (params (AxisValue :type "Float (single-precision)"))
  (set `self.LocationPos` (+ (`self.LocationPos`) (* (* AxisValue 20.0) (`self.GetActorForwardVector`)))))

(event `InputAxis|InputAxis_Right`
  (params (AxisValue :type "Float (single-precision)"))
  (set `self.LocationPos` (+ (`self.LocationPos`) (* (* AxisValue 20.0) (`self.GetActorRightVector`)))))

(event `InputAction|InputAction_RotationRight`
  (params (Key :type "Key Structure"))
  (:`Pressed`
    (set `self.RotationView` (`KismetMathLibrary.ComposeRotators` (`self.RotationView`) (struct :`Yaw` 45.0)))))

(event `InputAction|InputAction_RotationLeft`
  (params (Key :type "Key Structure"))
  (:`Pressed`
    (set `self.RotationView` (`KismetMathLibrary.ComposeRotators` (`self.RotationView`) (struct :`Yaw` -45.0)))))

(fn `UserConstructionScript`)