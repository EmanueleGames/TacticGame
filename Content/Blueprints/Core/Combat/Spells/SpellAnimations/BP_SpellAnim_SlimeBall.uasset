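; Spell animation actor for the Slime Ball combat spell, lobbing a three-mesh green slime ball from the origin tile to the target tile.
; A timeline drives the position lerp with a height offset, plus mesh opacity and scale.
; Partway through playback it notifies a hit once for every attacked tile index so units can react, then completes the animation when the timeline finishes.
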(event `self.Event_PlaySpellAnimation`
  (bind _transform_location (`KismetMathLibrary.BreakTransform` (`self.GetTileTransform` (`self.OriginIndex`))))
  (bind _transform_location_2 (`KismetMathLibrary.BreakTransform` (`self.GetTileTransform` (`self.TargetIndex`))))
  (bind _transform_location_3 (`KismetMathLibrary.BreakTransform` (`self.GetTileTransform` (`self.OriginIndex`))))
  ;[1 1 1] We position the SlimeBall on the OriginIndex Tile
  (`self.K2_SetActorLocation` _transform_location)
  (bind (_direction _locationalpha _locationz _opacity _scale) (`Timeline|Timeline_SlimeBall` :!via `PlayFromStart`)
    (:`Update`
      ;[1 1 1] We Animate from the OriginTile to the TargetTile
      (`self.K2_SetActorLocation` (+ (`KismetMathLibrary.VLerp` _transform_location_3 _transform_location_2 _locationalpha) (`KismetMathLibrary.MakeVector` 0.0 0.0 _locationz)))
      ;[1 1 1] And we play with the opacity to animate the SlimeBall
      (`MeshComponent.SetScalarParameterValueOnMaterials` (`self.StaticMesh_Ball1`) "Opacity" _opacity)
      (`MeshComponent.SetScalarParameterValueOnMaterials` (`self.StaticMesh_Ball3`) "Opacity" _opacity)
      (`MeshComponent.SetScalarParameterValueOnMaterials` (`self.StaticMesh_Ball2`) "Opacity" _opacity)
      ;[1 1 1] We animate the SlimeBall scaling it
      (`SceneComponent.SetRelativeScale3D` (`self.Anim_Scale`) _scale)
      ;[1 1 1] At the proper time during the timeline (depends on the spell)
      (if (>= (`TimelineComponent.GetPlaybackPosition` (`self.Timeline_SlimeBall`)) 0.55)
        ;[1 1 1] Notify (just once) that we hit the tile (so the Unit can play the Hit animation)
        (`/Engine/EditorBlueprintResources/StandardMacros.DoOnce` false
          (:`Completed`
            (for _array_element (`self.AttackIndexes`)
              (`self.OnSpellAnimationHitTile` self _array_element))))))
    (:`Finished`
      ;[1 1 1] Responsable to destroy the BP when Animation ends
      (`self.Event_CompleteSpellAnimation`))))

(fn `UserConstructionScript`
  (`parent.UserConstructionScript`)
  (`MeshComponent.SetVectorParameterValueOnMaterials` (`self.StaticMesh_Ball1`) "Color" (`KismetMathLibrary.Conv_LinearColorToVector` (struct :`G` 0.291667 :`B` 0.069203 :`A` 1.0)))
  (`MeshComponent.SetVectorParameterValueOnMaterials` (`self.StaticMesh_Ball3`) "Color" (`KismetMathLibrary.Conv_LinearColorToVector` (struct :`R` 0.189605 :`G` 0.958333 :`B` 0.476418 :`A` 1.0)))
  (`MeshComponent.SetVectorParameterValueOnMaterials` (`self.StaticMesh_Ball2`) "Color" (`KismetMathLibrary.Conv_LinearColorToVector` (struct :`G` 0.807292 :`B` 0.169529 :`A` 1.0))))