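; Animated wind gust shape for a spell animation, moved from an origin to a target transform and destroyed shortly after it finishes.
; A timeline at a variable play rate interpolates the actor transform and drives material opacity for fading.
; Partway through, it fires a completion event once so the owning animation is notified before the shape is gone.
; The construction script creates two dynamic translucent materials with randomly brightened green tints.
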(event `self.ReceiveBeginPlay`
  ;[1 1 1] We use PlayRate to give the animation speed
  ; a little bit of variety, so it's less boring
  (`TimelineComponent.SetPlayRate` (`self.Timeline_AnimatedWindGust`) (`self.PlayRate`))
  ;[1 1 1] Spell aniamtion, we're using a timeline to realize a simple interpolation between Origin and Target Tile
  (bind (_direction _transformalpha _opacity) (`Timeline|Timeline_AnimatedWindGust` :!via `PlayFromStart`)
    (:`Update`
      (`self.K2_SetActorTransform` (`KismetMathLibrary.TLerp` (`self.OriginTransform`) (`self.TargetTransform`) _transformalpha))
      ;[1 1 1] And to fade in/out meshes
      (`MeshComponent.SetScalarParameterValueOnMaterials` (`self.AnimatedWindGust`) "Opacity" _opacity)
      (if (>= (`TimelineComponent.GetPlaybackPosition` (`self.Timeline_AnimatedWindGust`)) 0.35)
        (`/Engine/EditorBlueprintResources/StandardMacros.DoOnce` false
          (:`Completed`
            ;[1 1 1 1 16] We need this to destroy the Blueprint responsable to create the animation (witch is different from the object used in the animation destriyed right after the delay)
            (`self.OnShapeAnimationCompleted` self)))))
    (:`Finished`
      ;[1 1 1] After a short delay, we destroy the shape used to animate
      (`KismetSystemLibrary.Delay` 0.5)
      (`self.K2_DestroyActor`))))

(fn `UserConstructionScript`
  ;[1 1 1] For each element of the WindGast we create a Material Instance and then set the Color for it (with a bit of randomness)
  (bind _returnvalue (`PrimitiveComponent.CreateDynamicMaterialInstance` (`self.AnimatedWindGust`) 0 "/Game/Art/Materials/M_TranslucentColor.M_TranslucentColor" "None"))
  (`MaterialInstanceDynamic.SetVectorParameterValue` _returnvalue "Color" (* (struct :`G` 0.703125 :`B` 0.088694 :`A` 1.0) (`KismetMathLibrary.RandomFloatInRange` 0.8 1.5)))
  (bind _returnvalue_2 (`PrimitiveComponent.CreateDynamicMaterialInstance` (`self.AnimatedWindGust`) 1 "/Game/Art/Materials/M_TranslucentColor.M_TranslucentColor" "None"))
  (`MaterialInstanceDynamic.SetVectorParameterValue` _returnvalue_2 "Color" (* (struct :`R` 0.213379 :`G` 0.890625 :`B` 0.43234 :`A` 1.0) (`KismetMathLibrary.RandomFloatInRange` 0.8 1.5))))