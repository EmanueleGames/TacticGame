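; Spell animation actor for a sword throw that flies like a boomerang from the origin tile to the target tile and back.
; On play it faces the target, then a timeline lerps the actor between the tiles while offsetting, spinning and scaling a child component for an arcing path.
; It signals the tile hit once at a set playback time and completes the spell animation when the timeline finishes.
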(event `self.Event_PlaySpellAnimation`
  (bind _transform_location (`KismetMathLibrary.BreakTransform` (`self.GetTileTransform` (`self.OriginIndex`))))
  (bind _transform_location_2 (`KismetMathLibrary.BreakTransform` (`self.GetTileTransform` (`self.TargetIndex`))))
  (bind _transform_location_3 (`KismetMathLibrary.BreakTransform` (`self.GetTileTransform` (`self.OriginIndex`))))
  ;[1 1 1] We position and orient the sword from the OriginIndex to the TargetIndex
  (`self.K2_SetActorLocationAndRotation` _transform_location_3 (`KismetMathLibrary.FindLookAtRotation` (`KismetMathLibrary.Conv_Vector2DToVector` (`KismetMathLibrary.Conv_IntPointToVector2D` (`self.OriginIndex`))) (`KismetMathLibrary.Conv_Vector2DToVector` (`KismetMathLibrary.Conv_IntPointToVector2D` (`self.TargetIndex`)))))
  (bind (_direction _actorlocationalpha _locationy _rotationz _scale) (`Timeline|Timeline_SwordThrow` :!via `PlayFromStart`)
    (:`Update`
      ;[1 1 1] We give the sword a boomerang animation, it reaches the target and then comes back
      (`self.K2_SetActorLocation` (`KismetMathLibrary.VLerp` _transform_location _transform_location_2 _actorlocationalpha))
      ;[1 1 1] We make the animation prettier by adding effect on the Transform
      (`SceneComponent.K2_SetRelativeTransform` (`self.Anim_LocationRotationScale`) (`KismetMathLibrary.MakeTransform` (`KismetMathLibrary.MakeVector` 0.0 _locationy) (`KismetMathLibrary.MakeRotator` 0.0 0.0 _rotationz) (`KismetMathLibrary.Conv_DoubleToVector` _scale)) false false)
      ;[1 1 1] At the proper time during the timeline (depends on the spell)
      (if (>= (`TimelineComponent.GetPlaybackPosition` (`self.Timeline_SwordThrow`)) 0.3)
        ;[1 1 1] Notify (just once) that we hit the tile (so the Unit can play the Hit animation)
        (`/Engine/EditorBlueprintResources/StandardMacros.DoOnce` false
          (:`Completed`
            (`self.OnSpellAnimationHitTile` self (`self.TargetIndex`))))))
    (:`Finished`
      ;[1 1 1] Responsable to destroy the BP when Animation ends
      (`self.Event_CompleteSpellAnimation`))))

(fn `UserConstructionScript`
  (`parent.UserConstructionScript`))