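; Heal spell animation Blueprint that plays a green wave with plus signs on the target tile.
; A timeline scales and rotates the shared pivot and drives material opacity on the meshes, whose shades of green are set in the construction script.
; Shortly into playback it notifies the tile hit once so the unit can react, then completes the spell animation when the timeline finishes.
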(event `self.Event_PlaySpellAnimation`
  (bind _anim_rotationscale (`self.Anim_RotationScale`))
  (bind _transform_location (`KismetMathLibrary.BreakTransform` (`self.GetTileTransform` (`self.TargetIndex`))))
  ;[1 1 1] We position the HealWave on the Target Tile
  (`self.K2_SetActorLocation` _transform_location)
  (bind (_direction _scale _rotation _opacity) (`Timeline|Timeline_Heal` :!via `PlayFromStart`)
    (:`Update`
      ;[1 1 1] We animate the Wave and Plus scaling them
      (`SceneComponent.SetRelativeScale3D` _anim_rotationscale _scale)
      ;[1 1 1] The Rotation won't be visible on the wave,
      ; but on the plus signs
      (`SceneComponent.K2_SetRelativeRotation` _anim_rotationscale (`KismetMathLibrary.MakeRotator` 0.0 0.0 _rotation) false false)
      ;[1 1 1] And we play with the opacity to animate the Wave/Plus
      (`MeshComponent.SetScalarParameterValueOnMaterials` (`self.StaticMesh_Inner`) "Opacity" _opacity)
      (`MeshComponent.SetScalarParameterValueOnMaterials` (`self.StaticMesh_Middle`) "Opacity" _opacity)
      (`MeshComponent.SetScalarParameterValueOnMaterials` (`self.StaticMesh_Outer`) "Opacity" _opacity)
      (`MeshComponent.SetScalarParameterValueOnMaterials` (`self.StaticMesh_Plus1`) "Opacity" _opacity)
      (`MeshComponent.SetScalarParameterValueOnMaterials` (`self.StaticMesh_Plus2`) "Opacity" _opacity)
      (`MeshComponent.SetScalarParameterValueOnMaterials` (`self.StaticMesh_Plus3`) "Opacity" _opacity)
      ;[1 1 1] At the proper time during the timeline (depends on the spell)
      (if (>= (`TimelineComponent.GetPlaybackPosition` (`self.Timeline_Heal`)) 0.2)
        ;[1 1 1] Notify (just once) that we hit the tile (so the Unit can play the Hit animation)
        (`/Engine/EditorBlueprintResources/StandardMacros.DoOnce` false
          (:`Completed`
            (`self.OnSpellAnimationHitTile` self (`self.TargetIndex`))))))
    (:`Finished`
      ;[1 1 1] Responsable to destroy the BP when Animation ends
      (`self.Event_CompleteSpellAnimation`))))

(fn `UserConstructionScript`
  (`parent.UserConstructionScript`)
  (`MeshComponent.SetVectorParameterValueOnMaterials` (`self.StaticMesh_Inner`) "Color" (`KismetMathLibrary.Conv_LinearColorToVector` (struct :`R` 0.658824 :`G` 0.901961 :`B` 0.741176 :`A` 1.0)))
  (`MeshComponent.SetVectorParameterValueOnMaterials` (`self.StaticMesh_Plus1`) "Color" (`KismetMathLibrary.Conv_LinearColorToVector` (struct :`R` 0.658824 :`G` 0.901961 :`B` 0.741176 :`A` 1.0)))
  (`MeshComponent.SetVectorParameterValueOnMaterials` (`self.StaticMesh_Middle`) "Color" (`KismetMathLibrary.Conv_LinearColorToVector` (struct :`R` 0.26964 :`G` 0.739583 :`B` 0.333855 :`A` 1.0)))
  (`MeshComponent.SetVectorParameterValueOnMaterials` (`self.StaticMesh_Plus2`) "Color" (`KismetMathLibrary.Conv_LinearColorToVector` (struct :`R` 0.26964 :`G` 0.739583 :`B` 0.333855 :`A` 1.0)))
  (`MeshComponent.SetVectorParameterValueOnMaterials` (`self.StaticMesh_Outer`) "Color" (`KismetMathLibrary.Conv_LinearColorToVector` (struct :`R` 0.130344 :`G` 0.807292 :`B` 0.380741 :`A` 1.0)))
  (`MeshComponent.SetVectorParameterValueOnMaterials` (`self.StaticMesh_Plus3`) "Color" (`KismetMathLibrary.Conv_LinearColorToVector` (struct :`R` 0.130344 :`G` 0.807292 :`B` 0.380741 :`A` 1.0))))