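; BP_SpellAnim_RunChickenRun is the spell animation for the Run Chicken Run spell, overriding the parent's EventPlaySpellAnimation.
; It moves the actor to the target tile and sets its widget image to the spell's icon texture.
; A timeline then moves the widget along Z, resizes it and fades it in and out, and on finish calls EventCompleteSpellAnimation to end and destroy the actor.
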(event `self.Event_PlaySpellAnimation`
  (bind _widget (`self.Widget`))
  (bind _transform_location (`KismetMathLibrary.BreakTransform` (`self.GetTileTransform` (`self.TargetIndex`))))
  ;[1 1 1] We position the Widget (the image) on the TargetTile
  (`self.K2_SetActorLocation` _transform_location)
  ;[1 1 1] From the widget we get access to the Image and put it into a variable
  (bind _output_get (set `self.W_Image` (cast `/Game/Blueprints/Core/Combat/Spells/SpellAnimations/Components/W_Image` (`WidgetComponent.GetUserWidgetObject` (`self.Widget`)) :!pure true)))
  ;[1 1 1] We set the image from a texture
  (`Image.SetBrushFromTexture` (`/Game/Blueprints/Core/Combat/Spells/SpellAnimations/Components/W_Image.Image_Component` _output_get) "/Game/Blueprints/Core/Combat/Spells/SpellAnimations/Assets/Icon_RunChickenRun_NoBackground.Icon_RunChickenRun_NoBackground" false)
  (bind (_direction _locationz _drawsize _opacity) (`Timeline|Timeline_RunChickenRun` :!via `PlayFromStart`)
    (:`Update`
      ;[1 1 1] We move the image along Z
      (`SceneComponent.K2_SetRelativeLocation` _widget (`KismetMathLibrary.MakeVector` 0.0 0.0 _locationz) false false)
      ;[1 1 1] And scale it
      (`WidgetComponent.SetDrawSize` _widget (`KismetMathLibrary.MakeVector2D` _drawsize _drawsize))
      ;[1 1 1] The image will fade in and out
      (`Widget.SetRenderOpacity` (`self.W_Image`) _opacity))
    (:`Finished`
      ;[1 1 1] Responsable to destroy the BP when Animation ends
      (`self.Event_CompleteSpellAnimation`))))

(fn `UserConstructionScript`
  (`parent.UserConstructionScript`))