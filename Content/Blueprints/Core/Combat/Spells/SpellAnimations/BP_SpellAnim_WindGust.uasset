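; Spell animation Blueprint for the Wind Gust area-of-effect spell, radiating gusts from the target tile to the other attacked tiles.
; The target tile registers its hit after a brief delay.
; Each remaining tile gets a spawned BP_AnimatedWindGust that faces it, growing as it travels at a randomized play rate.
; Each gust's completion callback triggers that tile's hit and removes its index, completing the spell once none remain.
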(event `self.Event_PlaySpellAnimation`
  (bind _transform_location (`KismetMathLibrary.BreakTransform` (`self.GetTileTransform` (`self.TargetIndex`))))
  (`KismetSystemLibrary.Delay` 0.1) ; To give the Unit time before hooking to the callback
  ;[1 1 1 1 16] We're ignoring the target, because the AoE has its epicenter in the target and spawns the WindGusts from the target to the Attacked Tiles.
  ; The target Index gets removed right away and the (eventual) Unit on hit gets hit also right away
  ; the rest of the Attacked Indices instead, wait for the animation
  (`self.OnSpellAnimationHitTile` self (`self.TargetIndex`))
  (`KismetArrayLibrary.Array_RemoveItem` (`self.AttackIndexes`) (`self.TargetIndex`))
  ;[1 1 1] Since its an AoE, we loop on the attack indices
  (for _array_element (`self.AttackIndexes`)
    (bind _transform_location_2 (`KismetMathLibrary.BreakTransform` (`self.GetTileTransform` _array_element)))
    (bind _returnvalue (`KismetMathLibrary.FindLookAtRotation` _transform_location _transform_location_2))
    ;[1 1 1] And for each attack index, we spawn the WingGust BluePrint properly positioned and orientated
    (bind _returnvalue_2 (`|SpawnActorFromClass` "/Game/Blueprints/Core/Combat/Spells/SpellAnimations/Components/BP_AnimatedWindGust.BP_AnimatedWindGust_C" (`KismetMathLibrary.MakeTransform` (0.0 0.0 0.0)) "AlwaysSpawn" "MultiplyWithRoot" null (`KismetMathLibrary.MakeTransform` _transform_location _returnvalue (0.6 0.6 0.6)) (`KismetMathLibrary.MakeTransform` _transform_location_2 _returnvalue (1.2 1.2 1.2)) (`KismetMathLibrary.RandomFloatInRange` 0.8 1.5) _array_element null))
    ;[1 1 1] Since we need to destroy the BP at the end of the animation.
    ; We hook ourself to the event that will tell us when all the WindGusts have done with their animation (it's in the parent class)
    (add `/Game/Blueprints/Core/Combat/Spells/SpellAnimations/Components/BP_AnimatedWindGust.OnShapeAnimationCompleted` _returnvalue_2 (delegate `OnShapeAniomationCompleted`))))

(event `OnShapeAniomationCompleted`
  (params (AnimatedShape :type "/Game/Blueprints/Core/Combat/Spells/SpellAnimations/Components/BP_AnimatedWindGust Object Reference"))
  (bind _index (`/Game/Blueprints/Core/Combat/Spells/SpellAnimations/Components/BP_AnimatedWindGust.Index` AnimatedShape))
  (bind _attackindexes (`self.AttackIndexes`))
  ;[1 1 1] This notify the eventual Units hit by the spell to play their Hit animation when the spell reaches the Target Tile
  (`self.OnSpellAnimationHitTile` self _index)
  ;[1 1 1 1 16] To keep track of all the tiles examined/still to process of the current attack,
  ; we remove the Tile just processed from the AttackedIndices
  (`KismetArrayLibrary.Array_RemoveItem` _attackindexes _index)
  ;[1 1 1] When all the AttackIndices have been processed
  ; it means we're done with the spell
  (if (== (`KismetArrayLibrary.Array_Length` _attackindexes) 0)
    (`self.Event_CompleteSpellAnimation`) ; Notify the end of the animation
  ))

(fn `UserConstructionScript`
  (`parent.UserConstructionScript`))