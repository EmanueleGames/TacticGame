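; BP_AnimatedShape is a spell visual actor that flies a colored mesh from an origin to a target tile.
; On BeginPlay it applies the mesh, material and color, then runs a timeline at a set play rate to interpolate between origin and target transforms.
; A fixed lift avoids terrain flicker and a height offset curve adds a projectile arc.
; On finish it fires a completion dispatcher, then destroys itself after a short delay.
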(event `self.ReceiveBeginPlay`
  (bind _animatedshape (`self.AnimatedShape`))
  ;[1 1 1] Animation basic elements: mesh, material, color
  (`StaticMeshComponent.SetStaticMesh` _animatedshape (`self.Mesh`))
  (`PrimitiveComponent.SetMaterial` _animatedshape 0 (`self.Material`))
  (`MeshComponent.SetVectorParameterValueOnMaterials` _animatedshape "Color" (`KismetMathLibrary.Conv_LinearColorToVector` (`self.Color`)))
  ;[1 1 1] We use PlayRate to give the animation speed
  ; a little bit of variety, so it's less boring
  (`TimelineComponent.SetPlayRate` (`self.Timeline_PlayAnimation`) (`self.PlayRate`))
  ;[1 1 1] Spell aniamtion, we're using a timeline to realize a simple interpolation between Origin and Target Tile
  (bind (_direction _transformalpha _heightoffset) (`Timeline|Timeline_PlayAnimation` :!via `PlayFromStart`)
    (:`Update`
      (bind (_returnvalue_location _returnvalue_rotation _returnvalue_scale) (`KismetMathLibrary.BreakTransform` (`KismetMathLibrary.TLerp` (`self.OriginTransform`) (`self.TargetTransform`) _transformalpha)))
      (`self.K2_SetActorTransform` (`KismetMathLibrary.MakeTransform` (+ _returnvalue_location (0.0 0.0 50.0) (`KismetMathLibrary.MakeVector` 0.0 0.0 _heightoffset)) _returnvalue_rotation _returnvalue_scale)))
    (:`Finished`
      ;[1 1 1 1 16] We need this to destroy the Blueprint responsable to create the animation (witch is different from the object used in the animation destriyed right after the delay)
      (`self.OnShapeAnimationCompleted` self)
      ;[1 1 1] After a short delay, we destroy the shape used to animate
      (`KismetSystemLibrary.Delay` 0.5)
      (`self.K2_DestroyActor`))))

(fn `UserConstructionScript`)