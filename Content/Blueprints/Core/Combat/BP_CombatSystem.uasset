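; Combat system that tracks units in a grid-based battle and keeps each unit's index, tile occupancy and world location in sync with the Grid.
; SetUnitIndexOnGrid does the bookkeeping, fires an index-changed dispatcher and uses (-999,-999) as the off-grid index.
; Unit movement and grid dispatchers trigger updates; units left on invalid tile types are destroyed.
; Grid regeneration forces the update, since indices stay unchanged.
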(event `self.ReceiveBeginPlay`
  (bind _grid (`self.Grid`))
  ;[1 1 1 1 16] We bind on the Grid Generated and Tile Updated dispatchers to update Unit position when the grid gets modified
  ; Es. removing a unit when grid gets destroyed under it, shifting a unit if the tile under it gets higher or lower, etc.
  (add `/Game/Blueprints/Core/Grid/BP_Grid.OnGridGenerated` _grid (`|CreateDelegate` :!event `OnGridGenerated`))
  (add `/Game/Blueprints/Core/Grid/BP_Grid.OnTileDataUpdated` _grid (`|CreateDelegate` :!event `OnTileDataUpdated`)))

(fn `AddUnitInCombat`
  (params (Unit :type "/Game/Blueprints/Core/Units/BP_Unit Object Reference") (Index :type "IntPoint Structure"))
  ;[1 1 1] Unit gets added in the list
  (`KismetArrayLibrary.Array_Add` (`self.UnitsInCombat`) (`local.Unit`))
  ;[1 1 1] Unit knows its position on the Grid
  (`self.SetUnitIndexOnGrid` (`local.Unit`) Index)
  ;[1 1 1] Each Units needs a Grid reference for its movement
  (`/Game/Blueprints/Core/Units/BP_Unit.SetGrid` (`local.Unit`) (`self.Grid`))
  ;[1 1 1] We bind to the event that notify us when the unit reaches a new Tile
  ; to keep the combat system status updated and consistent
  (add `/Game/Blueprints/Core/Units/BP_Unit.OnUnitReachedNewTile` (`local.Unit`) (`|CreateDelegate` :!event `OnUnitReachedNewTile`)))

(fn `OnGridGenerated`
  (locals (CopyOfUnitsInCombat :type "Array of /Game/Blueprints/Core/Units/BP_Unit Object Reference"))
  ;[1 1 1] Since we have to operate on the unit inside the list by updateing or removing them,
  ; we can't operate directly in the list because the loop could break.
  ; To avoid this, we copy the list in a local variable and operate on this variable
  (bind _output_get (set `local.CopyOfUnitsInCombat` (`self.UnitsInCombat`)))
  (for _array_element _output_get
    (bind _index (`/Game/Blueprints/Core/Units/BP_Unit.Index` _array_element))
    ;[1 1 1] Lets check if the unit needs to be removed by comparing its allowed TileTypes with the one generated
    (if (`KismetArrayLibrary.Array_Contains` (`.ValidTileTypes_3_929725CE49027623BFBC479EBA9580D6` (break `/Game/Blueprints/Core/Units/Utilities/S_UnitData_Stats` (`.Stats_8_1FF4029D4CCC943B93A92087BC3004A2` (break `/Game/Blueprints/Core/Units/Utilities/S_UnitData` (`/Game/Blueprints/Core/Units/BP_Unit.UnitData` _array_element))))) (`.Type_8_8F74F19243475FAB39F94AA272B2F514` (break `/Game/Blueprints/Core/Grid/Utilities/S_TileData` (`BlueprintMapLibrary.Map_Find` (`/Game/Blueprints/Core/Grid/BP_Grid.GridTiles` (`self.Grid`)) _index))))
      (`self.SetUnitIndexOnGrid` _array_element _index true) ; No need to remove, just update position\nAnd FORCE is set TRUE because the indices will be the same as before so we need to bypass the check inside the function
      (else
        (`self.RemoveUnitFromCombat` _array_element) ; Unit needs to be removed
      ))))

(fn `OnTileDataUpdated`
  (params (index :type "IntPoint Structure"))
  (locals (CopyOfUnitsInCombat :type "Array of /Game/Blueprints/Core/Units/BP_Unit Object Reference"))
  ;[1 1 1] Since we have to operate on the unit inside the list by updateing or removing them,
  ; we can't operate directly in the list because the loop could break.
  ; To avoid this, we copy the list in a local variable and operate on this variable
  (bind _output_get (set `local.CopyOfUnitsInCombat` (`self.UnitsInCombat`)))
  (for _array_element _output_get
    (bind _index (`/Game/Blueprints/Core/Units/BP_Unit.Index` _array_element))
    ;[1 1 1] Before doing any operation we check if between the units in combat there is one at the position of the input index that needs to be updated
    (if (`KismetMathLibrary.Equal_IntPointIntPoint` (`local.index`) _index)
      ;[1 1 1] Lets check if the unit needs to be removed by comparing its allowed TileTypes with the new one we just updated
      (if (`KismetArrayLibrary.Array_Contains` (`.ValidTileTypes_3_929725CE49027623BFBC479EBA9580D6` (break `/Game/Blueprints/Core/Units/Utilities/S_UnitData_Stats` (`.Stats_8_1FF4029D4CCC943B93A92087BC3004A2` (break `/Game/Blueprints/Core/Units/Utilities/S_UnitData` (`/Game/Blueprints/Core/Units/BP_Unit.UnitData` _array_element))))) (`.Type_8_8F74F19243475FAB39F94AA272B2F514` (break `/Game/Blueprints/Core/Grid/Utilities/S_TileData` (`BlueprintMapLibrary.Map_Find` (`/Game/Blueprints/Core/Grid/BP_Grid.GridTiles` (`self.Grid`)) _index))))
        (`self.SetUnitIndexOnGrid` _array_element _index) ; No need to remove, just update position
        (break)
        (else
          (`self.RemoveUnitFromCombat` _array_element) ; Unit needs to be removed
          (break))))))

(fn `OnUnitReachedNewTile`
  (params (Unit :type "/Game/Blueprints/Core/Units/BP_Unit Object Reference") (Index :type "IntPoint Structure"))
  (`self.SetUnitIndexOnGrid` Unit Index) ; Update Unit position on Grid
)

(fn `RemoveUnitFromCombat`
  (params (Unit :type "/Game/Blueprints/Core/Units/BP_Unit Object Reference") (DestroyUnit :type Boolean :default true))
  (`KismetArrayLibrary.Array_RemoveItem` (`self.UnitsInCombat`) (`local.Unit`))
  (`self.SetUnitIndexOnGrid` (`local.Unit`) (make `IntPoint` -999 -999))
  (if DestroyUnit
    ;[1 1 1] Removes the unit from the scene
    (`self.K2_DestroyActor` (`local.Unit`))))

(fn `SetUnitIndexOnGrid`
  (params (Unit :type "/Game/Blueprints/Core/Units/BP_Unit Object Reference") (Index :type "IntPoint Structure") (Force :type Boolean :default false))
  (locals (PreviousTile :type "/Game/Blueprints/Core/Grid/Utilities/S_TileData Structure"))
  (bind (_value _returnvalue) (`BlueprintMapLibrary.Map_Find` (`/Game/Blueprints/Core/Grid/BP_Grid.GridTiles` (`self.Grid`)) (`local.Index`)))
  (`|ExecutionSequence`
    (:`then_0`
      ;[1 1 1] We compare the old and the new index,
      ; if they are the same, we don't do anything
      (if (or (!= (`/Game/Blueprints/Core/Units/BP_Unit.Index` (`local.Unit`)) (`local.Index`)) (`local.Force`))
        (`|ExecutionSequence`
          (:`then_0`
            ;[1 1 1 1 16] First we use the index contained in the Unit to access the TileData from the Grid
            (bind _output_get (set `local.PreviousTile` (`BlueprintMapLibrary.Map_Find` (`/Game/Blueprints/Core/Grid/BP_Grid.GridTiles` (`self.Grid`)) (`/Game/Blueprints/Core/Units/BP_Unit.Index` (`local.Unit`)))))
            ;[1 1 1] Then we check if the previous tile data has a unit identical to the one we have in input
            (if (== (`.UnitOnTile_16_1A24A24A4845A31FB93E7BBEC72A5FD3` (break `/Game/Blueprints/Core/Grid/Utilities/S_TileData` _output_get)) (`local.Unit`))
              ;[1 1 1] If they're the same, we set the UnitOnTile as empty in the previous tile structure and update its values in the structure (using the same index we're overwriting old values in the GridTiles)
              (bind _structout (setmembers `/Game/Blueprints/Core/Grid/Utilities/S_TileData` :`StructRef` (`local.PreviousTile`) :`UnitOnTile` null)) ; Selecting this node will let us choice what pin to expose
              (`BlueprintMapLibrary.Map_Add` (`/Game/Blueprints/Core/Grid/BP_Grid.GridTiles` (`self.Grid`)) (`.Index_4_844FDD494ED72091EFDF51BFC3ED2CE5` (break `/Game/Blueprints/Core/Grid/Utilities/S_TileData` _structout)) _structout)))
          (:`then_1`
            ;[1 1 1] We first update the index in the Unit data
            (set `/Game/Blueprints/Core/Units/BP_Unit.Index` (`local.Index`) (`local.Unit`))
            ;[1 1 1] Then we exclude [-999,-999] as valid index
            ; because it's reserved for initialization off grid
            (if (!= (`local.Index`) (make `IntPoint` -999 -999))
              ;[1 1 1] Now we're ready to get the data of the tile in the grid at the corresponding index in input and update the unit placed on it (with the one in input)
              (bind _structout_2 (setmembers `/Game/Blueprints/Core/Grid/Utilities/S_TileData` :`StructRef` (`BlueprintMapLibrary.Map_Find` (`/Game/Blueprints/Core/Grid/BP_Grid.GridTiles` (`self.Grid`)) (`local.Index`)) :`UnitOnTile` (`local.Unit`))) ; Selecting this node will let us choice what pin to expose
              ;[1 1 1] Then we overwrite the values in the list
              (`BlueprintMapLibrary.Map_Add` (`/Game/Blueprints/Core/Grid/BP_Grid.GridTiles` (`self.Grid`)) (`.Index_4_844FDD494ED72091EFDF51BFC3ED2CE5` (break `/Game/Blueprints/Core/Grid/Utilities/S_TileData` _structout_2)) _structout_2)))
          (:`then_2`
            ;[1 1 1] This events is needed because even if we updated the index of the Unit in the Grid, when the unit moves the Selected Tile wont update accordingly to its movement. For expample, if we move from Tile A to Tile B, at the end of the movement the Selected Unit is gonna be on Tile B while the Selected Tile is still Tile A. And this events updates the selected Tile to keep the selection consistency
            (`self.OnUnitGridIndexChanged` (`local.Unit`))))))
    (:`then_1`
      (`self.K2_SetActorLocation` (`local.Unit`) (select `bool` _returnvalue :`false` (-99999.0 -99999.0 -99999.0) :`true` (.location (`.Transform_7_D016BDCC41B32F0EC4D85EB94D99E603` (break `/Game/Blueprints/Core/Grid/Utilities/S_TileData` _value)))) false false))))

(fn `UserConstructionScript`)