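; Ranger unit AI that adjusts the generic unit AI's movement to favor running away from enemies.
; CastSpell flags the turn once any spell with a damaging HP impact is cast, then continues the parent logic.
; GetUnitMovementLogic retreats after a damaging cast, otherwise alternates by turn parity between retreating and getting closer.
; The turn counter resets at combat start, and the damage flag clears each turn.
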(event `self.CastSpell`
  ;[1 1 1] First we want to check if the Spell that is going to be casted is a damaging one
  (bind _spelldata (`/Game/Blueprints/Core/Combat/Spells/Utilities/BFL_Spells.GetSpellDataFromSpell` (`.Spell_11_048F0208424B968706ECEEA2E383354B` (break `/Game/Blueprints/Core/Units/AI/S_UnitAiSpellCastingData` (`self.AiSpellCasting`)))))
  (set `self.DamagedAnUnitThisTurn` (or (`self.DamagedAnUnitThisTurn`) (< (`.X` (break `IntPoint` (`.MinMaxModifier_Hp_2_6DDF92144525D3619EA8028342570120` (break `/Game/Blueprints/Core/Combat/Spells/Utilities/S_SpellData_Impact` (`.Impact_19_502CDF9B4E4405DCA26C9980B11823D1` (break `/Game/Blueprints/Core/Combat/Spells/Utilities/S_SpellData` _spelldata)))))) 0)))
  (`parent.CastSpell`) ; Keep following the General AI CastSpell logic
)

(fn `AiCombatStarted`
  (set `self.TurnCount` 0) ; Reset Turn Count
  (`parent.AiCombatStarted`))

(fn `AiPlayTurn`
  (`/Engine/EditorBlueprintResources/StandardMacros.IncrementInt` (`self.TurnCount`)
    (:`  `
      (set `self.DamagedAnUnitThisTurn` false) ; Reset the flag
      (`parent.AiPlayTurn`) ; Same AI logic of all generic Units
    )))

(fn `GetUnitMovementLogic`
  (returns (MovementLogic :type "/Game/Blueprints/Core/Units/AI/E_UnitAiMovementLogic Enum"))
  (return (select `bool` (and (`/Game/Blueprints/Core/Utilities/BFL_Utilities.IsIntEven` (`self.TurnCount`)) (not (`self.DamagedAnUnitThisTurn`))) :`false` "NewEnumerator2" :`true` "NewEnumerator0" :!type "/Game/Blueprints/Core/Units/AI/E_UnitAiMovementLogic Enum")))

(fn `UserConstructionScript`
  (`parent.UserConstructionScript`))