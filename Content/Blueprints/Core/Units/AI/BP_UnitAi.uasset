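; BP_UnitAi runs a unit's turn in a grid tactics combat system, stepping through delayed states before calling NextUnit.
; Spell selection, positioning and casting are placeholder steps that only set state.
; End-turn movement chains two async pathfinding requests through bind/unbind callbacks: reachable tiles, then a path to the chosen one.
; Movement logic picks the tile nearest enemies or allies, or maximizes distance from the closest one.
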(event `Event_RunAILogic`
  (`self.SetAiStateWithDelay` "NewEnumerator1")
  (`self.DecideWitchSpellToCast`))

(event `DecideWitchSpellToCast`
  (`self.SetAiStateWithDelay` "NewEnumerator2")
  (`self.DecideWitchSpellToCast_Done`))

(event `DecideWitchSpellToCast_Done`
  (`self.MoveToSpellCastingLocation`))

(event `MoveToSpellCastingLocation`
  (`self.SetAiStateWithDelay` "NewEnumerator3")
  (`self.MoveToSpellCastingLocation_Done`))

(event `MoveToSpellCastingLocation_Done`
  (`self.CastSpell`))

(event `CastSpell`
  (`self.SetAiStateWithDelay` "NewEnumerator4")
  (`self.CastSpell_Done`))

(event `CastSpell_Done`
  (`self.DecideWhereToEndTurn`))

(event `MoveToEndTurnLocation_Done`
  (`self.SetAiStateWithDelay` "NewEnumerator6")
  (`self.AiEndTurn`))

(event `DecideWhereToEndTurn`
  (bind _unit (`self.Unit`))
  (bind ((`ValidTileTypes_3_929725CE49027623BFBC479EBA9580D6` _validtiletypes) (`CanMoveDiagonally_7_7E720D6645739EC9FF74959433CD15E1` _canmovediagonally) (`MP_Current_10_FB397B3D409E5FAEA964D8A44B0876D5` _mp_current)) (break `/Game/Blueprints/Core/Units/Utilities/S_UnitData_Stats` (`.Stats_8_1FF4029D4CCC943B93A92087BC3004A2` (break `/Game/Blueprints/Core/Units/Utilities/S_UnitData` (`/Game/Blueprints/Core/Units/BP_Unit.UnitData` _unit)))))
  (`self.SetAiStateWithDelay` "NewEnumerator5")
  ;[1 1 1] Does the Unit have at least one step? (can move?)
  (if (> (`.MP_Current_10_FB397B3D409E5FAEA964D8A44B0876D5` (break `/Game/Blueprints/Core/Units/Utilities/S_UnitData_Stats` (`.Stats_8_1FF4029D4CCC943B93A92087BC3004A2` (break `/Game/Blueprints/Core/Units/Utilities/S_UnitData` (`/Game/Blueprints/Core/Units/BP_Unit.UnitData` (`self.Unit`)))))) 0)
    ;[1 1 1] We have MovementPoints, lets bind to the event
    ; that notify us when the pathfinding for the reachables  is done
    (add `/Game/Blueprints/Core/Grid/BP_GridPathfinding.OnPathfindingCompleted` (`self.GetPathfinding`) (delegate `OnCompleted_EndTurnReachables`))
    ;[1 1 1] And ask for the Reachables, when done will notify us with the event we just bound to
    (`/Game/Blueprints/Core/Grid/BP_GridPathfinding.FindPath` (`self.GetPathfinding`) (`/Game/Blueprints/Core/Units/BP_Unit.Index` _unit) (make `IntPoint` -999 -999) _canmovediagonally _validtiletypes 0.1 15.0 true _mp_current)
    (else
      (`self.DecideWhereToEndTurn_Done` (`|MakeArray`)) ; Can't move
    )))

(event `OnCompleted_EndTurnReachables`
  (params (Path :type "Array of IntPoint Structure (by ref)"))
  (bind _unit (`self.Unit`))
  (bind ((`ValidTileTypes_3_929725CE49027623BFBC479EBA9580D6` _validtiletypes) (`CanMoveDiagonally_7_7E720D6645739EC9FF74959433CD15E1` _canmovediagonally) (`MP_Current_10_FB397B3D409E5FAEA964D8A44B0876D5` _mp_current)) (break `/Game/Blueprints/Core/Units/Utilities/S_UnitData_Stats` (`.Stats_8_1FF4029D4CCC943B93A92087BC3004A2` (break `/Game/Blueprints/Core/Units/Utilities/S_UnitData` (`/Game/Blueprints/Core/Units/BP_Unit.UnitData` _unit)))))
  ;[1 1 1 1 16] Unbind from the Pathfinding Completed event
  ; because we're gonna re-use FindPath again and we don't want to be notified here again
  ; otherwise the execution would fire again from the event OnCompleted_EndTurnReachables
  (remove `/Game/Blueprints/Core/Grid/BP_GridPathfinding.OnPathfindingCompleted` (`self.GetPathfinding`) (delegate `OnCompleted_EndTurnReachables`))
  (bind _bestindex (`self.FindBestIndexInReachables` Path)) ; Decides what is the best Tile to move to\nfor the  specific Unit in use of the AI
  ;[1 1 1] We bind again to the same event, but this time we are not interested in the reachables anymore, we will be instead notified when the path to the BestIndex is completed
  (add `/Game/Blueprints/Core/Grid/BP_GridPathfinding.OnPathfindingCompleted` (`self.GetPathfinding`) (delegate `OnCompleted_EndTurnPath`))
  ;[1 1 1] Find us the Path to the BestIndex
  (`/Game/Blueprints/Core/Grid/BP_GridPathfinding.FindPath` (`self.GetPathfinding`) (`/Game/Blueprints/Core/Units/BP_Unit.Index` _unit) _bestindex _canmovediagonally _validtiletypes 0.1 15.0 false _mp_current))

(event `OnCompleted_EndTurnPath`
  (params (Path :type "Array of IntPoint Structure (by ref)"))
  ;[1 1 1 1 16] Unbind from the Pathfinding Completed event
  ; because we're gonna re-use FindPath again and we don't want to be notified here again
  ; otherwise the execution would fire again from the event OnCompleted_EndTurnPath
  (remove `/Game/Blueprints/Core/Grid/BP_GridPathfinding.OnPathfindingCompleted` (`self.GetPathfinding`) (delegate `OnCompleted_EndTurnPath`))
  ;[1 1 1] Path to the BestIndex is set, this step is complete
  ; In the next one the AI is gonna move the Unit
  (`self.DecideWhereToEndTurn_Done` Path))

(event `DecideWhereToEndTurn_Done`
  (params (Path :type "Array of IntPoint Structure"))
  (`self.MoveToEndTurnLocation` Path))

(event `MoveToEndTurnLocation`
  (params (Path :type "Array of IntPoint Structure"))
  ;[1 1 1] Do we have a Path? We need to move or not?
  (if (> (`KismetArrayLibrary.Array_Length` Path) 0)
    (`self.SetAiStateWithDelay` "NewEnumerator7")
    ;[1 1 1] We want be notified when the Unit has reached its TargetTile
    (add `/Game/Blueprints/Core/Units/BP_Unit.OnUnitFinishedWalking` (`self.Unit`) (delegate `OnCompleted_EndTurnUnitWalking`))
    (`/Game/Blueprints/Core/Combat/BP_CombatSystem.MoveUnit` (`self.CombatSystem`) (`self.Unit`) Path) ; Move the Unit
    (else
      (`self.MoveToEndTurnLocation_Done`) ; No Path, step is done!
    )))

(event `OnCompleted_EndTurnUnitWalking`
  (params (Unit :type "/Game/Blueprints/Core/Units/BP_Unit Object Reference"))
  ;[1 1 1] Unbind from the OnUnitFinishedWalking event
  ; because we're gonna re-use Move Unit again and we don't want to be notified here again
  ; otherwise the execution would fire again from the event OnCompleted_EndTurnUnitWalking
  (remove `/Game/Blueprints/Core/Units/BP_Unit.OnUnitFinishedWalking` Unit (delegate `OnCompleted_EndTurnUnitWalking`))
  (`self.MoveToEndTurnLocation_Done`) ; Move complete, step is done!
)

(fn `AiEndTurn`
  ;[1 1 1] Calls the next Unit in the turn order
  (`/Game/Blueprints/Core/Combat/BP_CombatSystem.NextUnit` (`self.CombatSystem`)))

(fn `AiPlayTurn`
  (`self.Event_RunAILogic`))

(fn `FindBestIndexInReachables`
  (params (Reachables :type "Array of IntPoint Structure (by ref)"))
  (returns (BestIndex :type "IntPoint Structure"))
  (locals (EnemiesOrAllies :type "Array of IntPoint Structure"))
  (bind _movementlogic (break `/Game/Blueprints/Core/Units/Utilities/S_UnitData_AI` (`.Ai_14_CFD0EC8F478A64C63AE3BA83872C58F6` (break `/Game/Blueprints/Core/Units/Utilities/S_UnitData` (`/Game/Blueprints/Core/Units/BP_Unit.UnitData` (`self.Unit`))))))
  (`|ExecutionSequence`
    (:`then_0`
      ;[1 1 1] Get the Unit behaviour
      (switch `/Game/Blueprints/Core/Units/AI/E_UnitAiMovementLogic` _movementlogic
        (:`NewEnumerator0`
          ;[1 1 1] We need the Enemies to determine the best move
          (bind _units (`self.GetEnemyUnits` (`|MakeArray`) :!label _label))
          (bind _keys (`BlueprintMapLibrary.Map_Keys` _units))
          (set `local.EnemiesOrAllies` _keys))
        (:`NewEnumerator1`
          ;[1 1 1] We need the Allies to determine the best move
          (bind _units_2 (`self.GetAllyUnits` false :!label _label_2))
          (bind _keys_2 (`BlueprintMapLibrary.Map_Keys` _units_2))
          (set `local.EnemiesOrAllies` _keys_2))
        (:`NewEnumerator2`
          (goto _label))
        (:`NewEnumerator3`
          (goto _label_2))))
    (:`then_1`
      (switch `/Game/Blueprints/Core/Units/AI/E_UnitAiMovementLogic` _movementlogic
        (:`NewEnumerator0`
          _)
        (:`NewEnumerator1`
          _)
        (:`NewEnumerator2`
          ;[1 1 1] We want to move AWAY from the Units found on step 0
          (bind _index (`self.FindFarthestIndex` (`local.Reachables`) (`local.EnemiesOrAllies`) :!label _label_3))
          (return _index))
        (:`NewEnumerator3`
          (goto _label_3)))
      ;[1 1 1] We want to move TOWARDS the Unit found on step 0
      (bind _index_2 (`self.FindClosestIndex` (`local.Reachables`) (`local.EnemiesOrAllies`)))
      (return _index_2))))

(fn `FindClosestIndex`
  (params (Reachables :type "Array of IntPoint Structure") (PossibleTargets :type "Array of IntPoint Structure"))
  (returns (Index :type "IntPoint Structure"))
  (locals (Ret :type "IntPoint Structure") (SmallestDistance :type Integer) (Reachable :type "IntPoint Structure") (Target :type "IntPoint Structure") (NewDistance :type Integer :default 0))
  (set `local.SmallestDistance` 999999999)
  ;[1 1 1] Loop on the Reachables...
  (for _array_element (`local.Reachables`)
    (set `local.Reachable` _array_element)
    ;[1 1 1] ...and on the Targets
    (for _array_element_2 (`local.PossibleTargets`)
      (set `local.Target` _array_element_2)
      ;[1 1 1] Calculate the distance between each couple Reachable-Target
      (bind _output_get (set `local.NewDistance` (`/Game/Blueprints/Core/Grid/BP_GridPathfinding.GetMinimumCostBetweenTwoTiles` (`/Game/Blueprints/Core/Grid/BP_Grid.GridPathfinding_AI` (`/Game/Blueprints/Core/Combat/BP_CombatSystem.Grid` (`self.CombatSystem`))) (`local.Reachable`) (`local.Target`) (`.CanMoveDiagonally_7_7E720D6645739EC9FF74959433CD15E1` (break `/Game/Blueprints/Core/Units/Utilities/S_UnitData_Stats` (`.Stats_8_1FF4029D4CCC943B93A92087BC3004A2` (break `/Game/Blueprints/Core/Units/Utilities/S_UnitData` (`/Game/Blueprints/Core/Units/BP_Unit.UnitData` (`self.Unit`)))))))))
      ;[1 1 1] And compare it with the SmallestDistance found until now
      (if (< _output_get (`local.SmallestDistance`))
        ;[1 1 1] If lower than we update our Output and our new Smallest Distance
        ; (if we find a better Reachable, we update again and overwrite them)
        (set `local.Ret` (`local.Reachable`))
        (set `local.SmallestDistance` (`local.NewDistance`)))))
  (return (`local.Ret`)) ; Function is done!
)

(fn `FindFarthestIndex`
  (params (Reachables :type "Array of IntPoint Structure") (IndexesToAvoid :type "Array of IntPoint Structure"))
  (returns (Index :type "IntPoint Structure"))
  (locals (Ret :type "IntPoint Structure") (BiggestDistance :type Integer) (Reachable :type "IntPoint Structure") (ToAvoid :type "IntPoint Structure") (NewDistance :type Integer))
  (set `local.BiggestDistance` -99999999)
  ;[1 1 1] Loop on the Reachables...
  (for _array_element (`local.Reachables`)
    (set `local.Reachable` _array_element)
    (set `local.NewDistance` 999999999)
    ;[1 1 1] ...and on the Indexes to avoid
    (for _array_element_2 (`local.IndexesToAvoid`)
      (set `local.ToAvoid` _array_element_2)
      ;[1 1 1] we update the new Distance with the smallest value between the old value and the cost just calculated
      ; we're asking: is this Tile ToAvoid closer (more dangerous) to the current Reachable than the ones before
      (set `local.NewDistance` (`KismetMathLibrary.Min` (`local.NewDistance`) (`/Game/Blueprints/Core/Grid/BP_GridPathfinding.GetMinimumCostBetweenTwoTiles` (`/Game/Blueprints/Core/Grid/BP_Grid.GridPathfinding_AI` (`/Game/Blueprints/Core/Combat/BP_CombatSystem.Grid` (`self.CombatSystem`))) (`local.Reachable`) (`local.ToAvoid`) (`.CanMoveDiagonally_7_7E720D6645739EC9FF74959433CD15E1` (break `/Game/Blueprints/Core/Units/Utilities/S_UnitData_Stats` (`.Stats_8_1FF4029D4CCC943B93A92087BC3004A2` (break `/Game/Blueprints/Core/Units/Utilities/S_UnitData` (`/Game/Blueprints/Core/Units/BP_Unit.UnitData` (`self.Unit`))))))))))
    ;[1 1 1] When we have decided how close is the closest threat for the current Reachable
    ; We have all the elements to decide if this Reachable is safer (far away) than the others
    (if (> (`local.NewDistance`) (`local.BiggestDistance`))
      ;[1 1 1] If safer, we update our Return and compare values
      ; (if we find a safer Reachable, we update again and overwrite them)
      (set `local.Ret` (`local.Reachable`))
      (set `local.BiggestDistance` (`local.NewDistance`))))
  (return (`local.Ret`)) ; Function is done!
)

(fn `GetAllyUnits`
  (params (IncludeSelf :type Boolean))
  (returns (Units :type "Map of IntPoint Structure to /Game/Blueprints/Core/Units/BP_Unit Object Reference"))
  (locals (Ret :type "Map of IntPoint Structure to /Game/Blueprints/Core/Units/BP_Unit Object Reference") (UnitLocal :type "/Game/Blueprints/Core/Units/BP_Unit Object Reference"))
  (bind _unitlocal (`local.UnitLocal`))
  ;[1 1 1] Find all the Unit that are on the same Team of the Unit in input and loop them
  (bind _result (`BlueprintSetLibrary.Set_ToArray` (`.UnitSet_3_BEF553954C5D7EB6C9912FB3D4D40761` (break `/Game/Blueprints/Core/Combat/Utilities/S_UnitSet` (`BlueprintMapLibrary.Map_Find` (`/Game/Blueprints/Core/Combat/BP_CombatSystem.UnitTeams` (`self.CombatSystem`)) (`/Game/Blueprints/Core/Units/BP_Unit.TeamIndex` (`self.Unit`)))))))
  (for _array_element _result
    (set `local.UnitLocal` _array_element)
    ;[1 1 1] We only return alive Units
    (if (`/Game/Blueprints/Core/Units/BP_Unit.IsAlive` (`local.UnitLocal`))
      ;[1 1 1] Based on the boolean input, we ignore/include ourself among the Ally Units
      (if (or (!= (`local.UnitLocal`) (`self.Unit`)) (`local.IncludeSelf`))
        ;[1 1 1] Add the Unit to the Return Array
        (`BlueprintMapLibrary.Map_Add` (`local.Ret`) (`/Game/Blueprints/Core/Units/BP_Unit.Index` _unitlocal) _unitlocal))))
  (return (`local.Ret`)))

(fn `GetEnemyUnits`
  (params (SpecificTeamIndex :type "Array of Integer"))
  (returns (Units :type "Map of IntPoint Structure to /Game/Blueprints/Core/Units/BP_Unit Object Reference"))
  (locals (Ret :type "Map of IntPoint Structure to /Game/Blueprints/Core/Units/BP_Unit Object Reference") (Teams :type "Array of Integer") (UnitLocal :type "/Game/Blueprints/Core/Units/BP_Unit Object Reference"))
  (bind _unitlocal (`local.UnitLocal`))
  ;[1 1 1] Was any specific Team requested in input?
  ; If not, we're gonna return every Unit from every Enemy Team
  (if (> (`KismetArrayLibrary.Array_Length` SpecificTeamIndex) 0)
    ;[1 1 1] Get only specified Teams
    (set `local.Teams` (`local.SpecificTeamIndex`))
    (else
      ;[1 1 1] Get all Teams
      (bind _keys (`BlueprintMapLibrary.Map_Keys` (`/Game/Blueprints/Core/Combat/BP_CombatSystem.UnitTeams` (`self.CombatSystem`))))
      (set `local.Teams` _keys)))
  ;[1 1 1] exclude ally Team
  (`KismetArrayLibrary.Array_Remove` (`local.Teams`) (`/Game/Blueprints/Core/Units/BP_Unit.TeamIndex` (`self.Unit`)))
  ;[1 1 1] Loop on each filtered Team...
  (for _array_element (`local.Teams`)
    (bind _result (`BlueprintSetLibrary.Set_ToArray` (`.UnitSet_3_BEF553954C5D7EB6C9912FB3D4D40761` (break `/Game/Blueprints/Core/Combat/Utilities/S_UnitSet` (`BlueprintMapLibrary.Map_Find` (`/Game/Blueprints/Core/Combat/BP_CombatSystem.UnitTeams` (`self.CombatSystem`)) _array_element)))))
    ;[1 1 1] ...and on every Unit on that Team
    (for _array_element_2 _result
      (set `local.UnitLocal` _array_element_2)
      ;[1 1 1] We only return alive Units
      (if (`/Game/Blueprints/Core/Units/BP_Unit.IsAlive` (`local.UnitLocal`))
        ;[1 1 1] Add the Unit to the Return Array
        (`BlueprintMapLibrary.Map_Add` (`local.Ret`) (`/Game/Blueprints/Core/Units/BP_Unit.Index` _unitlocal) _unitlocal))))
  (return (`local.Ret`)))

(fn `GetPathfinding`
  (returns (PathfindingAI :type "/Game/Blueprints/Core/Grid/BP_GridPathfinding Object Reference"))
  (return (`/Game/Blueprints/Core/Grid/BP_Grid.GridPathfinding_AI` (`/Game/Blueprints/Core/Combat/BP_CombatSystem.Grid` (`self.CombatSystem`)))))

(fn `UserConstructionScript`)