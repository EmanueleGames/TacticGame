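; Grid-based tactics unit actor whose type-driven data sets its mesh, animation, HP/MP/AP stats and available spells.
; A timeline walks it tile by tile along paths, with separate location and rotation curves plus a hop between heights.
; Spell hits change HP immediately but defer bar, number and hit/death animations until the spell animation reaches its tile.
; Also handles hover/selection tint, team colors, grid-shaped line-of-sight collision and broadcasts change events.
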(event `self.ReceiveBeginPlay`
  (`self.SetAnimationState` "NewEnumerator0")
  ;[1 1 1] HP bar initialization
  (bind _output_get (set `self.HpBar` (cast `/Game/Blueprints/Core/Units/Widget/W_HpBar` (`WidgetComponent.GetUserWidgetObject` (`self.Widget_HpBar`)) :!pure true)))
  (`/Game/Blueprints/Core/Units/Widget/W_HpBar.Event_SetUnit` _output_get self))

(event `Event_FollowPath`
  (params (Path :type "Array of IntPoint Structure"))
  ;[1 1 1] Does the path have at least one step?
  (if (> (`KismetArrayLibrary.Array_Length` Path) 0)
    ;[1 1 1] Beginning of the movement
    (set `self.CurrentPathToFollow` Path)
    (`self.OnUnitStartedWalking` self) ; To notify the start of the movement\n(es. to remove old reachable tiles)
    (`self.Event_ContinueToFollowPath`)))

(event `Event_ContinueToFollowPath`
  (bind _previustransform_location (`KismetMathLibrary.BreakTransform` (`self.PreviusTransform`)))
  (bind _nexttransform_location (`KismetMathLibrary.BreakTransform` (`self.NextTransform`)))
  (bind (_previustransform_location_2 _previustransform_rotation) (`KismetMathLibrary.BreakTransform` (`self.PreviusTransform`)))
  (bind (_nexttransform_location_2 _nexttransform_rotation) (`KismetMathLibrary.BreakTransform` (`self.NextTransform`)))
  (bind _previustransform_location_3 (`KismetMathLibrary.BreakTransform` (`self.PreviusTransform`)))
  (bind _timeline_unitmovement (`self.Timeline_UnitMovement`))
  (bind (_index _type _transform) (break `/Game/Blueprints/Core/Grid/Utilities/S_TileData` (`BlueprintMapLibrary.Map_Find` (`/Game/Blueprints/Core/Grid/BP_Grid.GridTiles` (`self.Grid`)) (`|GetArrayItem` (`self.CurrentPathToFollow`)))))
  (bind (_returnvalue_roll _returnvalue_pitch _returnvalue_yaw) (`KismetMathLibrary.BreakRotator` (`KismetMathLibrary.FindLookAtRotation` _previustransform_location_3 (.location _transform))))
  ;[1 1 1] Is there another step to make? True = continue, False = stop
  (if (> (`KismetArrayLibrary.Array_Length` (`self.CurrentPathToFollow`)) 0)
    (`self.SetAnimationState` "NewEnumerator1") ; Change Unit animation
    ;[1 1 1] PreviousTile is always the Unit current position (X)
    (set `self.PreviusTransform` (`self.GetTransform`))
    ;[1 1 1] To get the next tile we get the first element from what's left in the path to follow.
    ; NB. Current path to follow removes a step after it's made by the unit, so the first element will always be the next step to follow
    (set `self.NextTransform` (`KismetMathLibrary.MakeTransform` (.location _transform) (`KismetMathLibrary.MakeRotator` 0.0 0.0 _returnvalue_yaw)))
    ;[1 1 1] Before calling the timeline to interpolate the two transforms
    ; we set its playrate to adjust the speed of the animation
    (`TimelineComponent.SetPlayRate` _timeline_unitmovement (/ (`TimelineComponent.GetTimelineLength` _timeline_unitmovement) (`self.MoveDurationPerTile`)))
    ;[1 1 1 1 16] This let us interpolate between all the points dictated by the path to follow.
    ; If we doucle click on the Timeline node, we can set up the interpolation curves (we called them LocationAlpha and RotationAlpha).
    ; We have two different lerping curves because we want the location to be linear from start to end, but the rotation has to be quicker (unit has to look completely in the correct direction way before the step is completed) and smoother (no angles on the curve)
    ; Every game update the Update pin fires out and we set the "delta location and rotation" for the corresponding actor based on how much "delta time" has passed.
    ; To accomplish this we feed the final node with Lerp nodes that interpolates between two transform variables
    ; "Previous" contains data for the tile X and "Next" for the tile X+1.
    (bind (_direction _locationalpha _rotationalpha _jump) (`Timeline|Timeline_UnitMovement` :!via `PlayFromStart`)
      (:`Update`
        (`self.K2_SetActorLocationAndRotation` (+ (`KismetMathLibrary.VLerp` _previustransform_location _nexttransform_location _locationalpha) (`KismetMathLibrary.MakeVector` 0.0 0.0 (`KismetMathLibrary.SelectFloat` 0.0 _jump (`KismetMathLibrary.NearlyEqual_FloatFloat` (.z (.location (`self.PreviusTransform`))) (.z (.location (`self.NextTransform`))) 5.0)))) (`KismetMathLibrary.RLerp` _previustransform_rotation _nexttransform_rotation _rotationalpha true)))
      (:`Finished`
        ;[1 1 1] Before moving to the next step, we notify that the Unit has reached a new Tile
        (`self.OnUnitReachedNewTile` self (`|GetArrayItem` (`self.CurrentPathToFollow`)))
        ;[1 1 1] After each step made, before looping to the next adjacent tile couple, the last step is removed from the list of the remaining step to do
        (`KismetArrayLibrary.Array_Remove` (`self.CurrentPathToFollow`))
        (`self.Event_ContinueToFollowPath`)))
    (else
      (`self.SetAnimationState` "NewEnumerator0") ; Movement is over\nChange Unit animation
      ;[1 1 1] We notify the end of the movement
      (`self.OnUnitFinishedWalking` self))))

(event `Debug_RespawnAfterFewSeconds`
  (`KismetSystemLibrary.Delay` 2.0)
  ;[1 1 1] Unit healed to the Max
  (`self.SetCurrentHp` (`.HP_Max_20_56606D324C12E5DB5E7681B94263A483` (break `/Game/Blueprints/Core/Units/Utilities/S_UnitData_Stats` (`.Stats_8_1FF4029D4CCC943B93A92087BC3004A2` (break `/Game/Blueprints/Core/Units/Utilities/S_UnitData` (`self.UnitData`))))))
  (`self.SetAnimationState` "NewEnumerator5") ; Play the Respawn animation
  (`/Game/Blueprints/Core/Units/Widget/W_HpBar.Event_UpdateHpBar` (`self.HpBar`)) ; Update the Unit's HP bar
)

(fn `CanCastSpell`
  (params (SpellData :type "/Game/Blueprints/Core/Combat/Spells/Utilities/S_SpellData Structure"))
  (returns (CanCast :type Boolean))
  ;[1 1 1] Is the Unit allowed to cast this Spell?
  (if (`KismetArrayLibrary.Array_Contains` (`.AvailableSpells_18_24F66AD5497458F1B1752385743D6DA8` (break `/Game/Blueprints/Core/Units/Utilities/S_UnitData_Stats` (`.Stats_8_1FF4029D4CCC943B93A92087BC3004A2` (break `/Game/Blueprints/Core/Units/Utilities/S_UnitData` (`self.UnitData`))))) (`.Spell_3_DC79AC3F43915DAB55E99DB935B726D0` (break `/Game/Blueprints/Core/Combat/Spells/Utilities/S_SpellData` (`local.SpellData`))))
    ;[1 1 1] Does the Unit have enough AP to cast this Spell?
    (if (>= (`.AP_Current_29_DA4363EA4B23A31EDE4C1398F75B2355` (break `/Game/Blueprints/Core/Units/Utilities/S_UnitData_Stats` (`.Stats_8_1FF4029D4CCC943B93A92087BC3004A2` (break `/Game/Blueprints/Core/Units/Utilities/S_UnitData` (`self.UnitData`))))) (`.Cost_Ap_2_FADCC34944B1CB01238AA984C5CCD6F0` (break `/Game/Blueprints/Core/Combat/Spells/Utilities/S_SpellData_Requirements` (`.Requirements_17_D26D930945DE0FDAF93B6D99C4DC81EF` (break `/Game/Blueprints/Core/Combat/Spells/Utilities/S_SpellData` (`local.SpellData`))))))
      (return true)
      (else
        (return false)))
    (else
      (return false))))

(fn `CombatEnded`
  (`KismetSystemLibrary.PrintString` "Vacation time!")
  ;[1 1 1] Unit has full MP and AP when Combat ends
  (`self.ResetMp`)
  (`self.ResetAp`))

(fn `CombatStarted`
  (`KismetSystemLibrary.PrintString` "I'm in combat!")
  ;[1 1 1] Unit has full MP and AP when Combat starts
  (`self.ResetMp`)
  (`self.ResetAp`))

(fn `GetAnimationState`
  (returns (State :type "/Game/Art/Units/E_UnitAnimationState Enum"))
  (bind _state (message `/Game/Art/Units/BPI_UnitAnimation.GetUnitAnimationState` (`SkeletalMeshComponent.GetAnimInstance` (`self.SkeletalMesh`))))
  (return _state))

(fn `ModifyCurrentAp`
  (params (Modifier :type Integer) (ShowNumber :type Boolean))
  (`self.SetCurrentAp` (+ Modifier (`.AP_Current_29_DA4363EA4B23A31EDE4C1398F75B2355` (break `/Game/Blueprints/Core/Units/Utilities/S_UnitData_Stats` (`.Stats_8_1FF4029D4CCC943B93A92087BC3004A2` (break `/Game/Blueprints/Core/Units/Utilities/S_UnitData` (`self.UnitData`)))))) ShowNumber))

(fn `ModifyCurrentHp`
  (params (Modifier :type Integer))
  (`self.SetCurrentHp` (+ Modifier (`.HP_Current_19_F5821CEE4224044CA52AE58AC941E5A9` (break `/Game/Blueprints/Core/Units/Utilities/S_UnitData_Stats` (`.Stats_8_1FF4029D4CCC943B93A92087BC3004A2` (break `/Game/Blueprints/Core/Units/Utilities/S_UnitData` (`self.UnitData`))))))))

(fn `ModifyCurrentMp`
  (params (Modifier :type Integer) (ShowNumber :type Boolean))
  (`self.SetCurrentMp` (+ Modifier (`.MP_Current_10_FB397B3D409E5FAEA964D8A44B0876D5` (break `/Game/Blueprints/Core/Units/Utilities/S_UnitData_Stats` (`.Stats_8_1FF4029D4CCC943B93A92087BC3004A2` (break `/Game/Blueprints/Core/Units/Utilities/S_UnitData` (`self.UnitData`)))))) ShowNumber))

(fn `OnSpellAnimationHitTile`
  (params (SpellAnimation :type "/Game/Blueprints/Core/Combat/Spells/BP_SpellAnimation Object Reference") (Index :type "IntPoint Structure"))
  (locals (SpellImpactReal :type "/Game/Blueprints/Core/Combat/Spells/Utilities/S_SpellData_Impact_Real Structure"))
  (bind (_value _returnvalue) (`BlueprintMapLibrary.Map_Find` (`self.IncomingSpellImpacts`) (`local.SpellAnimation`)))
  ;[1 1 1] check if the index of the Tile under the Unit is the same index targeted by the Spell
  (if (`KismetMathLibrary.Equal_IntPointIntPoint` (`local.Index`) Index)
    ;[1 1 1] Check we still need to process the spell
    (if _returnvalue
      (set `local.SpellImpactReal` _value)
      ;[1 1 1] To avoid process the same spell again
      (`BlueprintMapLibrary.Map_Remove` (`self.IncomingSpellImpacts`) (`local.SpellAnimation`))
      ;[1 1 1] If the spell deals damage or heals the Unit (not neutral)
      (if (!= (`.Modifier_Hp_4_6DDF92144525D3619EA8028342570120` (break `/Game/Blueprints/Core/Combat/Spells/Utilities/S_SpellData_Impact_Real` (`local.SpellImpactReal`))) 0)
        ;[1 1 1] Update HP bar and play animated numbers
        (`/Game/Blueprints/Core/Units/Widget/W_HpBar.Event_UpdateHpBar` (`self.HpBar`)) ; Update the Unit's HP bar
        (`|SpawnActorFromClass` "/Game/Blueprints/Core/Units/Widget/BP_AnimatedNumber.BP_AnimatedNumber_C" (`KismetMathLibrary.MakeTransform` (`self.K2_GetActorLocation`)) "Undefined" "MultiplyWithRoot" null (`.Modifier_Hp_4_6DDF92144525D3619EA8028342570120` (break `/Game/Blueprints/Core/Combat/Spells/Utilities/S_SpellData_Impact_Real` (`local.SpellImpactReal`))) "NewEnumerator0" null) ; Spawn the Animated Number
        ;[1 1 1] If the spell deals damage to the Unit (not neutral or heal)
        (if (< (`.Modifier_Hp_4_6DDF92144525D3619EA8028342570120` (break `/Game/Blueprints/Core/Combat/Spells/Utilities/S_SpellData_Impact_Real` (`local.SpellImpactReal`))) 0)
          ;[1 1 1] Is the Unit dead?
          (if (== (`.HP_Current_19_F5821CEE4224044CA52AE58AC941E5A9` (break `/Game/Blueprints/Core/Units/Utilities/S_UnitData_Stats` (`.Stats_8_1FF4029D4CCC943B93A92087BC3004A2` (break `/Game/Blueprints/Core/Units/Utilities/S_UnitData` (`self.UnitData`))))) 0)
            ;[1 1 1 1 16] If there were 1 or more spell in act before the one that killed the Unit
            ; we avoid to play the death animation more than once by checking id the Unit is already animating its death, if not we start the animation
            (if (`|EnumInequality` (`self.GetAnimationState`) "NewEnumerator4")
              (`self.SetAnimationState` "NewEnumerator4") ; Play Death animation
            )
            (else
              (`self.SetAnimationState` "NewEnumerator3") ; Play Hit animation
            )))))))

(fn `ResetAp`
  (`self.SetCurrentAp` (`.AP_Max_28_1D0AED0B46551EB3D4DF219545237E89` (break `/Game/Blueprints/Core/Units/Utilities/S_UnitData_Stats` (`.Stats_8_1FF4029D4CCC943B93A92087BC3004A2` (break `/Game/Blueprints/Core/Units/Utilities/S_UnitData` (`self.UnitData`))))) true))

(fn `ResetMp`
  (`self.SetCurrentMp` (`.MP_Max_23_3B0BB7B1467D1E4FA1664A9FE87012CB` (break `/Game/Blueprints/Core/Units/Utilities/S_UnitData_Stats` (`.Stats_8_1FF4029D4CCC943B93A92087BC3004A2` (break `/Game/Blueprints/Core/Units/Utilities/S_UnitData` (`self.UnitData`))))) true))

(fn `SetAnimationState`
  (params (State :type "/Game/Art/Units/E_UnitAnimationState Enum" :default "NewEnumerator0"))
  (message `/Game/Art/Units/BPI_UnitAnimation.SetUnitAnimationState` (`SkeletalMeshComponent.GetAnimInstance` (`self.SkeletalMesh`)) State))

(fn `SetCurrentAp`
  (params (Ap :type Integer) (ShowNumber :type Boolean))
  (locals (Difference :type Integer :default 0))
  (bind ((`AP_Current_29_DA4363EA4B23A31EDE4C1398F75B2355` _ap_current) (`AP_Max_28_1D0AED0B46551EB3D4DF219545237E89` _ap_max)) (break `/Game/Blueprints/Core/Units/Utilities/S_UnitData_Stats` (`.Stats_8_1FF4029D4CCC943B93A92087BC3004A2` (break `/Game/Blueprints/Core/Units/Utilities/S_UnitData` (`self.UnitData`)))))
  ;[1 1 1] We save the difference NewValue-ActualValue cos we need it for Number animation
  (set `local.Difference` (- Ap _ap_current))
  ;[1 1 1] Update the current AP value in the UnitData_Stat
  (bind _structout (setmembers `/Game/Blueprints/Core/Units/Utilities/S_UnitData_Stats` :`StructRef` (`.Stats_8_1FF4029D4CCC943B93A92087BC3004A2` (break `/Game/Blueprints/Core/Units/Utilities/S_UnitData` (`self.UnitData`))) :`AP_Current` (`KismetMathLibrary.Clamp` Ap 0 _ap_max)))
  ;[1 1 1] Update UnitData_Stats inside UnitData
  (setmembers `/Game/Blueprints/Core/Units/Utilities/S_UnitData` :`StructRef` (`self.UnitData`) :`Stats` _structout)
  (`self.OnUnitStatsChanged` self) ; Notify stat changed
  ;[1 1 1] If there's was an actual movement and we wanna display the Number animation...
  (if (and (`local.ShowNumber`) (!= (`local.Difference`) 0))
    ;[1 1 1] Spawn it with the difference calculated before
    (`|SpawnActorFromClass` "/Game/Blueprints/Core/Units/Widget/BP_AnimatedNumber.BP_AnimatedNumber_C" (`KismetMathLibrary.MakeTransform` (`self.K2_GetActorLocation`)) "Undefined" "MultiplyWithRoot" null (`local.Difference`) "NewEnumerator2" null)))

(fn `SetCurrentHp`
  (params (Hp :type Integer))
  ;[1 1 1] Update the current HP value in the UnitData_Stat
  (bind _structout (setmembers `/Game/Blueprints/Core/Units/Utilities/S_UnitData_Stats` :`StructRef` (`.Stats_8_1FF4029D4CCC943B93A92087BC3004A2` (break `/Game/Blueprints/Core/Units/Utilities/S_UnitData` (`self.UnitData`))) :`HP_Current` (`KismetMathLibrary.Clamp` Hp 0 (`.HP_Max_20_56606D324C12E5DB5E7681B94263A483` (break `/Game/Blueprints/Core/Units/Utilities/S_UnitData_Stats` (`.Stats_8_1FF4029D4CCC943B93A92087BC3004A2` (break `/Game/Blueprints/Core/Units/Utilities/S_UnitData` (`self.UnitData`))))))))
  ;[1 1 1] Update UnitData_Stats inside UnitData
  (setmembers `/Game/Blueprints/Core/Units/Utilities/S_UnitData` :`StructRef` (`self.UnitData`) :`Stats` _structout)
  (`self.OnUnitStatsChanged` self) ; Notify stat changed
)

(fn `SetCurrentMp`
  (params (Mp :type Integer) (ShowNumber :type Boolean))
  (locals (Difference :type Integer :default 0))
  (bind ((`MP_Current_10_FB397B3D409E5FAEA964D8A44B0876D5` _mp_current) (`MP_Max_23_3B0BB7B1467D1E4FA1664A9FE87012CB` _mp_max)) (break `/Game/Blueprints/Core/Units/Utilities/S_UnitData_Stats` (`.Stats_8_1FF4029D4CCC943B93A92087BC3004A2` (break `/Game/Blueprints/Core/Units/Utilities/S_UnitData` (`self.UnitData`)))))
  ;[1 1 1] We save the difference NewValue-ActualValue cos we need it for Number animation
  (set `local.Difference` (- Mp _mp_current))
  ;[1 1 1] Update the current MP value in the UnitData_Stat
  (bind _structout (setmembers `/Game/Blueprints/Core/Units/Utilities/S_UnitData_Stats` :`StructRef` (`.Stats_8_1FF4029D4CCC943B93A92087BC3004A2` (break `/Game/Blueprints/Core/Units/Utilities/S_UnitData` (`self.UnitData`))) :`MP_Current` (`KismetMathLibrary.Clamp` Mp 0 _mp_max)))
  ;[1 1 1] Update UnitData_Stats inside UnitData
  (setmembers `/Game/Blueprints/Core/Units/Utilities/S_UnitData` :`StructRef` (`self.UnitData`) :`Stats` _structout)
  (`self.OnUnitStatsChanged` self) ; Notify stat changed
  ;[1 1 1] If there's was an actual movement and we wanna display the Number animation...
  (if (and (`local.ShowNumber`) (!= (`local.Difference`) 0))
    ;[1 1 1] Spawn it with the difference calculated before
    (`|SpawnActorFromClass` "/Game/Blueprints/Core/Units/Widget/BP_AnimatedNumber.BP_AnimatedNumber_C" (`KismetMathLibrary.MakeTransform` (`self.K2_GetActorLocation`)) "Undefined" "MultiplyWithRoot" null (`local.Difference`) "NewEnumerator1" null)))

(fn `SetGrid`
  (params (Grid :type "/Game/Blueprints/Core/Grid/BP_Grid Object Reference"))
  (bind _mesh_teamindex (`self.Mesh_TeamIndex`))
  (bind _collision_lineofsight (`self.Collision_LineOfSight`))
  (bind (_returnvalue_x _returnvalue_y _returnvalue_z) (`KismetMathLibrary.BreakVector` (`SceneComponent.K2_GetComponentScale` (`self.Collision_LineOfSight`))))
  (bind (_meshsize _mesh) (break `/Game/Blueprints/Core/Grid/GridShapes/S_GridShapeData` (`/Game/Blueprints/Core/Grid/BP_Grid.GetCurrentShapeData` (`self.Grid`))))
  (bind ((`MeshSize_2_09D7913C41F06EB5C6F9088AC614A7CA` _meshsize_2) (`FlatMesh_12_0AE789804219F7B62751CC8875408A2A` _flatmesh) (`FlatMaterial_18_EA13732247B5B91176C6D194C204038A` _flatmaterial)) (break `/Game/Blueprints/Core/Grid/GridShapes/S_GridShapeData` (`/Game/Blueprints/Core/Grid/BP_Grid.GetCurrentShapeData` (`self.Grid`))))
  (bind (_returnvalue_x_2 _returnvalue_y_2) (`KismetMathLibrary.BreakVector` (/ (`/Game/Blueprints/Core/Grid/BP_Grid.GridTileSize` (`self.Grid`)) _meshsize)))
  (set `self.Grid` Grid)
  ;[1 1 1] The Units have a collision mesh to block LineOfSight for spells. This collision box has to respect the shape of the grid and the size of its tiles
  (`StaticMeshComponent.SetStaticMesh` _collision_lineofsight _mesh) ; shape of the grid
  (`SceneComponent.SetAbsolute` _collision_lineofsight false true true) ; This blocks the collision box to rotate\ntogether with the Unit when it moves
  (`SceneComponent.SetWorldScale3D` _collision_lineofsight (`KismetMathLibrary.MakeVector` _returnvalue_x_2 _returnvalue_y_2 _returnvalue_z)) ; size of the grid tiles
  ;[1 1 1] Setup the Mesh under the Unit that indicates the Team by the color (color is set in SetTeamIndex function)
  (`StaticMeshComponent.SetStaticMesh` _mesh_teamindex _flatmesh)
  (`PrimitiveComponent.SetMaterial` _mesh_teamindex 0 _flatmaterial)
  (`MeshComponent.SetScalarParameterValueOnMaterials` _mesh_teamindex "isFilled" 1.0) ; To color the middle of the square
  (`SceneComponent.SetAbsolute` _mesh_teamindex false true true)
  (`SceneComponent.SetWorldScale3D` _mesh_teamindex (/ (`/Game/Blueprints/Core/Grid/BP_Grid.GridTileSize` (`self.Grid`)) _meshsize_2))
  (`SceneComponent.K2_SetRelativeLocation` _mesh_teamindex (`KismetMathLibrary.MakeVector` 0.0 0.0 (+ (`/Game/Blueprints/Core/Grid/BP_GridVisual.OffsetFromGround` (`/Game/Blueprints/Core/Grid/BP_Grid.GridVisual` (`self.Grid`))) 5.0)) false false))

(fn `SetGridIndex`
  (params (Index :type "IntPoint Structure"))
  (set `self.Index` Index))

(fn `SetIsHovered`
  (params (Hovered :type Boolean))
  (set `self.IsHovered` Hovered)
  (`self.UpdateVisualIfHoveredOrSelected`)
  ;[1 1 1] Notify the change of hovered Unit
  (`self.OnUnitHoveredChanged` self))

(fn `SetIsSelected`
  (params (Selected :type Boolean))
  (set `self.IsSelected` Selected)
  (`self.UpdateVisualIfHoveredOrSelected`)
  ;[1 1 1] Notify the change of selected Unit
  (`self.OnUnitSelectedChanged` self))

(fn `SetTeamIndex`
  (params (Index :type Integer))
  (set `self.TeamIndex` Index)
  ;[1 1 1] HP bar fill color changes based on the Unit Team
  (`ProgressBar.SetFillColorAndOpacity` (`/Game/Blueprints/Core/Units/Widget/W_HpBar.ProgressBar_Hp` (`self.HpBar`)) (`/Game/Blueprints/Core/Combat/Utilities/BFL_Combat.GetTeamColor` (`self.TeamIndex`)))
  ;[1 1 1] Tile color under the Unit changes based on the Unit Team
  (`MeshComponent.SetVectorParameterValueOnMaterials` (`self.Mesh_TeamIndex`) "Color" (`KismetMathLibrary.Conv_LinearColorToVector` (`/Game/Blueprints/Core/Combat/Utilities/BFL_Combat.GetTeamColor` (`self.TeamIndex`))))
  ;[1 1 1] By Finn: Tile opacity under the Unit a bit transparent
  ; to let the Tile selection visible under it
  (`MeshComponent.SetScalarParameterValueOnMaterials` (`self.Mesh_TeamIndex`) "Opacity" 0.6))

(fn `SetUnitData`
  (params (Data :type "/Game/Blueprints/Core/Units/Utilities/S_UnitData Structure (by ref)"))
  (bind _skeletalmesh (`self.SkeletalMesh`))
  (bind _output_get (set `self.UnitData` Data))
  (bind (_mesh _animbp) (break `/Game/Blueprints/Core/Units/Utilities/S_UnitData_Assets` (`.Assets_5_056CBBFF4790CD88526296BC494FAEB5` (break `/Game/Blueprints/Core/Units/Utilities/S_UnitData` _output_get))))
  (`SkeletalMeshComponent.SetSkeletalMeshAsset` _skeletalmesh _mesh)
  (`SkeletalMeshComponent.SetAnimInstanceClass` _skeletalmesh _animbp))

(fn `TurnEnded`
  (`KismetSystemLibrary.PrintString` "Sleep time!")
  ;[1 1 1] Unit has full MP and AP when its Turn ends
  (`self.ResetMp`)
  (`self.ResetAp`))

(fn `TurnStarted`
  (`KismetSystemLibrary.PrintString` "It's my turn!"))

(fn `UnitCastSpell`
  (params (TargetIndex :type "IntPoint Structure") (SpellData :type "/Game/Blueprints/Core/Combat/Spells/Utilities/S_SpellData Structure"))
  ;[1 1 1] We make the Unit look towards the TargetTile
  (`self.K2_SetActorRotation` (`KismetMathLibrary.FindLookAtRotation` (`KismetMathLibrary.MakeVector` (.x (`self.K2_GetActorLocation`)) (.y (`self.K2_GetActorLocation`))) (`KismetMathLibrary.MakeVector` (.x (.location (`.Transform_7_D016BDCC41B32F0EC4D85EB94D99E603` (break `/Game/Blueprints/Core/Grid/Utilities/S_TileData` (`BlueprintMapLibrary.Map_Find` (`/Game/Blueprints/Core/Grid/BP_Grid.GridTiles` (`self.Grid`)) (`local.TargetIndex`)))))) (.y (.location (`.Transform_7_D016BDCC41B32F0EC4D85EB94D99E603` (break `/Game/Blueprints/Core/Grid/Utilities/S_TileData` (`BlueprintMapLibrary.Map_Find` (`/Game/Blueprints/Core/Grid/BP_Grid.GridTiles` (`self.Grid`)) (`local.TargetIndex`)))))))))
  ;[1 1 1] Play the Attack animation
  (`self.SetAnimationState` "NewEnumerator2")
  ;[1 1 1] the Unit spend AP to cast the Spell
  (`self.ModifyCurrentAp` (- 0 (`.Cost_Ap_2_FADCC34944B1CB01238AA984C5CCD6F0` (break `/Game/Blueprints/Core/Combat/Spells/Utilities/S_SpellData_Requirements` (`.Requirements_17_D26D930945DE0FDAF93B6D99C4DC81EF` (break `/Game/Blueprints/Core/Combat/Spells/Utilities/S_SpellData` (`local.SpellData`)))))) true))

(fn `UnitHitBySpell`
  (params (SpellImpactReal :type "/Game/Blueprints/Core/Combat/Spells/Utilities/S_SpellData_Impact_Real Structure") (SpellAnimation :type "/Game/Blueprints/Core/Combat/Spells/BP_SpellAnimation Object Reference"))
  (bind _modifier_hp (break `/Game/Blueprints/Core/Combat/Spells/Utilities/S_SpellData_Impact_Real` (`local.SpellImpactReal`)))
  ;[1 1 1] For each spell that target the Unit we save data about the animation and the impact, to decide if and when the Unit needs to play its hit animation
  (`BlueprintMapLibrary.Map_Add` (`self.IncomingSpellImpacts`) SpellAnimation SpellImpactReal)
  (add `/Game/Blueprints/Core/Combat/Spells/BP_SpellAnimation.OnSpellAnimationHitTile` SpellAnimation (`|CreateDelegate` :!event `OnSpellAnimationHitTile`))
  ;[1 1 1] If a spell doesn't do damage (like RunChickenRun), we stop
  (if (!= _modifier_hp 0)
    ;[1 1 1] We update the HP
    (`self.ModifyCurrentHp` _modifier_hp)))

(fn `UpdateVisualIfHoveredOrSelected`
  (bind _isselected (`self.IsSelected`))
  (`MeshComponent.SetVectorParameterValueOnMaterials` (`self.SkeletalMesh`) "ColorMultiply" (`KismetMathLibrary.Conv_LinearColorToVector` (* (* (* (struct :`R` 1.0 :`G` 1.0 :`B` 1.0 :`A` 1.0) (`KismetMathLibrary.SelectFloat` 2.5 1.0 (`self.IsHovered`))) (`KismetMathLibrary.SelectFloat` 2.5 1.0 _isselected)) (`KismetMathLibrary.SelectColor` (struct :`R` 0.8 :`G` 0.25 :`B` 0.5 :`A` 1.0) (struct :`R` 1.0 :`G` 1.0 :`B` 1.0 :`A` 1.0) _isselected)))))

(fn `UserConstructionScript`
  (bind _unitdata (`/Game/Blueprints/Core/Units/Utilities/BFL_Units.GetDefaultDataFromUnitType` (`self.UnitType`)))
  (`self.SetUnitData` _unitdata))