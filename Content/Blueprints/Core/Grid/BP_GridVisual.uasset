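; BP_GridVisual is the actor that renders the grid's tiles, with tick disabled.
; On initialization it sets up a child-actor BP_GridMeshInst with the current shape's flat mesh and material, then centers itself at world origin raised by a ground offset.
; Tile updates remove the old instance and re-add it, colored by state, only for walkable types; destroying the visual clears all instances.
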(event `self.ReceiveBeginPlay`
  ;[1 1 1] Disables the Tick
  (`self.SetActorTickEnabled` false))

(fn `DestroyGridVisual`
  (bind _gridmeshinst (`self.GridMeshInst`))
  ;[1 1 1] Normal Grid
  (`/Engine/EditorBlueprintResources/StandardMacros.IsValid` _gridmeshinst
    (:`Is Valid`
      (`/Game/Blueprints/Core/Grid/Utilities/BP_GridMeshInst.ClearInstances` _gridmeshinst))))

(fn `InitializeGridVisual`
  (params (Grid :type "/Game/Blueprints/Core/Grid/BP_Grid Object Reference"))
  (bind (_meshsize _mesh _meshmaterial _flatmesh _flatmaterial) (break `/Game/Blueprints/Core/Grid/GridShapes/S_GridShapeData` (`/Game/Blueprints/Core/Grid/BP_Grid.GetCurrentShapeData` (`self.Grid`))))
  (set `self.Grid` Grid)
  (set `self.GridMeshInst` (cast `/Game/Blueprints/Core/Grid/Utilities/BP_GridMeshInst` (`ChildActorComponent.ChildActor` (`self.ChildActor_GridMeshInst`)) :!pure true))
  ;[1 1 1] Setup the components for the Normal Grid
  (`/Game/Blueprints/Core/Grid/Utilities/BP_GridMeshInst.InitializeGridMeshInst` :`self` (`self.GridMeshInst`) :`Mesh` _flatmesh :`Material` _flatmaterial :`Collision` "QueryOnly") ; Normal Grid - Colors based on State
  (`self.K2_SetActorLocation` (0.0 0.0 0.0)) ; Center Grid in World (0,0,0)
  (`self.SetOffsetFromGround` (`self.OffsetFromGround`)))

(fn `SetOffsetFromGround`
  (params (Offset :type "Float (double-precision)"))
  (bind (_returnvalue_x _returnvalue_y) (`KismetMathLibrary.BreakVector` (`self.K2_GetActorLocation`)))
  (set `self.OffsetFromGround` Offset)
  ;[1 1 1] Only the Z gets adjusted
  (`self.K2_SetActorLocation` (`KismetMathLibrary.MakeVector` _returnvalue_x _returnvalue_y (`self.OffsetFromGround`))))

(fn `UpdateTileVisual`
  (params (Data :type "/Game/Blueprints/Core/Grid/Utilities/S_TileData Structure"))
  (bind (_data_index _data_type) (break `/Game/Blueprints/Core/Grid/Utilities/S_TileData` (`local.Data`)))
  (bind (_data_index_2 _data_type_2 _data_transform _data_states) (break `/Game/Blueprints/Core/Grid/Utilities/S_TileData` (`local.Data`)))
  ;[1 1 1] Normal Grid
  ;;[1 1 1] The first thing is to remove the old tile
  (`/Game/Blueprints/Core/Grid/Utilities/BP_GridMeshInst.RemoveInstance` (`self.GridMeshInst`) _data_index)
  ;;[1 1 1] The tile is created only if the type is walkable
  (if (`/Game/Blueprints/Core/Grid/Utilities/BFL_TileData.IsTileTypeWalkable` _data_type)
    (`/Game/Blueprints/Core/Grid/Utilities/BP_GridMeshInst.AddInstance` (`self.GridMeshInst`) _data_index_2 _data_transform _data_states)))

(fn `UserConstructionScript`)