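; Grid pathfinding helper that finds the valid neighbor tiles of a given tile index on a referenced Grid.
; GetNeighborsIndices switches on grid shape, handling only Square, with four cardinal neighbors and optional diagonals.
; GetValidTileNeighbors filters those through the grid's tile map, keeping walkable tiles whose height difference is within the tile's Z size.
; No path search is implemented here, and the event graph is empty.
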(fn `GetNeighborIndicesForSquare`
  (params (Index :type "IntPoint Structure") (IncludeDiagonals :type Boolean))
  (returns (Neighbors :type "Array of IntPoint Structure"))
  (locals (RetNeighbors :type "Array of IntPoint Structure"))
  (bind _array (`|MakeArray` (+ (`local.Index`) (make `IntPoint` 1)) (+ (`local.Index`) (make `IntPoint` 0 1)) (+ (`local.Index`) (make `IntPoint` -1)) (+ (`local.Index`) (make `IntPoint` 0 -1))))
  (if IncludeDiagonals
    (bind _output_get (set `local.RetNeighbors` _array))
    (`KismetArrayLibrary.Array_Append` _output_get (`|MakeArray` (+ (`local.Index`) (make `IntPoint` 1 1)) (+ (`local.Index`) (make `IntPoint` -1 1)) (+ (`local.Index`) (make `IntPoint` -1 -1)) (+ (`local.Index`) (make `IntPoint` 1 -1))))
    (return (`local.RetNeighbors`))
    (else
      (return _array))))

(fn `GetNeighborsIndices`
  (params (Index :type "IntPoint Structure") (IncludeDiagonals :type Boolean))
  (returns (Neighbors :type "Array of IntPoint Structure"))
  (switch `/Game/Blueprints/Core/Grid/GridShapes/E_GridShape` (`/Game/Blueprints/Core/Grid/BP_Grid.GridShape` (`self.Grid`))
    (:`NewEnumerator1`
      (return (`self.GetNeighborIndicesForSquare` (`local.Index`) (`local.IncludeDiagonals`))))))

(fn `GetValidTileNeighbors`
  (params (Index :type "IntPoint Structure") (IncludeDiagonals :type Boolean))
  (returns (RetNeighbors :type "Array of IntPoint Structure"))
  (locals (Data :type "/Game/Blueprints/Core/Grid/Utilities/S_TileData Structure") (InputData :type "/Game/Blueprints/Core/Grid/Utilities/S_TileData Structure") (ValidIndices :type "Array of IntPoint Structure"))
  (bind _data_index (break `/Game/Blueprints/Core/Grid/Utilities/S_TileData` (`local.Data`)))
  (bind (_data_index_2 _data_type) (break `/Game/Blueprints/Core/Grid/Utilities/S_TileData` (`local.Data`)))
  (bind (_gridtilesize_x _gridtilesize_y _gridtilesize_z) (`KismetMathLibrary.BreakVector` (`/Game/Blueprints/Core/Grid/BP_Grid.GridTileSize` (`self.Grid`))))
  ;[1 1 1] We need the Data for the tile corresponding to the index in Input
  ; to compare it later with its neighbors
  (set `local.InputData` (`BlueprintMapLibrary.Map_Find` (`/Game/Blueprints/Core/Grid/BP_Grid.GridTiles` (`self.Grid`)) (`local.Index`)))
  ;[1 1 1] Then we find neighbors indices
  (bind _neighbors (`self.GetNeighborsIndices` (`local.Index`) (`local.IncludeDiagonals`)))
  ;[1 1 1] Before returning the Neighbors Indices, we access their data to check if they need to be discarded
  (for _array_element _neighbors
    (set `local.Data` (`BlueprintMapLibrary.Map_Find` (`/Game/Blueprints/Core/Grid/BP_Grid.GridTiles` (`self.Grid`)) _array_element))
    ;[1 1 1] Check 1 - The tile must be walkable
    (if (`/Game/Blueprints/Core/Grid/Utilities/BFL_TileData.IsTileTypeWalkable` _data_type)
      ;[1 1 1] Check 2 - We compare the height (Z coordinate) of the Tile in input with its Neighbors.
      ; If the difference is too steep (bigger than the Grid Tile Size along Z),
      ; then we don't consider that neighbor valid
      (if (<= (`KismetMathLibrary.Abs` (- (.z (.location (`.Transform_7_D016BDCC41B32F0EC4D85EB94D99E603` (break `/Game/Blueprints/Core/Grid/Utilities/S_TileData` (`local.InputData`))))) (.z (.location (`.Transform_7_D016BDCC41B32F0EC4D85EB94D99E603` (break `/Game/Blueprints/Core/Grid/Utilities/S_TileData` (`local.Data`))))))) _gridtilesize_z)
        ;[1 1 1] All checks passed, add the index to the valid neighbors array
        (`KismetArrayLibrary.Array_Add` (`local.ValidIndices`) _data_index))))
  ;[1 1 1] At the end, we return all the valid neighbors
  (return (`local.ValidIndices`)))

(fn `UserConstructionScript`)