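; Debug actor that shows X,Y index labels on the walkable tiles of BP_Grid.
; It binds to the grid's tile-updated and grid-destroyed dispatchers, keeping label updates event-driven and off Tick.
; A map from index to TextRenderActor reuses, spawns or destroys labels as tiles change.
; SetShowTileIndices toggles the display by rebuilding every label or clearing them all.
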(event `self.ReceiveBeginPlay`
  (bind _returnvalue (`GameplayStatics.GetActorOfClass` "/Game/Blueprints/Core/Grid/BP_Grid.BP_Grid_C"))
  (bind _output_get (set `self.Grid` _returnvalue))
  ;[1 1 1] Since the text containing the tile indices are only for debug use,
  ; we add them by using events.
  ; We listen to these two events (whose dispatchers are in the BP_Grid)
  ; to get notified everytime a tile is added/removed or the grid is destroyed
  (add `/Game/Blueprints/Core/Grid/BP_Grid.OnTileDataUpdated` _output_get (`|CreateDelegate` :!event `UpdateTextOnTile`))
  (add `/Game/Blueprints/Core/Grid/BP_Grid.OnGridDestroyed` _output_get (`|CreateDelegate` :!event `ClearAllTextActors`)))

(fn `ClearAllTextActors`
  ;[1 1 1] Clear all the map of Indices and TextActors, and destroy all the corresponding TextActors.
  ; Useful when we destroy the entire grid
  (bind _values (`BlueprintMapLibrary.Map_Values` (`self.SpawnedTexts`)))
  (for _array_element _values
    (`self.K2_DestroyActor` _array_element))
  (`BlueprintMapLibrary.Map_Clear` (`self.SpawnedTexts`)))

(fn `DestroyTextActor`
  (params (Index :type "IntPoint Structure"))
  (locals (Actor :type "TextRenderActor Object Reference"))
  ;[1 1 1] If we find a valid entry in our map for the index in input
  (bind _output_get (set `local.Actor` (`BlueprintMapLibrary.Map_Find` (`self.SpawnedTexts`) Index)))
  (`/Engine/EditorBlueprintResources/StandardMacros.IsValid` _output_get
    (:`Is Valid`
      ;[1 1 1] we destroy the actor and remove the entry from the map
      (`self.K2_DestroyActor` _output_get)
      (`BlueprintMapLibrary.Map_Remove` (`self.SpawnedTexts`) (`local.Index`)))))

(fn `GetTextActor`
  (params (Index :type "IntPoint Structure"))
  (returns (TextRenderedActor :type "TextRenderActor Object Reference"))
  (locals (TextActor :type "TextRenderActor Object Reference"))
  (bind _textactor (`local.TextActor`))
  (bind _textrender (`TextRenderActor.TextRender` (`local.TextActor`)))
  ;[1 1 1] First, we look for an entry in our map for the index in input
  (bind _output_get (set `local.TextActor` (`BlueprintMapLibrary.Map_Find` (`self.SpawnedTexts`) Index)))
  (`/Engine/EditorBlueprintResources/StandardMacros.IsValid` _output_get ; Since we don't wanna spawn a second Text actor for the same index, we check if it's valid
    (:`Is Valid`
      ;[1 1 1] It's valid, we just return it
      (return (`local.TextActor`)))
    (:`Is Not Valid`
      ;[1 1 1] Not valid, we spawn a new TextActor
      (bind _returnvalue (`|SpawnActorFromClass` "/Script/Engine.TextRenderActor" (`KismetMathLibrary.MakeTransform` (0.0 0.0 0.0)) "AlwaysSpawn" "MultiplyWithRoot" null null))
      (set `local.TextActor` _returnvalue)
      ;[1 1 1] add it to the map
      (`BlueprintMapLibrary.Map_Add` (`self.SpawnedTexts`) (`local.Index`) (`local.TextActor`))
      (`self.SetActorTickEnabled` _textactor false) ; Disabling the tick
      (`self.SetActorEnableCollision` _textactor false) ; Disabling the collision
      ;[1 1 1] Center the text both horizontally and vertically
      (`TextRenderComponent.SetHorizontalAlignment` _textrender "EHTA_Center")
      (`TextRenderComponent.SetVerticalAlignment` _textrender "EVRTA_TextCenter")
      ;[1 1 1] and return it
      (return (`local.TextActor`)))))

(fn `SetShowTileIndices`
  (params (ShowTileIndices :type Boolean))
  ;[1 1 1] The bool in input tells us
  ; if we wanna show the idices or not
  (bind _output_get (set `self.ShowTileIndices` ShowTileIndices))
  (if _output_get
    ;[1 1 1] We wanna see them, so we access all of them and update the corresponding TextActors
    (bind _keys (`BlueprintMapLibrary.Map_Keys` (`/Game/Blueprints/Core/Grid/BP_Grid.GridTiles` (`self.Grid`))))
    (for _array_element _keys
      (`self.UpdateTextOnTile` _array_element))
    (else
      (`self.ClearAllTextActors`) ; No Idices, clear all the TextActors
    )))

(fn `UpdateTextOnTile`
  (params (Index :type "IntPoint Structure"))
  (locals (TileData :type "/Game/Blueprints/Core/Grid/Utilities/S_TileData Structure") (TextActor :type "TextRenderActor Object Reference") (Text :type String))
  (bind (_index_x _index_y) (break `IntPoint` (`local.Index`)))
  (bind (_tiledata_index _tiledata_type) (break `/Game/Blueprints/Core/Grid/Utilities/S_TileData` (`local.TileData`)))
  (bind (_value _returnvalue) (`BlueprintMapLibrary.Map_Find` (`/Game/Blueprints/Core/Grid/BP_Grid.GridTiles` (`self.Grid`)) (`local.Index`)))
  (if (`self.ShowTileIndices`)
    (if _returnvalue
      ;[1 1 1] ... and put it in a local var
      (set `local.TileData` _value)
      ;[1 1 1] We check if the tile is walkable (no text on unwalkable ones)
      (if (`/Game/Blueprints/Core/Grid/Utilities/BFL_TileData.IsTileTypeWalkable` _tiledata_type)
        ;[1 1 1] We get the text actor corresponding to that index
        (bind _textrenderedactor (`self.GetTextActor` (`local.Index`)))
        (set `local.TextActor` _textrenderedactor)
        ;[1 1 1] We build the text to render on it
        (set `local.Text` (`KismetStringLibrary.Concat_StrStr` (`KismetStringLibrary.Conv_IntToString` _index_x) "," (`KismetStringLibrary.Conv_IntToString` _index_y)))
        ;[1 1 1] we set the text on the TextActor
        (`TextRenderComponent.K2_SetText` (`TextRenderActor.TextRender` (`local.TextActor`)) (`KismetTextLibrary.Conv_StringToText` (`local.Text`)))
        ;[1 1 1] And finally we move the TextActor to the corresponding Tile location
        ; and position, scale and orient it properly
        (`self.K2_SetActorTransform` (`local.TextActor`) (`KismetMathLibrary.MakeTransform` (+ (.location (`.Transform_7_D016BDCC41B32F0EC4D85EB94D99E603` (break `/Game/Blueprints/Core/Grid/Utilities/S_TileData` (`local.TileData`)))) (0.0 0.0 1.0)) (struct :`Pitch` 90.0 :`Yaw` 180.0) (2.0 2.0 2.0)) false false)
        (else
          ;[1 1 1] If the tile does not exist or it's not walkable,
          ; we destroy the TextActor cos we don't want it there
          (`self.DestroyTextActor` (`local.Index`) :!label _label)))
      (else
        (goto _label)))))

(fn `UserConstructionScript`)